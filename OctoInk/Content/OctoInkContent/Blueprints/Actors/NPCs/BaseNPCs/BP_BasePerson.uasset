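; Base NPC person that shows a prompt when the player is near and can start dialogue.
; Sphere overlaps with BP_MainGamePlayer toggle the prompt by setting the Plane's material to the quest prompt or clearing it.
; TalkToPlayer passes the NPC's Dialogue to the BP_MainWorld game mode to display; nothing in this Blueprint calls it.
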(event OnComponentBeginOverlap(Sphere)
  (params (OverlappedComponent :type Primitive%20Component%20Object%20Reference) (OtherActor :type Actor%20Object%20Reference) (OtherComp :type Primitive%20Component%20Object%20Reference) (OtherBodyIndex :type Integer) (bFromSweep :type Boolean) (SweepResult :type Hit%20Result%20Structure%20%28by%20ref%29))
  (Utilities|Casting|CastToBP_MainGamePlayer OtherActor)
  (CallFunction|ShowExclam))

(event OnComponentEndOverlap(Sphere)
  (params (OverlappedComponent :type Primitive%20Component%20Object%20Reference) (OtherActor :type Actor%20Object%20Reference) (OtherComp :type Primitive%20Component%20Object%20Reference) (OtherBodyIndex :type Integer))
  (Utilities|Casting|CastToBP_MainGamePlayer OtherActor)
  (CallFunction|HideExclam))

(event EventBeginPlay)

(event Collision|EventActorBeginOverlap
  (params (OtherActor :type Actor%20Object%20Reference)))

(event EventTick
  (params (DeltaSeconds :type Float%20%28single-precision%29)))

(fn ConstructionScript)

(fn TalktoPlayer
  (bind _asbp_main_world (Utilities|Casting|CastToBP_MainWorld (Game|GetGameMode)))
  (Default|ShowDialogue _asbp_main_world (Variables|Default|GetDialogue)))

(fn ShowExclam
  (Rendering|Material|SetMaterial (Variables|Default|GetPlane) 0 "/Game/OctoInkContent/Assets/UIAssets/Quest/quest_prompt_Mat.quest_prompt_Mat"))

(fn HideExclam
  (Rendering|Material|SetMaterial (Variables|Default|GetPlane) 0 "/Game/OctoInkContent/Assets/UIAssets/Obstacle/Nothing.Nothing"))