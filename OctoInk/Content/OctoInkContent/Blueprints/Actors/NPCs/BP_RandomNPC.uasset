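; BP_RandomNPC is a Spine-animated ambient NPC that walks between waypoints with a random skin and walk speed.
; NewMove uses AI MoveTo, pauses briefly at waypoints flagged with a certain action, then calls CalculatePath.
; CalculatePath picks a random neighbor from waypoint node pairs, flips the Spine renderer by Y direction and moves again.
; A separate Move event loops through a fixed NPCPath array.
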(event Custom|Move
  (AI|AIMoveTo (Pawn|GetControlledPawn (Pawn|GetController)) (Transformation|GetWorldLocation (Variables|/Script/Engine.TargetPoint|GetSpriteComponent (.Location (Utilities|Struct|BreakNPCPath (Utilities|Array|Get(acopy) (Variables|Default|GetNPCPath) (Variables|Default|GetNPCPathIndex)))))) 0 5.0 false
    (:OnSuccess
      (if (Utilities|Enum|Equal(Enum) (.Action (Utilities|Struct|BreakNPCPath (Utilities|Array|Get(acopy) (Variables|Default|GetNPCPath) (Variables|Default|GetNPCPathIndex)))) "NewEnumerator1")
        (Utilities|FlowControl|Delay 5.0))
      (Math|Integer|IncrementInt (Variables|Default|GetNPCPathIndex)
        (:%20%20
          (if (>= (Variables|Default|GetNPCPathIndex) (Utilities|Array|Length (Variables|Default|GetNPCPath)))
            (Variables|Default|SetNPCPathIndex 0)
            (CallFunction|Move)
            (else
              (CallFunction|Move))))))))

(event Custom|NewMove
  (AI|AIMoveTo (Pawn|GetControlledPawn (Pawn|GetController)) (Transformation|GetWorldLocation (Variables|/Script/Engine.TargetPoint|GetSpriteComponent (Variables|Default|GetCurrentLocation))) 0 5.0 false
    (:OnSuccess
      (if (Utilities|Enum|Equal(Enum) (Variables|/Game/OctoInkContent/Blueprints/Actors/NPCs/BP_WaypointComponent.BP_WaypointComponent_C|GetPlayerAction (Actor|GetComponentbyClass (Variables|Default|GetCurrentLocation) "/Game/OctoInkContent/Blueprints/Actors/NPCs/BP_WaypointComponent.BP_WaypointComponent_C")) "NewEnumerator1")
        (Utilities|FlowControl|Delay 5.0))
      (CallFunction|CalculatePath))))

(event EventBeginPlay
  (Class|SpineSkeletonAnimationComponent|SetAnimation (Variables|Default|GetSpineSkeletonAnimation) 0 "Walk" true)
  (Class|SpineSkeletonComponent|SetSkin (Variables|Default|GetSpineSkeletonAnimation) (.OutItem (Utilities|Array|Random (Variables|Default|GetRandomNPCSkins)))))

(event Collision|EventActorBeginOverlap
  (params (OtherActor :type Actor%20Object%20Reference)))

(event EventTick
  (params (DeltaSeconds :type Float%20%28single-precision%29)))

(fn ConstructionScript
  (Variables|/Script/Engine.CharacterMovementComponent|SetMaxWalkSpeed (Variables|Character|GetCharacterMovement) (Math|Random|RandomFloatinRange 4e+02 5e+02)))

(fn CalculatePath
  (bind _spineskeletonrenderer (Variables|Default|GetSpineSkeletonRenderer))
  (bind _possiblelocations (Variables|Default|GetPossibleLocations))
  (for _array_element (Variables|Default|GetWaypoints)
    (if (== (Variables|Default|GetCurrentLocation) (.Node1 (Utilities|Struct|BreakNPCWaypoints _array_element)))
      (Utilities|Array|Add _possiblelocations (.Node2 (Utilities|Struct|BreakNPCWaypoints _array_element)))
      (elif (== (.Node2 (Utilities|Struct|BreakNPCWaypoints _array_element)) (Variables|Default|GetCurrentLocation))
        (Utilities|Array|Add _possiblelocations (.Node1 (Utilities|Struct|BreakNPCWaypoints _array_element))))))
  (LocalVariables|SetChosenLocation (.OutItem (Utilities|Array|Random (Variables|Default|GetPossibleLocations))))
  (Utilities|FlowControl|Sequence
    (:then_0
      (if (>= (.y (- (Transformation|GetWorldLocation (Variables|/Script/Engine.TargetPoint|GetSpriteComponent (LocalVariables|GetChosenLocation))) (Transformation|GetWorldLocation (Variables|/Script/Engine.TargetPoint|GetSpriteComponent (Variables|Default|GetCurrentLocation))))) 0.0)
        (Transformation|SetWorldRotation _spineskeletonrenderer "0,-130.000000, 0" false false)
        (else
          (Transformation|SetWorldRotation _spineskeletonrenderer "0,50.000000, 0" false false))))
    (:then_1
      (Variables|Default|SetCurrentLocation (LocalVariables|GetChosenLocation))
      (CallFunction|NewMove))))