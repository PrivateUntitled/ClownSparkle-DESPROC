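; Onboarding elder NPC, a Spine-animated character that gives dialogue and a commission during the tutorial.
; It listens for the game mode's dialogue-finished event; after the first stage's dialogue it briefly locks movement, plays a skill animation, turns gray, hides its commissioner widget and inks the bridge.
; Interacting at the matching stage freezes the player and swaps all widgets for the commission panel.
; A separate function starts the commission dialogue through the game mode.
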(event Custom|InkBridge
  (params (Dialogue :type Onboarding%20Struct%20Structure))
  (bind _spineskeletonanimation (Variables|Default|GetSpineSkeletonAnimation))
  (if (Utilities|Enum|Equal(Enum) (Utilities|Struct|BreakOnboardingStruct Dialogue) "NewEnumerator0")
    (bind _asbp_onboarding_game_mode (Utilities|Casting|CastToBP_OnboardingGameMode (Game|GetGameMode)))
    (bind _asbp_player_base_controller (Utilities|Casting|CastToBP_PlayerBaseController (Game|GetPlayerController 0)))
    (Variables|/Game/OctoInkContent/Blueprints/Controllers/BP_PlayerBaseController.BP_PlayerBaseController_C|SetEnableMovement _asbp_player_base_controller false)
    (Class|SpineSkeletonAnimationComponent|SetAnimation _spineskeletonanimation 0 "skill" false)
    (Utilities|FlowControl|Delay 0.5)
    (Variables|/Game/OctoInkContent/Blueprints/Controllers/BP_PlayerBaseController.BP_PlayerBaseController_C|SetEnableMovement _asbp_player_base_controller true)
    (Class|SpineSkeletonComponent|SetSkin _spineskeletonanimation "gray elder")
    (Class|SpineSkeletonAnimationComponent|SetAnimation _spineskeletonanimation 0 "idle" true)
    (bind _asbp_commissioner_ui (Utilities|Casting|CastToBP_CommissionerUI (UserInterface|GetUserWidgetObject (Variables|Default|GetWidget))))
    (Widget|SetRenderOpacity _asbp_commissioner_ui 0.0)
    (Default|SetObstacleColor (Variables|/Game/OctoInkContent/Blueprints/GameMode/CommissionGameModes/BP_OnboardingGameMode.BP_OnboardingGameMode_C|GetBridgeRef _asbp_onboarding_game_mode) (Variables|Default|GetSet%20Color))
    (Audio|PlaySound2D "/Game/OctoInkContent/Assets/SFX/sounds/Ink.Ink" 1.0 1.0 0.0 0 0)))

(event EventBeginPlay
  (|CallParentFunction)
  (Class|SpineSkeletonComponent|SetSkin (Variables|Default|GetSpineSkeletonAnimation) "default elder")
  (bind _asbp_onboarding_game_mode (Utilities|Casting|CastToBP_OnboardingGameMode (Game|GetGameMode)))
  (EventDispatchers|BindEventtoDialogueFinished _asbp_onboarding_game_mode (delegate Custom|InkBridge)))

(event Collision|EventActorBeginOverlap
  (params (OtherActor :type Actor%20Object%20Reference))
  (|CallParentFunction OtherActor) ; This node is disabled and will not be called.\nDrag off pins to build functionality.
)

(event EventTick
  (params (DeltaSeconds :type Float%20%28single-precision%29))
  (|CallParentFunction DeltaSeconds) ; This node is disabled and will not be called.\nDrag off pins to build functionality.
)

(event EventDoInteraction
  (bind _returnvalue (Game|GetPlayerController 0))
  (bind _asbp_onboarding_game_mode (Utilities|Casting|CastToBP_OnboardingGameMode (Game|GetGameMode)))
  (if (== (Variables|/Game/OctoInkContent/Blueprints/GameMode/CommissionGameModes/BP_OnboardingGameMode.BP_OnboardingGameMode_C|GetNextStage _asbp_onboarding_game_mode) 1)
    (Utilities|FlowControl|Sequence
      (:then_0
        ;[1 1 1] Setting Movement
        (bind _asbp_player_base_controller (Utilities|Casting|CastToBP_PlayerBaseController _returnvalue))
        (Variables|/Game/OctoInkContent/Blueprints/Controllers/BP_PlayerBaseController.BP_PlayerBaseController_C|SetEnableMovement _asbp_player_base_controller false))
      (:then_1
        ;[1 1 1] Setting Mouse Cursor Visibility
        (Variables|/Script/Engine.PlayerController|SetbShowMouseCursor _returnvalue true))
      (:then_2
        (Viewport|RemoveAllWidgets))
      (:then_3
        ;[1 1 1] Adding New Widget
        (bind _returnvalue_2 (UserInterface|CreateWidget "/Game/OctoInkContent/Blueprints/Widgets/BP_CommissionPanel.BP_CommissionPanel_C"))
        (UserInterface|Viewport|AddtoViewport _returnvalue_2 0)))))

(fn ConstructionScript
  (|CallParentFunction))

(fn TalktoElder
  (bind _asbp_onboarding_game_mode (Utilities|Casting|CastToBP_OnboardingGameMode (Game|GetGameMode)))
  (Default|PlayDialogue _asbp_onboarding_game_mode (Variables|/Game/OctoInkContent/Blueprints/GameMode/CommissionGameModes/BP_OnboardingGameMode.BP_OnboardingGameMode_C|GetStartCommisisonDialogue _asbp_onboarding_game_mode)))