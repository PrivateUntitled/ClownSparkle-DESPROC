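; Commissioner NPC that plays dialogue and opens the commission panel, with dialogue branches for Hannah, Nidas and Rio.
; Interaction picks first-time or regular dialogue by tutorial stage, then the dialogue-finished callback advances that stage on first meetings and switches to the panel or main-world HUD.
; It also listens for finished commissions through the main world game mode, playing win dialogue on a commission's first completion.
; On BeginPlay it rotates its widget using the player's sprite-to-camera direction.
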(event Custom|CheckDialogue
  (params (DialogueType :type DialogueType%20Enum :default "NewEnumerator6"))
  (bind _gameinstanceref (Variables|Default|GetGameInstanceRef))
  (bind _tutorialdata (Variables|/Game/OctoInkContent/Blueprints/SaveData/MyGame.MyGame_C|GetTutorialData _gameinstanceref))
  (switch Utilities|FlowControl|Switch|SwitchonDialogueType DialogueType
    (:NewEnumerator17
      (Utilities|Struct|SetmembersinTutorialData _tutorialdata "NewEnumerator12")
      (Default|SettingWidget (Variables|Default|GetMainWorldRef) true true "/Game/OctoInkContent/Blueprints/Widgets/BP_CommissionPanel.BP_CommissionPanel_C" :!label _label))
    (:NewEnumerator18
      (goto _label))
    (:NewEnumerator19
      (Default|SettingWidget (Variables|Default|GetMainWorldRef) false false "/Game/OctoInkContent/Blueprints/Widgets/MainWorld/BP_TempMainWorldHUD.BP_TempMainWorldHUD_C" :!label _label_2))
    (:NewEnumerator20
      (Utilities|Struct|SetmembersinTutorialData _tutorialdata "NewEnumerator15")
      (goto _label))
    (:NewEnumerator22
      (goto _label_2))
    (:NewEnumerator21
      (goto _label))
    (:NewEnumerator27
      (Utilities|Struct|SetmembersinTutorialData _tutorialdata "NewEnumerator17")
      (goto _label))
    (:NewEnumerator28
      (goto _label))
    (:NewEnumerator29
      (goto _label_2))))

(event Custom|CustomEvent_1
  (params (Commission :type Commission%20Enum :default "NewEnumerator0"))
  (bind _asmy_game (Utilities|Casting|CastToMyGame (Game|GetGameInstance)))
  (switch Utilities|FlowControl|Switch|SwitchonCommission Commission
    (:NewEnumerator0
      (if (== (.Commision1Completions (Utilities|Struct|BreakCommissionData (Variables|/Game/OctoInkContent/Blueprints/SaveData/MyGame.MyGame_C|GetCommissionData _asmy_game))) 1)
        (Default|SettingWidget (Variables|Default|GetMainWorldRef) false true "/Game/OctoInkContent/Blueprints/Widgets/MainWorld/BP_DialogueHUD.BP_DialogueHUD_C" :!label _label)
        (Default|PlayDialogue (Variables|Default|GetMainWorldRef) (Variables|Default|GetFirstWinDialogue))
        (EventDispatchers|BindEventtoDialogueFinished (Variables|Default|GetMainWorldRef) (EventDispatchers|CreateEvent :!event Custom|CheckDialogue))))
    (:NewEnumerator1
      (if (== (.Commision2Completions (Utilities|Struct|BreakCommissionData (Variables|/Game/OctoInkContent/Blueprints/SaveData/MyGame.MyGame_C|GetCommissionData _asmy_game))) 1)
        (goto _label)))
    (:NewEnumerator2
      (if (== (.Commision3Completions (Utilities|Struct|BreakCommissionData (Variables|/Game/OctoInkContent/Blueprints/SaveData/MyGame.MyGame_C|GetCommissionData _asmy_game))) 1)
        (goto _label)))))

(event EventBeginPlay
  (|CallParentFunction)
  (bind _asbp_puzzle_player (Utilities|Casting|CastToBP_PuzzlePlayer (Game|Player|GetPlayerPawn 0)))
  (Transformation|SetWorldRotation (Variables|Default|GetWidget) (Math|Rotator|FindLookatRotation (Transformation|GetWorldLocation (Variables|/Script/Paper2D.PaperCharacter|GetSprite _asbp_puzzle_player)) (Transformation|GetWorldLocation (Variables|/Game/OctoInkContent/Blueprints/Actors/Player/BP_BasePlayer.BP_BasePlayer_C|GetCamera _asbp_puzzle_player))) false false)
  (bind _asbp_main_world (Utilities|Casting|CastToBP_MainWorld (Game|GetGameMode)))
  (Variables|Default|SetMainWorldRef _asbp_main_world)
  (bind _asmy_game (Utilities|Casting|CastToMyGame (Game|GetGameInstance)))
  (Variables|Default|SetGameInstanceRef _asmy_game)
  (EventDispatchers|BindEventtoFinishedCommission (Variables|Default|GetMainWorldRef) (delegate Custom|CustomEvent_1)))

(event Collision|EventActorBeginOverlap
  (params (OtherActor :type Actor%20Object%20Reference))
  (|CallParentFunction OtherActor) ; This node is disabled and will not be called.\nDrag off pins to build functionality.
)

(event EventTick
  (params (DeltaSeconds :type Float%20%28single-precision%29))
  (|CallParentFunction DeltaSeconds) ; This node is disabled and will not be called.\nDrag off pins to build functionality.
)

(event EventDoInteraction
  (bind _gameinstanceref (Variables|Default|GetGameInstanceRef))
  (bind _tutorialdata (Variables|/Game/OctoInkContent/Blueprints/SaveData/MyGame.MyGame_C|GetTutorialData _gameinstanceref))
  (bind _tutorialstage (Utilities|Struct|BreakTutorialData _tutorialdata))
  (Viewport|RemoveAllWidgets)
  (Utilities|FlowControl|Sequence
    (:then_0
      (Default|SettingWidget (Variables|Default|GetMainWorldRef) false true "/Game/OctoInkContent/Blueprints/Widgets/MainWorld/BP_DialogueHUD.BP_DialogueHUD_C")
      (Development|PrintString (Utilities|String|EnumtoString _tutorialstage))
      (if (Utilities|Enum|Equal(Enum) _tutorialstage (Variables|Default|GetTutorialState))
        (Default|PlayDialogue (Variables|Default|GetMainWorldRef) (Variables|Default|GetFirstTimeDialogue))
        (else
          (Default|PlayDialogue (Variables|Default|GetMainWorldRef) (Variables|Default|GetRegularDialogue)))))
    (:then_1
      (EventDispatchers|BindEventtoDialogueFinished (Variables|Default|GetMainWorldRef) (delegate Custom|CheckDialogue)))))

(fn ConstructionScript
  (|CallParentFunction))