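; Tutorial lesson NPC that plays first-time or filler dialogue on interaction, depending on the game instance's tutorial stage.
; Game-mode delegates trigger closing dialogue on IB completion and route finished dialogues by type across the Sunni, Elder and Inna branches.
; These branches swap HUDs, show tutorial tasks, advance stages, toggle commissioner visibility and lock World 2 obstacles.
; Player interactable events toggle its prompt widget, angled toward the camera at BeginPlay.
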(event Custom|FinishedDialogue
  (params (DialogueType :type DialogueType%20Enum :default "NewEnumerator6"))
  (bind _mainworldref (Variables|Default|GetMainWorldRef))
  (switch Utilities|FlowControl|Switch|SwitchonDialogueType DialogueType
    (:NewEnumerator15
      (Default|SettingWidget (Variables|Default|GetMainWorldRef) false false "/Game/OctoInkContent/Blueprints/Widgets/BP_TutorialTasks.BP_TutorialTasks_C")
      (Default|PrintTutorialText (Variables|Default|GetMainWorldRef) "/Game/OctoInkContent/DataAssets/DataAssets/Lessons/DA_InspirationTutorial.DA_InspirationTutorial"))
    (:NewEnumerator31
      (Default|SettingWidget (Variables|Default|GetMainWorldRef) false false "/Game/OctoInkContent/Blueprints/Widgets/MainWorld/BP_TempMainWorldHUD.BP_TempMainWorldHUD_C"))
    (:NewEnumerator16
      (Default|SettingWidget (Variables|Default|GetMainWorldRef) false false "/Game/OctoInkContent/Blueprints/Widgets/MainWorld/BP_TempMainWorldHUD.BP_TempMainWorldHUD_C")
      (Utilities|Struct|SetmembersinTutorialData (Variables|/Game/OctoInkContent/Blueprints/SaveData/MyGame.MyGame_C|GetTutorialData (Variables|Default|GetGameInstanceRef)) "NewEnumerator11")
      (bind _asbp_world_1game_mode (Utilities|Casting|CastToBP_World1GameMode (Game|GetGameMode)))
      (Default|SetCommissionerVisibility _asbp_world_1game_mode false))
    (:NewEnumerator23
      (bind _returnvalue (UserInterface|CreateWidget "/Game/OctoInkContent/Blueprints/BP_YesNoButton.BP_YesNoButton_C"))
      (Variables|/Game/OctoInkContent/Blueprints/BP_YesNoButton.BP_YesNoButton_C|SetDialogueType _returnvalue DialogueType)
      (UserInterface|Viewport|AddtoViewport _returnvalue 0)
      (Variables|/Script/Engine.PlayerController|SetbShowMouseCursor (Game|GetPlayerController 0) true))
    (:NewEnumerator35
      (bind _asbp_world_2game_mode (Utilities|Casting|CastToBP_World2GameMode (Game|GetGameMode)))
      (Default|OpenMixingGuideTask _asbp_world_2game_mode)
      (Variables|/Game/OctoInkContent/Blueprints/Actors/Obstacles/BP_Obstacle.BP_Obstacle_C|SetCanInk (Utilities|Array|Get(acopy) (Variables|/Game/OctoInkContent/Blueprints/GameMode/WorldGameModes/BP_BaseWorldGameMode.BP_BaseWorldGameMode_C|GetObstacles _asbp_world_2game_mode) 1) false)
      (bind _asbp_obstacle_pointer (Utilities|Casting|CastToBP_ObstaclePointer (UserInterface|GetWidget (Variables|/Game/OctoInkContent/Blueprints/Actors/Obstacles/BP_Obstacle.BP_Obstacle_C|GetWidget (Utilities|Array|Get(acopy) (Variables|/Game/OctoInkContent/Blueprints/GameMode/WorldGameModes/BP_BaseWorldGameMode.BP_BaseWorldGameMode_C|GetObstacles _asbp_world_2game_mode) 1)))))
      (Default|HideLock _asbp_obstacle_pointer true))
    (:NewEnumerator36
      (Default|SettingWidget (Variables|Default|GetMainWorldRef) false false "/Game/OctoInkContent/Blueprints/Widgets/BP_TutorialTasks.BP_TutorialTasks_C")
      (Default|PrintTutorialText _mainworldref "/Game/OctoInkContent/DataAssets/DataAssets/Lessons/DA_MixingIcebreaker.DA_MixingIcebreaker")
      (bind _asbp_world_2game_mode_2 (Utilities|Casting|CastToBP_World2GameMode _mainworldref))
      (Variables|/Game/OctoInkContent/Blueprints/Actors/Obstacles/BP_Obstacle.BP_Obstacle_C|SetCanInk (Utilities|Array|Get(acopy) (Variables|/Game/OctoInkContent/Blueprints/GameMode/WorldGameModes/BP_BaseWorldGameMode.BP_BaseWorldGameMode_C|GetObstacles _asbp_world_2game_mode_2) 1) true)
      (bind _asbp_obstacle_pointer_2 (Utilities|Casting|CastToBP_ObstaclePointer (UserInterface|GetWidget (Variables|/Game/OctoInkContent/Blueprints/Actors/Obstacles/BP_Obstacle.BP_Obstacle_C|GetWidget (Utilities|Array|Get(acopy) (Variables|/Game/OctoInkContent/Blueprints/GameMode/WorldGameModes/BP_BaseWorldGameMode.BP_BaseWorldGameMode_C|GetObstacles _asbp_world_2game_mode_2) 1)))))
      (Default|HideLock _asbp_obstacle_pointer_2 false))
    (:NewEnumerator24
      (Default|SettingWidget (Variables|Default|GetMainWorldRef) false false "/Game/OctoInkContent/Blueprints/Widgets/MainWorld/BP_TempMainWorldHUD.BP_TempMainWorldHUD_C"))
    (:NewEnumerator32
      (Default|SettingWidget (Variables|Default|GetMainWorldRef) false false "/Game/OctoInkContent/Blueprints/Widgets/MainWorld/BP_TempMainWorldHUD.BP_TempMainWorldHUD_C")
      (Utilities|Struct|SetmembersinTutorialData (Variables|/Game/OctoInkContent/Blueprints/SaveData/MyGame.MyGame_C|GetTutorialData (Variables|Default|GetGameInstanceRef)) "NewEnumerator13")
      (bind _asbp_world_2game_mode_3 (Utilities|Casting|CastToBP_World2GameMode (Game|GetGameMode)))
      (Default|SetCommissionerVisibility _asbp_world_2game_mode_3 false))
    (:NewEnumerator26
      (Default|SettingWidget (Variables|Default|GetMainWorldRef) false false "/Game/OctoInkContent/Blueprints/Widgets/MainWorld/BP_TempMainWorldHUD.BP_TempMainWorldHUD_C")
      (Utilities|Struct|SetmembersinTutorialData (Variables|/Game/OctoInkContent/Blueprints/SaveData/MyGame.MyGame_C|GetTutorialData (Variables|Default|GetGameInstanceRef)) "NewEnumerator16")
      (CallFunction|SetCommissionerVisibility false))
    (:NewEnumerator25
      (Default|SettingWidget (Variables|Default|GetMainWorldRef) false false "/Game/OctoInkContent/Blueprints/Widgets/BP_TutorialTasks.BP_TutorialTasks_C")
      (Default|PrintTutorialText (Variables|Default|GetMainWorldRef) "/Game/OctoInkContent/DataAssets/DataAssets/Lessons/DA_VerticalTutorial.DA_VerticalTutorial"))
    (:NewEnumerator33
      (Default|SettingWidget (Variables|Default|GetMainWorldRef) false false "/Game/OctoInkContent/Blueprints/Widgets/MainWorld/BP_TempMainWorldHUD.BP_TempMainWorldHUD_C"))))

(event Custom|IBComplete
  (Default|SettingWidget (Variables|Default|GetMainWorldRef) false true "/Game/OctoInkContent/Blueprints/Widgets/MainWorld/BP_DialogueHUD.BP_DialogueHUD_C")
  (Default|PlayDialogue (Variables|Default|GetMainWorldRef) (Variables|Default|GetFinishDialogue))
  (EventDispatchers|BindEventtoDialogueFinished (Variables|Default|GetMainWorldRef) (EventDispatchers|CreateEvent :!event Custom|FinishedDialogue)))

(event EventBeginPlay
  (|CallParentFunction)
  (bind _asmy_game (Utilities|Casting|CastToMyGame (Game|GetGameInstance)))
  (Variables|Default|SetGameInstanceRef _asmy_game)
  (bind _asbp_puzzle_player (Utilities|Casting|CastToBP_PuzzlePlayer (Game|Player|GetPlayerPawn 0)))
  (Transformation|SetWorldRotation (Variables|Default|GetWidget) (Math|Rotator|FindLookatRotation (Transformation|GetWorldLocation (Variables|/Script/Paper2D.PaperCharacter|GetSprite _asbp_puzzle_player)) (Transformation|GetWorldLocation (Variables|/Game/OctoInkContent/Blueprints/Actors/Player/BP_BasePlayer.BP_BasePlayer_C|GetCamera _asbp_puzzle_player))) false false)
  (bind _asbp_base_world_game_mode (Utilities|Casting|CastToBP_BaseWorldGameMode (Game|GetGameMode)))
  (bind _output_get (Variables|Default|SetMainWorldRef _asbp_base_world_game_mode))
  (EventDispatchers|BindEventtoDialogueFinished _output_get (EventDispatchers|CreateEvent :!event Custom|FinishedDialogue))
  (EventDispatchers|BindEventtoIBCompleted _asbp_base_world_game_mode (delegate Custom|IBComplete))
  (bind _asbp_base_player (Utilities|Casting|CastToBP_BasePlayer (Game|Player|GetPlayerPawn 0)))
  (EventDispatchers|BindEventtoOnEnterInteractable _asbp_base_player (EventDispatchers|CreateEvent :!event BPBusStopAutoGenFunc))
  (EventDispatchers|BindEventtoOnExitInteractable _asbp_base_player (EventDispatchers|CreateEvent :!event BPBusStopAutoGenFunc1)))

(event Collision|EventActorBeginOverlap
  (params (OtherActor :type Actor%20Object%20Reference))
  (|CallParentFunction OtherActor) ; This node is disabled and will not be called.\nDrag off pins to build functionality.
)

(event EventTick
  (params (DeltaSeconds :type Float%20%28single-precision%29))
  (|CallParentFunction DeltaSeconds) ; This node is disabled and will not be called.\nDrag off pins to build functionality.
)

(event EventDoInteraction
  (|CallParentFunction)
  (bind _asbp_player_base_controller (Utilities|Casting|CastToBP_PlayerBaseController (Game|GetPlayerController 0)))
  (if (not (Variables|/Game/OctoInkContent/Blueprints/Controllers/BP_PlayerBaseController.BP_PlayerBaseController_C|GetInDialogue _asbp_player_base_controller))
    (Variables|/Game/OctoInkContent/Blueprints/Controllers/BP_PlayerBaseController.BP_PlayerBaseController_C|SetInDialogue _asbp_player_base_controller true)
    (bind _asbp_main_world (Utilities|Casting|CastToBP_MainWorld (Game|GetGameMode)))
    (Default|SettingWidget _asbp_main_world false true "/Game/OctoInkContent/Blueprints/Widgets/MainWorld/BP_DialogueHUD.BP_DialogueHUD_C")
    (if (Utilities|Enum|Equal(Enum) (.TutorialStage (Utilities|Struct|BreakTutorialData (Variables|/Game/OctoInkContent/Blueprints/SaveData/MyGame.MyGame_C|GetTutorialData (Variables|Default|GetGameInstanceRef)))) (Variables|Default|GetTutorialState))
      (Default|PlayDialogue _asbp_main_world (Variables|Default|GetFirstTimeDialogue))
      (else
        (Default|PlayDialogue _asbp_main_world (Variables|Default|GetFillerDialogue))))))

(fn ConstructionScript
  (|CallParentFunction))

(fn SetCommissionerVisibility
  (params (HidePerson :type Boolean))
  (bind _returnvalue (not HidePerson))
  (bind _self self)
  (bind _capsulecomponent (Variables|/Script/Engine.Character|GetCapsuleComponent _self))
  (Development|SetHiddeninGame _capsulecomponent HidePerson true)
  (Collision|SetActorEnableCollision _self _returnvalue)
  (Actor|Tick|SetActorTickEnabled _self _returnvalue)
  (Development|SetHiddeninGame _capsulecomponent true false))

(fn BPBusStopAutoGenFunc
  (params (ItemEntered :type Actor%20Object%20Reference))
  (if (== ItemEntered self)
    (bind _asbp_ib_lesson_ui (Utilities|Casting|CastToBP_IB_LessonUI (UserInterface|GetUserWidgetObject (Variables|Default|GetWidget))))
    (Widget|SetVisibility (Variables|/Game/OctoInkContent/Blueprints/Widgets/BP_IB_LessonUI.BP_IB_LessonUI_C|GetImage_1 _asbp_ib_lesson_ui) "Visible")))

(fn BPBusStopAutoGenFunc1
  (params (ItemExited :type Actor%20Object%20Reference))
  (if (== ItemExited self)
    (bind _asbp_ib_lesson_ui (Utilities|Casting|CastToBP_IB_LessonUI (UserInterface|GetUserWidgetObject (Variables|Default|GetWidget))))
    (Widget|SetVisibility (Variables|/Game/OctoInkContent/Blueprints/Widgets/BP_IB_LessonUI.BP_IB_LessonUI_C|GetImage_1 _asbp_ib_lesson_ui) "Hidden")))