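; Base NPC actor that loops a Spine "swim" animation and patrols waypoints through AI MoveTo.
; Move cycles through the ordered NPCPath, while NewMove wanders a waypoint graph, each pausing at points flagged by an action enum.
; CalculatePath gathers nodes linked to CurrentLocation from Waypoints edge pairs, picks one at random and calls NewMove again.
; Neither movement routine is started within this Blueprint.
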(event Custom|Move
  (AI|AIMoveTo (Pawn|GetControlledPawn (Pawn|GetController)) (Transformation|GetWorldLocation (Variables|/Script/Engine.TargetPoint|GetSpriteComponent (.Location (Utilities|Struct|BreakNPCPath (Utilities|Array|Get(acopy) (Variables|Default|GetNPCPath) (Variables|Default|GetNPCPathIndex)))))) 0 5.0 false
    (:OnSuccess
      (if (Utilities|Enum|Equal(Enum) (.Action (Utilities|Struct|BreakNPCPath (Utilities|Array|Get(acopy) (Variables|Default|GetNPCPath) (Variables|Default|GetNPCPathIndex)))) "NewEnumerator1")
        (Utilities|FlowControl|Delay 5.0))
      (Math|Integer|IncrementInt (Variables|Default|GetNPCPathIndex)
        (:%20%20
          (if (>= (Variables|Default|GetNPCPathIndex) (Utilities|Array|Length (Variables|Default|GetNPCPath)))
            (Variables|Default|SetNPCPathIndex 0)
            (CallFunction|Move)
            (else
              (CallFunction|Move))))))))

(event Custom|NewMove
  (bind _currentlocation (Variables|Default|GetCurrentLocation))
  (AI|AIMoveTo (Pawn|GetControlledPawn (Pawn|GetController)) "0, 0, 0" _currentlocation 5.0 false
    (:OnSuccess
      (if (Utilities|Enum|Equal(Enum) (Variables|/Game/OctoInkContent/Blueprints/Actors/NPCs/BP_WaypointComponent.BP_WaypointComponent_C|GetPlayerAction (Actor|GetComponentbyClass _currentlocation "/Game/OctoInkContent/Blueprints/Actors/NPCs/BP_WaypointComponent.BP_WaypointComponent_C")) "NewEnumerator1")
        (Utilities|FlowControl|Delay 5.0))
      (CallFunction|CalculatePath))))

(event EventBeginPlay
  (Class|SpineSkeletonAnimationComponent|SetAnimation (Variables|Default|GetSpineSkeletonAnimation) 0 "swim" true))

(event Collision|EventActorBeginOverlap
  (params (OtherActor :type Actor%20Object%20Reference)))

(event EventTick
  (params (DeltaSeconds :type Float%20%28single-precision%29)))

(fn ConstructionScript)

(fn CalculatePath
  (bind _possiblelocations (Variables|Default|GetPossibleLocations))
  (for _array_element (Variables|Default|GetWaypoints)
    (if (== (Variables|Default|GetCurrentLocation) (.Node1 (Utilities|Struct|BreakNPCWaypoints _array_element)))
      (Utilities|Array|Add _possiblelocations (.Node2 (Utilities|Struct|BreakNPCWaypoints _array_element)))
      (elif (== (.Node2 (Utilities|Struct|BreakNPCWaypoints _array_element)) (Variables|Default|GetCurrentLocation))
        (Utilities|Array|Add _possiblelocations (.Node1 (Utilities|Struct|BreakNPCWaypoints _array_element))))))
  (Variables|Default|SetCurrentLocation (.OutItem (Utilities|Array|Random (Variables|Default|GetPossibleLocations))))
  (CallFunction|NewMove))