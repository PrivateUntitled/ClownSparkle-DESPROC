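; BP_Piano is an interactable main-world piano that launches the BP_Minigame1 widget on interaction, passing itself to it.
; Each Tick it shows the icon widget's E prompt when it is the player's QuestInRange and the game mode allows minigames.
; Unconnected leftover nodes hold an older play-instrument routine that locks movement, plays sound and animation, and restores energy in timed steps, with a Sax mesh reference.
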(event Custom|OnExit
  (|CallParentFunction))

(event EventTick
  (params (DeltaSeconds :type Float%20%28single-precision%29))
  (|CallParentFunction DeltaSeconds)
  (bind _asbp_main_world (Utilities|Casting|CastToBP_MainWorld (Game|GetGameMode)))
  (bind _asbp_main_game_player (Utilities|Casting|CastToBP_MainGamePlayer (Game|Player|GetPlayerPawn 0)))
  (bind _asbp_minigame_icon (Utilities|Casting|CastToBP_MinigameIcon (UserInterface|GetWidget (Variables|Default|GetWidget))))
  (Default|ShowE _asbp_minigame_icon (and (== (Variables|/Game/OctoInkContent/Blueprints/Actors/Player/BP_MainGamePlayer.BP_MainGamePlayer_C|GetQuestInRange _asbp_main_game_player) self) (Variables|/Game/OctoInkContent/Blueprints/GameMode/BP_MainWorld.BP_MainWorld_C|GetCanPlayMinigames _asbp_main_world))))

(event EventDoInteraction
  (|CallParentFunction)
  (bind _returnvalue (UserInterface|CreateWidget "/Game/OctoInkContent/Blueprints/Widgets/Minigames/Minigames1/BP_Minigame1.BP_Minigame1_C"))
  (Default|Init _returnvalue self)
  (UserInterface|Viewport|AddtoViewport _returnvalue 0))

(event EventBeginPlay
  (|CallParentFunction))

(fn ConstructionScript)