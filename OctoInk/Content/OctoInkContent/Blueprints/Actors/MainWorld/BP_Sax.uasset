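; Interactable saxophone in the main world that launches a minigame.
; On BeginPlay its three meshes write custom depth with a shared stencil value.
; When the game mode allows minigames, interaction clears widgets, opens BP_Minigame1, shows the cursor, sets IsOnMinigame2 on the controller and disables player movement.
; A disconnected legacy graph plays the sax with animation and sound while restoring energy over timed loops.
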(event Custom|OnExit
  (|CallParentFunction))

(event EventDoInteraction
  (bind _returnvalue (Game|GetPlayerController 0))
  (|CallParentFunction)
  (bind _asbp_main_world (Utilities|Casting|CastToBP_MainWorld (Game|GetGameMode)))
  (if (Variables|/Game/OctoInkContent/Blueprints/GameMode/BP_MainWorld.BP_MainWorld_C|GetCanPlayMinigames _asbp_main_world)
    (Viewport|RemoveAllWidgets)
    (Variables|/Script/Engine.PlayerController|SetbShowMouseCursor _returnvalue true)
    (bind _returnvalue_2 (UserInterface|CreateWidget "/Game/OctoInkContent/Blueprints/Widgets/Minigames/Minigames1/BP_Minigame1.BP_Minigame1_C"))
    (Default|Init _returnvalue_2 self)
    (bind _asbp_player_main_game_controller (Utilities|Casting|CastToBP_PlayerMainGameController _returnvalue))
    (Variables|/Game/OctoInkContent/Blueprints/Controllers/BP_PlayerMainGameController.BP_PlayerMainGameController_C|SetisOnMinigame2 _asbp_player_main_game_controller true)
    (UserInterface|Viewport|AddtoViewport _returnvalue_2 0)
    (Variables|/Game/OctoInkContent/Blueprints/Controllers/BP_PlayerBaseController.BP_PlayerBaseController_C|SetEnableMovement (Variables|Default|GetPlayerControllerRef) false)))

(event EventBeginPlay
  (|CallParentFunction)
  (for _array_element (Utilities|Array|MakeArray (Variables|Default|GetStaticMesh) (Variables|Default|GetStaticMesh1) (Variables|Default|GetStaticMesh2))
    (Rendering|SetRenderCustomDepth _array_element true)
    (Rendering|SetCustomDepthStencilValue _array_element 5)))

(fn ConstructionScript)