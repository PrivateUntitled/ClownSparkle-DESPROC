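; Base interactable actor for main-world minigames, with a widget icon that shows its prompt when the player enters range.
; DoInteraction checks minigame availability, then calls OnWin on debug instant-win or locks movement and starts a recursive Delay-based timer.
; OnWin restores the HUD, optionally adds CurrentTime to the day clock, grants status-scaled energy and rolls for Inspiration with notifications.
; Movement unlocks afterward, waiting on the animator transition when energy crosses 50.
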(event Custom|Timer
  (if (not (Variables|/Game/OctoInkContent/Blueprints/Controllers/BP_PlayerBaseController.BP_PlayerBaseController_C|GetisOnMinigame (Variables|Default|GetPlayerControllerRef)))
    (bind _asbp_player_base_controller (Utilities|Casting|CastToBP_PlayerBaseController (Game|GetPlayerController 0)))
    (if (or (Variables|/Game/OctoInkContent/Blueprints/Controllers/BP_PlayerBaseController.BP_PlayerBaseController_C|GetisPauseMenuOpen _asbp_player_base_controller) (not (Utilities|Struct|BreakDebugData (Variables|/Game/OctoInkContent/Blueprints/SaveData/MyGame.MyGame_C|GetDebugData (Variables|Default|GetGameInstanceRef)))))
      ;[1 1 1] Dont Add Time if Game is Paused
      (Utilities|FlowControl|Delay 0.1)
      (CallFunction|Timer)
      (else
        (Math|Integer|IncrementInt (Variables|Default|GetCurrentTime)
          (:%20%20
            (Utilities|FlowControl|Delay 0.1)
            (CallFunction|Timer)))))))

(event Custom|CustomEvent
  (bind _asbp_player_base_controller (Utilities|Casting|CastToBP_PlayerBaseController (Game|GetPlayerController 0)))
  (Variables|/Game/OctoInkContent/Blueprints/Controllers/BP_PlayerBaseController.BP_PlayerBaseController_C|SetEnableMovement _asbp_player_base_controller true)
  (bind _asbp_player_main_game_controller (Utilities|Casting|CastToBP_PlayerMainGameController (Game|GetPlayerController 0)))
  (Variables|/Game/OctoInkContent/Blueprints/Controllers/BP_PlayerMainGameController.BP_PlayerMainGameController_C|SetisMinigameOpen _asbp_player_main_game_controller false)
  (Default|CallMinigamePopUpComplete))

(event Custom|OnWin
  (bind _gameinstanceref (Variables|Default|GetGameInstanceRef))
  (bind _maingamemoderef (Variables|Default|GetMainGameModeRef))
  (bind _gameinstanceref_2 (Variables|Default|GetGameInstanceRef))
  (bind _currenttime (Variables|Default|GetCurrentTime))
  (bind _gameinstanceref_3 (Variables|Default|GetGameInstanceRef))
  (bind _gameinstanceref_4 (Variables|Default|GetGameInstanceRef))
  (bind _gameinstanceref_5 (Variables|Default|GetGameInstanceRef))
  (bind _gamemodedata (Variables|/Game/OctoInkContent/Blueprints/SaveData/MyGame.MyGame_C|GetGameModeData _gameinstanceref_5))
  (bind _playerstats (Variables|/Game/OctoInkContent/Blueprints/SaveData/MyGame.MyGame_C|GetPlayerStats _gameinstanceref))
  (bind _playerstats_2 (Variables|/Game/OctoInkContent/Blueprints/SaveData/MyGame.MyGame_C|GetPlayerStats _gameinstanceref_3))
  (bind _playerstats_3 (Variables|/Game/OctoInkContent/Blueprints/SaveData/MyGame.MyGame_C|GetPlayerStats _gameinstanceref_2))
  (bind _inspirationdata (Variables|/Game/OctoInkContent/Blueprints/SaveData/MyGame.MyGame_C|GetInspirationData _gameinstanceref_4))
  (bind (_day _time _maxtime) (Utilities|Struct|BreakGameModeData _gamemodedata))
  (bind (_playerenergy _maxplayerenergy) (Utilities|Struct|BreakPlayerStats _playerstats_2))
  (bind (_playerenergy_2 _maxplayerenergy_2) (Utilities|Struct|BreakPlayerStats _playerstats))
  (bind (_playerenergy_3 _maxplayerenergy_3) (Utilities|Struct|BreakPlayerStats _playerstats_3))
  (bind _returnvalue (/ _currenttime _maxtime))
  (Utilities|FlowControl|Sequence
    (:then_0
      (Development|PrintString "Start")
      (if (Utilities|Struct|BreakTutorialData (Variables|/Game/OctoInkContent/Blueprints/SaveData/MyGame.MyGame_C|GetTutorialData (Variables|Default|GetGameInstanceRef)))
        (Default|SettingWidget _maingamemoderef false true "/Game/OctoInkContent/Blueprints/Widgets/MainWorld/BP_TempMainWorldHUD.BP_TempMainWorldHUD_C")
        (else
          (Default|SettingWidget _maingamemoderef false true "/Game/OctoInkContent/Blueprints/Widgets/BP_TutorialTasks.BP_TutorialTasks_C"))))
    (:then_1
      (if (Variables|Default|GetTrackTime)
        (Variables|/Game/OctoInkContent/Blueprints/GameMode/BP_MainWorld.BP_MainWorld_C|SetIsInMinigame (Variables|Default|GetMainGameModeRef) false)
        (Utilities|Struct|SetmembersinGameModeData _gamemodedata (+ _returnvalue _day) (+ _time (- _currenttime (* _returnvalue _maxtime))))))
    (:then_2
      (Utilities|FlowControl|Sequence
        (:then_0
          (bind _returnvalue_2 (Game|SpawnActorfromClass "/Game/OctoInkContent/Blueprints/Actors/MainWorld/BP_Notif.BP_Notif_C" (Math|Conversions|ToTransform(Vector) (Transformation|GetWorldLocation (Variables|/Game/OctoInkContent/Blueprints/Actors/Player/BP_BasePlayer.BP_BasePlayer_C|GetNotifSpawn (Variables|Default|GetMainGamePlayerRef)))) "Undefined" 0 0))
          (Default|SetText _returnvalue_2 "Task Completed!"))
        (:then_1
          (Utilities|FlowControl|Delay (Variables|Default|GetDuration))
          (if (!= _playerenergy_3 _maxplayerenergy_3)
            (Variables|Default|SetEnergyIncrease (Variables|Default|GetEnergyRecovered))
            (if (>= (Variables|Default|GetEnergyIncrease) 95.0)
              (Variables|Default|SetEnergyIncrease (Math|Conversions|ToFloat(Integer) (- _maxplayerenergy_2 _playerenergy_2))))
            ;[1 1 1] Day System - Energy Gain Reduction based on Status
            (switch Utilities|FlowControl|Switch|SwitchonEnergyStatus (Utilities|Struct|BreakPlayerStats (Variables|/Game/OctoInkContent/Blueprints/SaveData/MyGame.MyGame_C|GetPlayerStats (Variables|Default|GetGameInstanceRef)))
              (:NewEnumerator0
                _)
              (:NewEnumerator1
                (Variables|Default|SetEnergyIncrease (- (Variables|Default|GetEnergyIncrease) (* (Variables|Default|GetEnergyIncrease) 0.25))))
              (:NewEnumerator2
                (Variables|Default|SetEnergyIncrease (- (Variables|Default|GetEnergyIncrease) (* (Variables|Default|GetEnergyIncrease) 0.5)))))
            (bind _returnvalue_3 (Game|SpawnActorfromClass "/Game/OctoInkContent/Blueprints/Actors/MainWorld/BP_Notif.BP_Notif_C" (Math|Conversions|ToTransform(Vector) (Transformation|GetWorldLocation (Variables|/Game/OctoInkContent/Blueprints/Actors/Player/BP_BasePlayer.BP_BasePlayer_C|GetNotifSpawn (Variables|Default|GetMainGamePlayerRef)))) "Undefined" 0 0))
            (Default|SetText _returnvalue_3 (Utilities|Text|FormatText "{+}{Value}{%}" (Utilities|Text|ToText(String) "+") (Math|Float|Truncate (Variables|Default|GetEnergyIncrease)) (Utilities|Text|ToText(String) "Energy")))
            (Utilities|Struct|SetmembersinPlayerStats _playerstats_2 (Math|Float|Truncate (Math|Float|Clamp(Float) (+ (Math|Conversions|ToFloat(Integer) _playerenergy) (Variables|Default|GetEnergyIncrease)) 0.0 (Math|Conversions|ToFloat(Integer) _maxplayerenergy))))
            (Default|SetPlayerSpeed (Variables|Default|GetMainGamePlayerRef))
            (Utilities|FlowControl|Delay (Variables|Default|GetDuration)))
          (if (>= (Variables|Default|GetInspirationChance) (Math|Random|RandomIntegerinRange 0 100))
            (Utilities|Struct|SetmembersinInspirationData _inspirationdata (Utilities|Struct|BreakInspirationData _inspirationdata))
            (bind _returnvalue_4 (Game|SpawnActorfromClass "/Game/OctoInkContent/Blueprints/Actors/MainWorld/BP_Notif.BP_Notif_C" (Math|Conversions|ToTransform(Vector) (Transformation|GetWorldLocation (Variables|/Game/OctoInkContent/Blueprints/Actors/Player/BP_BasePlayer.BP_BasePlayer_C|GetNotifSpawn (Variables|Default|GetMainGamePlayerRef)))) "Undefined" 0 0))
            (Default|SetText _returnvalue_4 "Inspired")
            (Default|CallOnInspired (Variables|Default|GetMainGamePlayerRef)))
          (Utilities|Struct|SetmembersinPlayerStats (Variables|/Game/OctoInkContent/Blueprints/SaveData/MyGame.MyGame_C|GetPlayerStats (Variables|Default|GetGameInstanceRef)))
          (if (and (< (- (.PlayerEnergy (Utilities|Struct|BreakPlayerStats (Variables|/Game/OctoInkContent/Blueprints/SaveData/MyGame.MyGame_C|GetPlayerStats (Variables|Default|GetGameInstanceRef)))) (Math|Float|Truncate (Variables|Default|GetEnergyIncrease))) 50) (>= (.PlayerEnergy (Utilities|Struct|BreakPlayerStats (Variables|/Game/OctoInkContent/Blueprints/SaveData/MyGame.MyGame_C|GetPlayerStats (Variables|Default|GetGameInstanceRef)))) 50))
            (bind _asbp_player_animator (Utilities|Casting|CastToBP_PlayerAnimator (Variables|/Script/PaperZD.PaperZDCharacter|GetAnimInstance (Variables|Default|GetMainGamePlayerRef))))
            (EventDispatchers|BindEventtoTransitionDone _asbp_player_animator (delegate Custom|CustomEvent))
            (else
              (bind _asbp_player_base_controller (Utilities|Casting|CastToBP_PlayerBaseController (Game|GetPlayerController 0)))
              (Variables|/Game/OctoInkContent/Blueprints/Controllers/BP_PlayerBaseController.BP_PlayerBaseController_C|SetEnableMovement _asbp_player_base_controller true)
              (bind _asbp_player_main_game_controller (Utilities|Casting|CastToBP_PlayerMainGameController (Game|GetPlayerController 0)))
              (Variables|/Game/OctoInkContent/Blueprints/Controllers/BP_PlayerMainGameController.BP_PlayerMainGameController_C|SetisMinigameOpen _asbp_player_main_game_controller false)
              (Default|CallMinigamePopUpComplete))))))))

(event Custom|CustomEvent_0
  (params (ItemEntered :type Actor%20Object%20Reference))
  (if (== ItemEntered self)
    (bind _asbp_minigame_icon (Utilities|Casting|CastToBP_MinigameIcon (UserInterface|GetUserWidgetObject (Variables|Default|GetWidget))))
    (Default|ShowE _asbp_minigame_icon true)))

(event Custom|CustomEvent_2
  (params (ItemExited :type Actor%20Object%20Reference))
  (if (== ItemExited self)
    (bind _asbp_minigame_icon (Utilities|Casting|CastToBP_MinigameIcon (UserInterface|GetUserWidgetObject (Variables|Default|GetWidget))))
    (Default|ShowE _asbp_minigame_icon false)))

(event EventBeginPlay
  (|CallParentFunction)
  (bind _asmy_game (Utilities|Casting|CastToMyGame (Game|GetGameInstance)))
  (Variables|Default|SetGameInstanceRef _asmy_game)
  (Rendering|SetVisibility (Variables|Default|GetWidget) (Utilities|Struct|BreakMenuData (Variables|/Game/OctoInkContent/Blueprints/SaveData/MyGame.MyGame_C|GetGameStateData (Variables|Default|GetGameInstanceRef))) false)
  (bind _asbp_main_game_player (Utilities|Casting|CastToBP_MainGamePlayer (Game|Player|GetPlayerPawn 0)))
  (Variables|Default|SetMainGamePlayerRef _asbp_main_game_player)
  (Transformation|SetWorldRotation (Variables|Default|GetWidget) (Math|Rotator|FindLookatRotation (Transformation|GetWorldLocation (Variables|/Script/Paper2D.PaperCharacter|GetSprite (Variables|Default|GetMainGamePlayerRef))) (Transformation|GetWorldLocation (Variables|/Game/OctoInkContent/Blueprints/Actors/Player/BP_BasePlayer.BP_BasePlayer_C|GetCamera (Variables|Default|GetMainGamePlayerRef)))) false false)
  (bind _asbp_base_player (Utilities|Casting|CastToBP_BasePlayer (Game|Player|GetPlayerPawn 0)))
  (bind _asbp_minigame_icon (Utilities|Casting|CastToBP_MinigameIcon (UserInterface|GetUserWidgetObject (Variables|Default|GetWidget))))
  (Default|ShowE _asbp_minigame_icon false)
  (EventDispatchers|BindEventtoOnEnterInteractable _asbp_base_player (delegate Custom|CustomEvent_0))
  (EventDispatchers|BindEventtoOnExitInteractable _asbp_base_player (delegate Custom|CustomEvent_2)))

(event Collision|EventActorBeginOverlap
  (params (OtherActor :type Actor%20Object%20Reference))
  (|CallParentFunction OtherActor) ; This node is disabled and will not be called.\nDrag off pins to build functionality.
)

(event EventTick
  (params (DeltaSeconds :type Float%20%28single-precision%29))
  (|CallParentFunction DeltaSeconds) ; This node is disabled and will not be called.\nDrag off pins to build functionality.
)

(event EventDoInteraction
  (bind _asbp_player_main_game_controller (Utilities|Casting|CastToBP_PlayerMainGameController (Game|GetPlayerController 0)))
  (bind _asbp_main_world (Utilities|Casting|CastToBP_MainWorld (Game|GetGameMode)))
  (Variables|Default|SetMainGameModeRef _asbp_main_world)
  (if (and (Utilities|Struct|BreakMenuData (Variables|/Game/OctoInkContent/Blueprints/SaveData/MyGame.MyGame_C|GetGameStateData (Variables|Default|GetGameInstanceRef))) (not (Variables|/Game/OctoInkContent/Blueprints/Controllers/BP_PlayerBaseController.BP_PlayerBaseController_C|GetisOnMinigame _asbp_player_main_game_controller)))
    (if (Utilities|Struct|BreakDebugData (Variables|/Game/OctoInkContent/Blueprints/SaveData/MyGame.MyGame_C|GetDebugData (Variables|Default|GetGameInstanceRef)))
      (CallFunction|OnWin)
      (else
        (bind _asbp_player_base_controller (Utilities|Casting|CastToBP_PlayerBaseController (Game|GetPlayerController 0)))
        (Variables|/Game/OctoInkContent/Blueprints/Controllers/BP_PlayerBaseController.BP_PlayerBaseController_C|SetisOnMinigame _asbp_player_base_controller true)
        (Variables|Default|SetCurrentTime 0)
        (CallFunction|Timer)
        (Viewport|RemoveAllWidgets)
        (Variables|/Script/Engine.PlayerController|SetbShowMouseCursor (Game|GetPlayerController 0) true)
        (Variables|/Game/OctoInkContent/Blueprints/Controllers/BP_PlayerBaseController.BP_PlayerBaseController_C|SetEnableMovement (Variables|Default|GetPlayerControllerRef) false)
        (|CallParentFunction)))))

(event EventOnExit
  (|CallParentFunction)
  (bind _asbp_player_main_game_controller (Utilities|Casting|CastToBP_PlayerMainGameController (Game|GetPlayerController 0)))
  (Variables|/Game/OctoInkContent/Blueprints/Controllers/BP_PlayerBaseController.BP_PlayerBaseController_C|SetisOnMinigame _asbp_player_main_game_controller false)
  (Variables|/Game/OctoInkContent/Blueprints/Controllers/BP_PlayerBaseController.BP_PlayerBaseController_C|SetEnableMovement _asbp_player_main_game_controller true))

(fn ConstructionScript
  (|CallParentFunction))

(fn HideMinigameIcon
  (params (Shows :type Boolean))
  (Rendering|SetVisibility (Variables|Default|GetWidget) Shows false))