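; BP_Fridge is an interactable fridge actor in the main world that opens a minigame.
; It extends a parent's DoInteraction event, first checking the player controller's IsMinigameOpen flag so only one minigame opens at a time.
; When none is open, it sets the flag, creates the BP_Minigame2 widget, adds it to the viewport and initializes it with a reference to itself.
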(event EventBeginPlay
  (|CallParentFunction))

(event Collision|EventActorBeginOverlap
  (params (OtherActor :type Actor%20Object%20Reference))
  (|CallParentFunction OtherActor) ; This node is disabled and will not be called.\nDrag off pins to build functionality.
)

(event EventTick
  (params (DeltaSeconds :type Float%20%28single-precision%29))
  (|CallParentFunction DeltaSeconds))

(event EventDoInteraction
  (bind _playercontrollerref (Variables|Default|GetPlayerControllerRef))
  (|CallParentFunction)
  (if (not (Variables|/Game/OctoInkContent/Blueprints/Controllers/BP_PlayerMainGameController.BP_PlayerMainGameController_C|GetisMinigameOpen _playercontrollerref))
    (Variables|/Game/OctoInkContent/Blueprints/Controllers/BP_PlayerMainGameController.BP_PlayerMainGameController_C|SetisMinigameOpen _playercontrollerref true)
    (bind _returnvalue (UserInterface|CreateWidget "/Game/OctoInkContent/Blueprints/Widgets/Minigames/Minigames2/BP_Minigame2.BP_Minigame2_C"))
    (UserInterface|Viewport|AddtoViewport _returnvalue 0)
    (Default|Init _returnvalue self)))

(fn ConstructionScript
  (|CallParentFunction))