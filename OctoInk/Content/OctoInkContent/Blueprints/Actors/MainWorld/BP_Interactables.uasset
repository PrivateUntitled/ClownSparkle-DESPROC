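; BP_Interactables is an interactable actor for the main world, apparently a base for objects that lead into minigames.
; On BeginPlay it binds DoInteraction, left empty here, to the InteractedWithObject dispatcher and caches the main game player controller.
; OnExit calls BackToMainWorld on the BP_MainWorld game mode, then clears the controller's IsOnMinigame flag.
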(event Custom|OnExit
  (bind _asbp_main_world (Utilities|Casting|CastToBP_MainWorld (Game|GetGameMode)))
  (Default|BacktoMainWorld _asbp_main_world)
  (bind _asbp_player_main_game_controller (Utilities|Casting|CastToBP_PlayerMainGameController (Game|GetPlayerController 0)))
  (Variables|/Game/OctoInkContent/Blueprints/Controllers/BP_PlayerMainGameController.BP_PlayerMainGameController_C|SetisOnMinigame _asbp_player_main_game_controller false))

(event Custom|DoInteraction)

(event EventBeginPlay
  (EventDispatchers|BindEventtoInteractedwithObject (delegate Custom|DoInteraction))
  (bind _asbp_player_main_game_controller (Utilities|Casting|CastToBP_PlayerMainGameController (Game|GetPlayerController 0)))
  (Variables|Default|SetPlayerControllerRef _asbp_player_main_game_controller))

(event Collision|EventActorBeginOverlap
  (params (OtherActor :type Actor%20Object%20Reference)))

(event EventTick
  (params (DeltaSeconds :type Float%20%28single-precision%29)))

(fn ConstructionScript)