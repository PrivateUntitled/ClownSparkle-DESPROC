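; BP_Bed is an interactable bed that lets a tired player sleep to recover energy.
; Interaction sets the controller's IsMinigameOpen flag, then opens BP_Minigame4 with a bed reference only if CanSleep is true.
; OnWin advances game time by two hours for Tired or four for Exhausted, then resets energy, status and player speed; Normal status cannot sleep.
; Its widget's visibility follows CanSleep at BeginPlay.
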(event EventBeginPlay
  (|CallParentFunction)
  (bind _asmy_game (Utilities|Casting|CastToMyGame (Game|GetGameInstance)))
  (Variables|Default|SetGameInstance _asmy_game)
  (Rendering|SetVisibility (Variables|Default|GetWidget) (Utilities|Struct|BreakMenuData (Variables|/Game/OctoInkContent/Blueprints/SaveData/MyGame.MyGame_C|GetGameStateData (Variables|Default|GetGameInstanceRef))) false))

(event Collision|EventActorBeginOverlap
  (params (OtherActor :type Actor%20Object%20Reference))
  (|CallParentFunction OtherActor) ; This node is disabled and will not be called.\nDrag off pins to build functionality.
)

(event EventTick
  (params (DeltaSeconds :type Float%20%28single-precision%29))
  (|CallParentFunction DeltaSeconds) ; This node is disabled and will not be called.\nDrag off pins to build functionality.
)

(event EventDoInteraction
  (bind _playercontrollerref (Variables|Default|GetPlayerControllerRef))
  (|CallParentFunction)
  (if (not (Variables|/Game/OctoInkContent/Blueprints/Controllers/BP_PlayerMainGameController.BP_PlayerMainGameController_C|GetisMinigameOpen _playercontrollerref))
    (Variables|/Game/OctoInkContent/Blueprints/Controllers/BP_PlayerMainGameController.BP_PlayerMainGameController_C|SetisMinigameOpen _playercontrollerref true)
    (if (Utilities|Struct|BreakMenuData (Variables|/Game/OctoInkContent/Blueprints/SaveData/MyGame.MyGame_C|GetGameStateData (Variables|Default|GetGameInstanceRef)))
      (bind _returnvalue (UserInterface|CreateWidget "/Game/OctoInkContent/Blueprints/Widgets/Minigames/Mingiame4/BP_Minigame4.BP_Minigame4_C"))
      (Variables|/Game/OctoInkContent/Blueprints/Widgets/Minigames/Mingiame4/BP_Minigame4.BP_Minigame4_C|SetBedRef _returnvalue self)
      (UserInterface|Viewport|AddtoViewport _returnvalue 0))))

(event EventOnWin
  (bind _gameinstance (Variables|Default|GetGameInstance))
  (bind _gamemodedata (Variables|/Game/OctoInkContent/Blueprints/SaveData/MyGame.MyGame_C|GetGameModeData _gameinstance))
  (bind _maxtime (Utilities|Struct|BreakGameModeData _gamemodedata))
  (bind _returnvalue (/ _maxtime 24))
  (|CallParentFunction)
  (switch Utilities|FlowControl|Switch|SwitchonEnergyStatus (Utilities|Struct|BreakPlayerStats (Variables|/Game/OctoInkContent/Blueprints/SaveData/MyGame.MyGame_C|GetPlayerStats (Variables|Default|GetGameInstance)))
    (:NewEnumerator0
      (Development|PrintString "Cannot Sleep!"))
    (:NewEnumerator1
      (Default|TrackTime _gameinstance (* _returnvalue 2))
      (Development|PrintString "Slept for 2 hours")
      (Utilities|Struct|SetmembersinPlayerStats (Variables|/Game/OctoInkContent/Blueprints/SaveData/MyGame.MyGame_C|GetPlayerStats (Variables|Default|GetGameInstance)) 0 "NewEnumerator0" :!label _label)
      (bind _asbp_main_game_player (Utilities|Casting|CastToBP_MainGamePlayer (Game|Player|GetPlayerPawn 0)))
      (Default|SetPlayerSpeed _asbp_main_game_player))
    (:NewEnumerator2
      (Default|TrackTime _gameinstance (* _returnvalue 4))
      (Development|PrintString "Slept for 4 hours")
      (goto _label))))

(fn ConstructionScript
  (|CallParentFunction))