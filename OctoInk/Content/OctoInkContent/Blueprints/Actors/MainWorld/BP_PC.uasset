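; BP_PC is an interactable PC actor in the main world that opens the website widget.
; On BeginPlay it rotates its widget component using the look-at direction from the player's sprite to the player's camera.
; Interacting clears all widgets, then, if the main world game mode's CanOpenQuests flag is set, asks it to show BP_WebsiteWidget with the cursor visible and movement disabled.
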(event EventBeginPlay
  (|CallParentFunction)
  (bind _asbp_main_game_player (Utilities|Casting|CastToBP_MainGamePlayer (Game|Player|GetPlayerPawn 0)))
  (Transformation|SetWorldRotation (Variables|Default|GetWidget) (Math|Rotator|FindLookatRotation (Transformation|GetWorldLocation (Variables|/Script/Paper2D.PaperCharacter|GetSprite _asbp_main_game_player)) (Transformation|GetWorldLocation (Variables|/Game/OctoInkContent/Blueprints/Actors/Player/BP_BasePlayer.BP_BasePlayer_C|GetCamera _asbp_main_game_player))) false false))

(event Collision|EventActorBeginOverlap
  (params (OtherActor :type Actor%20Object%20Reference)))

(event EventTick
  (params (DeltaSeconds :type Float%20%28single-precision%29)))

(event EventDoInteraction
  (|CallParentFunction)
  (Viewport|RemoveAllWidgets)
  (bind _asbp_main_world (Utilities|Casting|CastToBP_MainWorld (Game|GetGameMode)))
  (if (Variables|/Game/OctoInkContent/Blueprints/GameMode/BP_MainWorld.BP_MainWorld_C|GetCanOpenQuests _asbp_main_world)
    (Default|SettingWidget _asbp_main_world true true "/Game/OctoInkContent/Blueprints/Widgets/Commission/BP_WebsiteWidget.BP_WebsiteWidget_C")))

(event EventOnExit
  (|CallParentFunction))

(fn ConstructionScript)