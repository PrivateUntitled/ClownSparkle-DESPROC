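; Floating world-space notification that displays the energy recovery widget, then fades out and destroys itself.
; On BeginPlay it turns the widget once toward the player's camera, then runs a delayed loop that lowers the widget's alpha until it reaches zero.
; Tick moves the root steadily upward at a set speed while the fade runs.
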(event EventBeginPlay
  (bind _asbase_player (Utilities|Casting|CastToBasePlayer (Game|Player|GetPlayerPawn 0)))
  (Transformation|SetWorldRotation (Variables|Default|GetWidget) (Math|Rotator|FindLookatRotation (Transformation|GetWorldLocation (Variables|Default|GetWidget)) (Transformation|GetWorldLocation (Variables|/Game/OctoInkContent/Blueprints/Actors/Player/BasePlayer.BasePlayer_C|GetCamera _asbase_player))) false false)
  (if (> (Variables|Default|GetAlpha) 0.0) :!label _label
    (bind _asbp_energy_recovery (Utilities|Casting|CastToBP_EnergyRecovery (UserInterface|GetUserWidgetObject (Variables|Default|GetWidget))))
    (bind _output_get (Variables|Default|SetAlpha (- (Variables|Default|GetAlpha) (Variables|Default|GetAlphaLoss))))
    (Default|SetAlpha _asbp_energy_recovery _output_get)
    (Utilities|FlowControl|Delay (Variables|Default|GetAlphaDelay))
    (goto _label)
    (else
      (Actor|DestroyActor))))

(event Collision|EventActorBeginOverlap
  (params (OtherActor :type Actor%20Object%20Reference)))

(event EventTick
  (params (DeltaSeconds :type Float%20%28single-precision%29))
  (bind _defaultsceneroot (Variables|Default|GetDefaultSceneRoot))
  (bind _returnvalue (Transformation|GetWorldLocation _defaultsceneroot))
  (Transformation|SetWorldLocation (Variables|Default|GetDefaultSceneRoot) (Math|Vector|MakeVector (.x _returnvalue) (.y _returnvalue) (+ (.z _returnvalue) (* DeltaSeconds (Variables|Default|GetSpeed)))) false false))

(fn ConstructionScript)