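; BP_PuzzlePlayer is the puzzle-mode player character, which carries a color and can Ink or Absorb puzzle interactables.
; A box overlap tracks the interactable in range, while the capsule flags standing inside one.
; Ink and Absorb forward to that object, play sound, flash an obstacle-colored particle material and call a matching event.
; MentalBlockRoll uses missing energy as the chance to freeze movement, setting a press count from player status.
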(event OnComponentEndOverlap(Sprite)
  (params (OverlappedComponent :type Primitive%20Component%20Object%20Reference) (OtherActor :type Actor%20Object%20Reference) (OtherComp :type Primitive%20Component%20Object%20Reference) (OtherBodyIndex :type Integer)))

(event OnComponentEndOverlap(Box)
  (params (OverlappedComponent :type Primitive%20Component%20Object%20Reference) (OtherActor :type Actor%20Object%20Reference) (OtherComp :type Primitive%20Component%20Object%20Reference) (OtherBodyIndex :type Integer))
  ;[1 1 1] Setting Puzzle Interactable Detection
  (bind _asbp_puzzle_interactable (Utilities|Casting|CastToBP_PuzzleInteractable OtherActor))
  (Variables|Default|SetObjectInRange 0)
  (Variables|/Game/OctoInkContent/Blueprints/Actors/Obstacles/BP_PuzzleInteractable.BP_PuzzleInteractable_C|SetInPlayerRange _asbp_puzzle_interactable false)
  (Default|OnExitInteractable _asbp_puzzle_interactable))

(event OnComponentBeginOverlap(CapsuleComponent)
  (params (OverlappedComponent :type Primitive%20Component%20Object%20Reference) (OtherActor :type Actor%20Object%20Reference) (OtherComp :type Primitive%20Component%20Object%20Reference) (OtherBodyIndex :type Integer) (bFromSweep :type Boolean) (SweepResult :type Hit%20Result%20Structure%20%28by%20ref%29))
  ;[1 1 1] Player Inside Obstacle Detector
  (Utilities|Casting|CastToBP_PuzzleInteractable OtherActor)
  (Variables|Default|SetIsPlayerInObstacle true))

(event OnComponentEndOverlap(CapsuleComponent)
  (params (OverlappedComponent :type Primitive%20Component%20Object%20Reference) (OtherActor :type Actor%20Object%20Reference) (OtherComp :type Primitive%20Component%20Object%20Reference) (OtherBodyIndex :type Integer))
  ;[1 1 1] Player Inside Obstacle Detector
  (Utilities|Casting|CastToBP_PuzzleInteractable OtherActor)
  (Variables|Default|SetIsPlayerInObstacle false))

(event OnComponentBeginOverlap(Box)
  (params (OverlappedComponent :type Primitive%20Component%20Object%20Reference) (OtherActor :type Actor%20Object%20Reference) (OtherComp :type Primitive%20Component%20Object%20Reference) (OtherBodyIndex :type Integer) (bFromSweep :type Boolean) (SweepResult :type Hit%20Result%20Structure%20%28by%20ref%29))
  ;[1 1 1] Setting Puzzle Interactable Detection
  (bind _asbp_puzzle_interactable (Utilities|Casting|CastToBP_PuzzleInteractable OtherActor))
  (if (!= _asbp_puzzle_interactable (Variables|Default|GetObjectInRange))
    (Variables|Default|SetObjectInRange _asbp_puzzle_interactable)
    (Variables|/Game/OctoInkContent/Blueprints/Actors/Obstacles/BP_PuzzleInteractable.BP_PuzzleInteractable_C|SetInPlayerRange _asbp_puzzle_interactable true)
    (Default|OnEnterInteractable _asbp_puzzle_interactable)))

(event OnComponentBeginOverlap(Sprite)
  (params (OverlappedComponent :type Primitive%20Component%20Object%20Reference) (OtherActor :type Actor%20Object%20Reference) (OtherComp :type Primitive%20Component%20Object%20Reference) (OtherBodyIndex :type Integer) (bFromSweep :type Boolean) (SweepResult :type Hit%20Result%20Structure%20%28by%20ref%29)))

(event Custom|StartParticleEffect
  ;[1 1 1] Playing Ink/Absorb Particle Effect
  (bind _asbp_obstacle (Utilities|Casting|CastToBP_Obstacle (Variables|Default|GetObjectInRange)))
  (Rendering|Material|SetMaterial (Variables|Default|GetParticleEffect) 0 (Variables|/Game/OctoInkContent/DataAssets/DataAssets/Color/PDA_Color.PDA_Color_C|GetParticleMaterial (Variables|/Game/OctoInkContent/Blueprints/Actors/Obstacles/BP_Obstacle.BP_Obstacle_C|GetCurrentColor _asbp_obstacle)))
  (Utilities|FlowControl|Delay 0.2)
  (Rendering|Material|SetMaterial (Variables|Default|GetParticleEffect) 0 "/Game/OctoInkContent/Assets/UIAssets/Obstacle/Nothing.Nothing"))

(event EventBeginPlay
  (|CallParentFunction))

(event Collision|EventActorBeginOverlap
  (params (OtherActor :type Actor%20Object%20Reference))
  (|CallParentFunction OtherActor) ; This node is disabled and will not be called.\nDrag off pins to build functionality.
)

(event EventTick
  (params (DeltaSeconds :type Float%20%28single-precision%29))
  (|CallParentFunction DeltaSeconds) ; This node is disabled and will not be called.\nDrag off pins to build functionality.
)

(fn ConstructionScript
  (|CallParentFunction))

(fn SetPlayerColor
  (params (NewCharacterColor :type PDA%20Color%20Object%20Reference))
  (bind _output_get (Variables|Default|SetCurrentColor NewCharacterColor))
  (Sprite|SetSpriteColor (Variables|Default|GetSprite) (Variables|/Game/OctoInkContent/DataAssets/DataAssets/Color/PDA_Color.PDA_Color_C|GetPlayerColor _output_get))
  (Variables|Default|SetHasColor (Utilities|Enum|NotEqual(Enum) (Variables|/Game/OctoInkContent/DataAssets/DataAssets/Color/PDA_Color.PDA_Color_C|GetColor (Variables|Default|GetCurrentColor)) "NewEnumerator6")))

(fn Ink
  (Utilities|FlowControl|Sequence
    (:then_0
      (bind _asbp_puzzle_interactable (Utilities|Casting|CastToBP_PuzzleInteractable (Variables|Default|GetObjectInRange)))
      (Default|Ink _asbp_puzzle_interactable))
    (:then_1
      (CallFunction|StartParticleEffect))
    (:then_2
      (Audio|PlaySoundatLocation "/Game/OctoInkContent/Assets/SFX/sounds/Ink.Ink" (Transformation|GetWorldLocation (Variables|Default|GetCapsuleComponent)) "0, 0, 0" 1.0 1.0 0.0 0 0 0))
    (:then_3
      (bind _asbp_puzzle_interactable_2 (Utilities|Casting|CastToBP_PuzzleInteractable (Variables|Default|GetObjectInRange)))
      (Default|CallOnInk _asbp_puzzle_interactable_2))))

(fn Absorb
  (Utilities|FlowControl|Sequence
    (:then_0
      (bind _asbp_puzzle_interactable (Utilities|Casting|CastToBP_PuzzleInteractable (Variables|Default|GetObjectInRange)))
      (Default|Absorb _asbp_puzzle_interactable))
    (:then_1
      (CallFunction|StartParticleEffect))
    (:then_2
      (Audio|PlaySoundatLocation "/Game/OctoInkContent/Assets/SFX/sounds/Absorb.Absorb" (Transformation|GetWorldLocation (Variables|Default|GetCapsuleComponent)) "0, 0, 0" 1.0 1.0 0.0 0 0 0))
    (:then_3
      (bind _asbp_puzzle_interactable_2 (Utilities|Casting|CastToBP_PuzzleInteractable (Variables|Default|GetObjectInRange)))
      (Default|CallOnAbsorb _asbp_puzzle_interactable_2))))

(fn MentalBlockRoll
  (bind _output_get (Variables|Default|SetMentalBlockChance (* (- 1 (/ (Variables|Default|GetEnergy) (Variables|Default|GetMaxEnergy))) 100)))
  (if (<= (Math|Random|RandomIntegerinRange 0 100) _output_get)
    (Variables|Default|SetIsMentalBlocked true)
    (Utilities|FlowControl|Sequence
      (:then_0
        (bind _asmy_game (Utilities|Casting|CastToMyGame (Game|GetGameInstance)))
        (switch Utilities|FlowControl|Switch|SwitchonEnergyStatus (Utilities|Struct|BreakPlayerStats (Variables|/Game/OctoInkContent/Blueprints/SaveData/MyGame.MyGame_C|GetPlayerStats _asmy_game))
          (:NewEnumerator0
            (Variables|Default|SetPressCount 2))
          (:NewEnumerator1
            (Variables|Default|SetPressCount 3))
          (:NewEnumerator2
            (Variables|Default|SetPressCount 5))))
      (:then_1
        (Components|Activation|Deactivate (Variables|Character|GetCharacterMovement)))
      (:then_2
        (Development|PrintString (Utilities|String|Append "Mental Block Chance" (Utilities|String|ToString(Integer) (Variables|Default|GetMentalBlockChance))))
        (Development|PrintString (Utilities|String|Append "Press Count" (Utilities|String|ToString(Integer) (Variables|Default|GetPressCount))))))))