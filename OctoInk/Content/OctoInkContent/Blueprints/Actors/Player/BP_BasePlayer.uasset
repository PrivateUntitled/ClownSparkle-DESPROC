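; Base player character whose energy level, read from the MyGame instance's PlayerStats, drives how it moves and how the screen looks.
; On BeginPlay, SetPlayerSpeed fades in the post-process vignette as energy drops and scales walk speed linearly with energy.
; It also switches the controller's dash multiplier at half energy, then writes energy back to PlayerStats.
; An archived, unconnected line-trace block toggles BP_Wall transparency between camera and sprite.
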(event EventBeginPlay
  (CallFunction|SetPlayerSpeed))

(fn ConstructionScript)

(fn SetPlayerSpeed
  (bind _returnvalue (Pawn|GetController))
  (bind _postprocessvolume (Variables|Default|GetPostProcessVolume))
  (bind _asmy_game (Utilities|Casting|CastToMyGame (Game|GetGameInstance)))
  (Variables|Default|SetEnergy (.PlayerEnergy (Utilities|Struct|BreakPlayerStats (Variables|/Game/OctoInkContent/Blueprints/SaveData/MyGame.MyGame_C|GetPlayerStats _asmy_game))))
  (Variables|Default|SetMaxEnergy (.MaxPlayerEnergy (Utilities|Struct|BreakPlayerStats (Variables|/Game/OctoInkContent/Blueprints/SaveData/MyGame.MyGame_C|GetPlayerStats _asmy_game))))
  (Utilities|FlowControl|Sequence
    (:then_0
      ;[1 1 1] Set World Vignette
      (if (!= _postprocessvolume 0)
        (Variables|/Script/Engine.PostProcessVolume|SetBlendWeight _postprocessvolume (- 1.0 (/ (Math|Conversions|ToFloat(Integer) (Variables|Default|GetEnergy)) (Math|Conversions|ToFloat(Integer) (Variables|Default|GetMaxEnergy)))))))
    (:then_1
      ;[1 1 1] Set Walk Speed
      (Variables|/Script/Engine.CharacterMovementComponent|SetMaxWalkSpeed (Variables|Character|GetCharacterMovement) (+ (* (Variables|Default|GetWalkSpeedSlope) (Math|Conversions|ToFloat(Integer) (Math|Integer|Clamp(Integer) (Variables|Default|GetEnergy) 0 (Variables|Default|GetMaxEnergy)))) (Variables|Default|GetMinWalkSpeed))))
    (:then_2
      ;[1 1 1] Set Dash Speed
      (if (>= (/ (Math|Conversions|ToFloat(Integer) (Variables|Default|GetEnergy)) (Math|Conversions|ToFloat(Integer) (Variables|Default|GetMaxEnergy))) 0.5)
        (bind _asbp_player_base_controller (Utilities|Casting|CastToBP_PlayerBaseController _returnvalue))
        (Variables|/Game/OctoInkContent/Blueprints/Controllers/BP_PlayerBaseController.BP_PlayerBaseController_C|SetDashMultiplier _asbp_player_base_controller 1e+01)
        (else
          (bind _asbp_player_base_controller_2 (Utilities|Casting|CastToBP_PlayerBaseController _returnvalue))
          (Variables|/Game/OctoInkContent/Blueprints/Controllers/BP_PlayerBaseController.BP_PlayerBaseController_C|SetDashMultiplier _asbp_player_base_controller_2 2.0))))
    (:then_3
      (bind _asmy_game_2 (Utilities|Casting|CastToMyGame (Game|GetGameInstance)))
      (Utilities|Struct|SetmembersinPlayerStats (Variables|/Game/OctoInkContent/Blueprints/SaveData/MyGame.MyGame_C|GetPlayerStats _asmy_game_2) (Variables|Default|GetEnergy) (Variables|Default|GetMaxEnergy)))))