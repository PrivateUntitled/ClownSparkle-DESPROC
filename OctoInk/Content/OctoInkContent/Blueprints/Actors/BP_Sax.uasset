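; Saxophone actor that restores the player's energy when the controller's PlayInstrument event fires.
; RecoverEnergy resets ConsecutiveAttempts, clears the sax mesh and adds about half the missing energy in equal steps stored in the GameInstance's PlayerStats.
; A delayed loop spreads the steps across the sound's duration, spawning a notification and updating player speed each time.
; When the loop ends, the mesh returns and IsBeingPlayed clears.
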(event Custom|Recover%20Energy
  (params (Delay :type Float%20%28single-precision%29))
  (bind _asmy_game (Utilities|Casting|CastToMyGame (Game|GetGameInstance)))
  (Utilities|Struct|SetmembersinPlayerStats (Variables|/Game/OctoInkContent/Blueprints/SaveData/MyGame.MyGame_C|GetPlayerStats _asmy_game))
  (Variables|Default|SetIsBeingPlayed true)
  (Components|StaticMesh|SetStaticMesh (Variables|Default|GetSax) 0)
  (bind _asmy_game_2 (Utilities|Casting|CastToMyGame (Game|GetGameInstance)))
  (Variables|Default|SetEnergyIncrease (/ (* (- (.MaxPlayerEnergy (Utilities|Struct|BreakPlayerStats (Variables|/Game/OctoInkContent/Blueprints/SaveData/MyGame.MyGame_C|GetPlayerStats _asmy_game_2))) (.PlayerEnergy (Utilities|Struct|BreakPlayerStats (Variables|/Game/OctoInkContent/Blueprints/SaveData/MyGame.MyGame_C|GetPlayerStats _asmy_game_2)))) 0.5) (Math|Conversions|ToFloat(Integer) (Variables|Default|GetMaxLoops))))
  (Variables|Default|SetCounter 0)
  (if (< (Variables|Default|GetCounter) (Variables|Default|GetMaxLoops)) :!label _label
    (bind _asmain_game_player (Utilities|Casting|CastToMainGamePlayer (Game|Player|GetPlayerPawn 0)))
    (bind _returnvalue (Game|SpawnActorfromClass "/Game/OctoInkContent/Blueprints/Actors/BP_Notif.BP_Notif_C" (Math|Conversions|ToTransform(Vector) (Transformation|GetWorldLocation (Variables|/Game/OctoInkContent/Blueprints/Actors/Player/MainGamePlayer.MainGamePlayer_C|GetNotifSpawn _asmain_game_player))) "Undefined" 0 0))
    (Default|RecoverEnergy _returnvalue self)
    (bind _asmy_game_3 (Utilities|Casting|CastToMyGame (Game|GetGameInstance)))
    (Utilities|Struct|SetmembersinPlayerStats (Variables|/Game/OctoInkContent/Blueprints/SaveData/MyGame.MyGame_C|GetPlayerStats _asmy_game_3) (Math|Float|Truncate (+ (Math|Conversions|ToFloat(Integer) (.PlayerEnergy (Utilities|Struct|BreakPlayerStats (Variables|/Game/OctoInkContent/Blueprints/SaveData/MyGame.MyGame_C|GetPlayerStats _asmy_game_3)))) (Variables|Default|GetEnergyIncrease))))
    (Default|SetPlayerSpeed _asmain_game_player)
    (Utilities|FlowControl|Delay (/ (Variables|/Script/Engine.SoundBase|GetDuration (Variables|Default|GetSound)) (Math|Conversions|ToFloat(Integer) (Variables|Default|GetMaxLoops))))
    (Math|Integer|IncrementInt (Variables|Default|GetCounter)
      (:%20%20
        (goto _label)))
    (else
      (Components|StaticMesh|SetStaticMesh (Variables|Default|GetSax) "/Game/OctoInkContent/Assets/GameAssets/HouseAssets/Sax.Sax")
      (Variables|Default|SetIsBeingPlayed false))))

(event EventBeginPlay
  (bind _asbp_player_main_game_controller (Utilities|Casting|CastToBP_PlayerMainGameController (Game|GetPlayerController 0)))
  (EventDispatchers|BindEventtoPlayInstrument _asbp_player_main_game_controller (delegate Custom|Recover%20Energy)))

(fn ConstructionScript)