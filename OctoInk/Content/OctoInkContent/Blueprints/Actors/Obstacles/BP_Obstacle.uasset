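; BP_Obstacle is a puzzle obstacle that holds a color the player can ink or absorb, optionally restricted to a required color.
; A BP_ObstaclePointer widget, rotated toward the camera on BeginPlay, shows current color and lock color.
; Tick checks range, player color and game-state permissions to display ink or absorb mouse prompts.
; Ink and Absorb extend parent events to toggle the color-match icon; helpers swap or copy colors to the player.
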(event Custom|DoColorAnimation
  (params (NewParam :type Color%20Structure)))

(event EventBeginPlay
  (|CallParentFunction)
  (Utilities|FlowControl|Sequence
    (:then_0
      (CallFunction|SetObstacleColor (Variables|Default|GetCurrentColor))
      (CallFunction|SetRequiredColor (Variables|Default|GetColorRequired))
      (CallFunction|SetObstacleRequirement))
    (:then_1
      (bind _asbp_puzzle_player (Utilities|Casting|CastToBP_PuzzlePlayer (Game|Player|GetPlayerPawn 0)))
      (Variables|Default|SetPlayerRef _asbp_puzzle_player)
      (bind _asbp_obstacle_pointer (Utilities|Casting|CastToBP_ObstaclePointer (UserInterface|GetWidget (Variables|Default|GetWidget))))
      (Variables|Default|SetObstaclePointerRef _asbp_obstacle_pointer))
    (:then_2
      (Transformation|SetWorldRotation (Variables|Default|GetWidget) (Math|Rotator|FindLookatRotation (Transformation|GetWorldLocation (Variables|/Script/Paper2D.PaperCharacter|GetSprite (Variables|Default|GetPlayerRef))) (Transformation|GetWorldLocation (Variables|/Game/OctoInkContent/Blueprints/Actors/Player/BP_BasePlayer.BP_BasePlayer_C|GetCamera (Variables|Default|GetPlayerRef)))) false false))))

(event Collision|EventActorBeginOverlap
  (params (OtherActor :type Actor%20Object%20Reference)))

(event EventTick
  (params (DeltaSeconds :type Float%20%28single-precision%29))
  (bind _playerref (Variables|Default|GetPlayerRef))
  (bind _playerref_2 (Variables|Default|GetPlayerRef))
  (|CallParentFunction DeltaSeconds)
  (bind _inkable (CallFunction|IsInkable))
  (if (Math|Boolean|ANDBoolean _inkable (Variables|Default|GetInPlayerRange) (Utilities|Enum|NotEqual(Enum) (Variables|/Game/OctoInkContent/DataAssets/DataAssets/Color/PDA_Color.PDA_Color_C|GetColor (Variables|/Game/OctoInkContent/Blueprints/Actors/Player/BP_PuzzlePlayer.BP_PuzzlePlayer_C|GetCurrentColor _playerref)) "NewEnumerator6") (not (Variables|/Game/OctoInkContent/Blueprints/Actors/Player/BP_PuzzlePlayer.BP_PuzzlePlayer_C|GetIsPlayerInObstacle _playerref)))
    (bind _asmy_game (Utilities|Casting|CastToMyGame (Game|GetGameInstance)))
    (if (Utilities|Struct|BreakMenuData (Variables|/Game/OctoInkContent/Blueprints/SaveData/MyGame.MyGame_C|GetGameStateData _asmy_game))
      (Default|PlayMouseAnimation (Variables|Default|GetObstaclePointerRef) true))
    (else
      (bind _absrobable (CallFunction|IsAbsorbable))
      (if (Math|Boolean|ANDBoolean _absrobable (Variables|Default|GetInPlayerRange) (Utilities|Enum|Equal(Enum) (Variables|/Game/OctoInkContent/DataAssets/DataAssets/Color/PDA_Color.PDA_Color_C|GetColor (Variables|/Game/OctoInkContent/Blueprints/Actors/Player/BP_PuzzlePlayer.BP_PuzzlePlayer_C|GetCurrentColor _playerref_2)) "NewEnumerator6") (not (Variables|/Game/OctoInkContent/Blueprints/Actors/Player/BP_PuzzlePlayer.BP_PuzzlePlayer_C|GetIsPlayerInObstacle _playerref_2)))
        (bind _asmy_game_2 (Utilities|Casting|CastToMyGame (Game|GetGameInstance)))
        (if (Utilities|Struct|BreakMenuData (Variables|/Game/OctoInkContent/Blueprints/SaveData/MyGame.MyGame_C|GetGameStateData _asmy_game_2))
          (Default|PlayMouseAnimation (Variables|Default|GetObstaclePointerRef) false)
          (Default|PlayAbsorbAnimation (Variables|Default|GetObstaclePointerRef)))
        (else
          (Default|HideAllMouse (Variables|Default|GetObstaclePointerRef)))))))

(event EventInk
  (|CallParentFunction)
  (if (Variables|Default|GetShowCorrectColor)
    (Default|ShowMatchesIcon (Variables|Default|GetObstaclePointerRef) (Utilities|Enum|Equal(Enum) (Variables|/Game/OctoInkContent/DataAssets/DataAssets/Color/PDA_Color.PDA_Color_C|GetColor (Variables|Default|GetCurrentColor)) (Variables|/Game/OctoInkContent/DataAssets/DataAssets/Color/PDA_Color.PDA_Color_C|GetColor (Variables|Default|GetColorRequired))))))

(event EventAbsorb
  (|CallParentFunction)
  (if (Variables|Default|GetShowCorrectColor)
    (Default|HideMatchingColor (Variables|Default|GetObstaclePointerRef))))

(fn ConstructionScript)

(fn SetObstacleColor
  (params (SetColor :type PDA%20Color%20Object%20Reference))
  (bind _asbp_obstacle_pointer (Utilities|Casting|CastToBP_ObstaclePointer (UserInterface|GetUserWidgetObject (Variables|Default|GetWidget))))
  (Default|SetPointerColor _asbp_obstacle_pointer SetColor))

(fn SetObstacleRequirement)

(fn IsEqualtoPlayerColor
  (params (PlayerColor :type Colors%20Enum :default "NewEnumerator0"))
  (if (Variables|Default|GetOnlyAcceptRequiredColors?)
    (return (Utilities|Enum|Equal(Enum) PlayerColor (Variables|/Game/OctoInkContent/DataAssets/DataAssets/Color/PDA_Color.PDA_Color_C|GetColor (Variables|Default|GetColorRequired))))
    (else
      (return true))))

(fn SwitchColors
  (bind _asbp_puzzle_player (Utilities|Casting|CastToBP_PuzzlePlayer (Game|Player|GetPlayerPawn 0)))
  (Utilities|FlowControl|Sequence
    (:then_0
      (LocalVariables|SetObstacleColor (Variables|Default|GetCurrentColor)))
    (:then_1
      (CallFunction|SetObstacleColor (Variables|/Game/OctoInkContent/Blueprints/Actors/Player/BP_PuzzlePlayer.BP_PuzzlePlayer_C|GetCurrentColor _asbp_puzzle_player)))
    (:then_2
      (Default|SetPlayerColor _asbp_puzzle_player (LocalVariables|GetObstacleColor)))))

(fn GetColor
  (bind _asbp_puzzle_player (Utilities|Casting|CastToBP_PuzzlePlayer (Game|Player|GetPlayerPawn 0)))
  (Default|SetPlayerColor _asbp_puzzle_player (Variables|Default|GetCurrentColor)))

(fn IsAbsorbable
  (return (and (Utilities|Enum|NotEqual(Enum) "NewEnumerator6" (Variables|/Game/OctoInkContent/DataAssets/DataAssets/Color/PDA_Color.PDA_Color_C|GetColor (Variables|Default|GetCurrentColor))) (Variables|Default|GetCanAbsorb))))

(fn IsInkable
  (bind _asbp_puzzle_player (Utilities|Casting|CastToBP_PuzzlePlayer (Game|Player|GetPlayerPawn 0)))
  (bind _notequaltoplayercolor (CallFunction|IsEqualtoPlayerColor (Variables|/Game/OctoInkContent/DataAssets/DataAssets/Color/PDA_Color.PDA_Color_C|GetColor (Variables|/Game/OctoInkContent/Blueprints/Actors/Player/BP_PuzzlePlayer.BP_PuzzlePlayer_C|GetCurrentColor _asbp_puzzle_player))))
  (return (Math|Boolean|ANDBoolean _notequaltoplayercolor (Utilities|Enum|Equal(Enum) (Variables|/Game/OctoInkContent/DataAssets/DataAssets/Color/PDA_Color.PDA_Color_C|GetColor (Variables|Default|GetCurrentColor)) "NewEnumerator6") (Variables|Default|GetCanInk))))

(fn SetRequiredColor
  (params (ColorRequired :type PDA%20Color%20Object%20Reference))
  (Variables|Default|SetColorRequired ColorRequired)
  (bind _asbp_obstacle_pointer (Utilities|Casting|CastToBP_ObstaclePointer (UserInterface|GetWidget (Variables|Default|GetWidget))))
  (if (!= ColorRequired 0)
    (Default|SetLockColor _asbp_obstacle_pointer ColorRequired)
    (else
      (Default|SetLockColor _asbp_obstacle_pointer))))

(fn SetColSourceColor
  (params (SetColor :type PDA%20Color%20Object%20Reference))
  (bind _asbp_obstacle_pointer (Utilities|Casting|CastToBP_ObstaclePointer (UserInterface|GetUserWidgetObject (Variables|Default|GetWidget))))
  (Default|SetColSourceColor _asbp_obstacle_pointer SetColor))