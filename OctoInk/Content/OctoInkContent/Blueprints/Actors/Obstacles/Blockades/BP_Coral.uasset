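; BP_Coral is a coral blockade obstacle that takes on a given obstacle color.
; It overrides the parent's SetObstacleColor to store the color and apply its coral material to the static mesh.
; The color also drives collision: one specific color switches the mesh to a custom object channel, while all others make it WorldStatic.
; All other graphs only defer to the parent or are disabled stubs.
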(event EventBeginPlay
  (|CallParentFunction) ; This node is disabled and will not be called.\nDrag off pins to build functionality.
)

(event Collision|EventActorBeginOverlap
  (params (OtherActor :type Actor%20Object%20Reference))
  (|CallParentFunction OtherActor) ; This node is disabled and will not be called.\nDrag off pins to build functionality.
)

(event EventTick
  (params (DeltaSeconds :type Float%20%28single-precision%29))
  (|CallParentFunction DeltaSeconds) ; This node is disabled and will not be called.\nDrag off pins to build functionality.
)

(fn ConstructionScript
  (|CallParentFunction))

(fn SetObstacleColor
  (params (SetColor :type PDA%20Color%20Object%20Reference))
  (|CallParentFunction SetColor)
  (Utilities|FlowControl|Sequence
    (:then_0
      (bind _output_get (Variables|Default|SetCurrentColor SetColor))
      (Rendering|Material|SetMaterial (Variables|Default|GetStaticMesh) 0 (Variables|/Game/OctoInkContent/DataAssets/DataAssets/Color/PDA_Color.PDA_Color_C|GetCoralColors _output_get)))
    (:then_1
      (if (Utilities|Enum|NotEqual(Enum) (Variables|/Game/OctoInkContent/DataAssets/DataAssets/Color/PDA_Color.PDA_Color_C|GetColor (Variables|Default|GetCurrentColor)) "NewEnumerator6")
        (Collision|SetCollisionObjectType (Variables|Default|GetStaticMesh) "ECC_WorldStatic")
        (else
          (Collision|SetCollisionObjectType (Variables|Default|GetStaticMesh) "ECC_GameTraceChannel1"))))))