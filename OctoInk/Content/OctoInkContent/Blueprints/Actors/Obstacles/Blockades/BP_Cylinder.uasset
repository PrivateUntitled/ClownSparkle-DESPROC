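; BP_Cylinder is a colorable cylinder blockade obstacle whose point light signals when its current color matches its required color.
; It extends a parent Blueprint, calling the parent logic on BeginPlay, Ink, Absorb and SetObstacleColor, then running ShowLight after each.
; ShowLight compares the two colors and unhides the light in game only when they are equal.
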(event EventBeginPlay
  (|CallParentFunction)
  (CallFunction|ShowLight))

(event Collision|EventActorBeginOverlap
  (params (OtherActor :type Actor%20Object%20Reference))
  (|CallParentFunction OtherActor) ; This node is disabled and will not be called.\nDrag off pins to build functionality.
)

(event EventTick
  (params (DeltaSeconds :type Float%20%28single-precision%29))
  (|CallParentFunction DeltaSeconds) ; This node is disabled and will not be called.\nDrag off pins to build functionality.
)

(event EventInk
  (|CallParentFunction)
  (CallFunction|ShowLight))

(event EventAbsorb
  (|CallParentFunction)
  (CallFunction|ShowLight))

(fn ConstructionScript
  (|CallParentFunction))

(fn ShowLight
  (Development|SetHiddeninGame (Variables|Default|GetPointLight) (not (Utilities|Enum|Equal(Enum) (Variables|/Game/OctoInkContent/DataAssets/DataAssets/Color/PDA_Color.PDA_Color_C|GetColor (Variables|Default|GetColorRequired)) (Variables|/Game/OctoInkContent/DataAssets/DataAssets/Color/PDA_Color.PDA_Color_C|GetColor (Variables|Default|GetCurrentColor)))) false))

(fn IsEqualtoPlayerColor
  (params (PlayerColor :type Colors%20Enum :default "NewEnumerator7"))
  (bind _notequaltoplayercolor (|CallParentFunction PlayerColor))
  (return _notequaltoplayercolor))

(fn SetObstacleColor
  (params (SetColor :type PDA%20Color%20Object%20Reference))
  (|CallParentFunction SetColor)
  (CallFunction|ShowLight))