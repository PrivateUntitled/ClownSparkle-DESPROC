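; BP_FlagBlockade is a blockade obstacle whose flag material follows its assigned color.
; It overrides SetObstacleColor, calling the parent, storing the color as CurrentColor and applying that color's FlagMaterial to material slot 1 of its static mesh.
; The construction script only calls the parent, and the event graph holds only disabled stub events.
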(event EventBeginPlay
  (|CallParentFunction) ; This node is disabled and will not be called.\nDrag off pins to build functionality.
)

(event Collision|EventActorBeginOverlap
  (params (OtherActor :type Actor%20Object%20Reference))
  (|CallParentFunction OtherActor) ; This node is disabled and will not be called.\nDrag off pins to build functionality.
)

(event EventTick
  (params (DeltaSeconds :type Float%20%28single-precision%29))
  (|CallParentFunction DeltaSeconds) ; This node is disabled and will not be called.\nDrag off pins to build functionality.
)

(fn ConstructionScript
  (|CallParentFunction))

(fn SetObstacleColor
  (params (SetColor :type PDA%20Color%20Object%20Reference))
  (|CallParentFunction SetColor)
  (bind _output_get (Variables|Default|SetCurrentColor SetColor))
  (Rendering|Material|SetMaterial (Variables|Default|GetStaticMesh) 1 (Variables|/Game/OctoInkContent/DataAssets/DataAssets/Color/PDA_Color.PDA_Color_C|GetFlagMaterial _output_get)))