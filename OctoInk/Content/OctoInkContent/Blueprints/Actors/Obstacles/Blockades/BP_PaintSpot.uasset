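; BP_PaintSpot is a paintable blockade spot that counts toward the level's required points.
; On BeginPlay it increments RequiredPoints on BP_Commission3GameMode, so each placed spot raises the total.
; The PaintWall event reveals the spot's decal, while the player color check defers entirely to the parent class.
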(event Custom|PaintWall
  (Rendering|SetVisibility (Variables|/Script/Engine.Actor|GetRootComponent (Variables|Default|GetDecal)) true false))

(event EventBeginPlay
  (|CallParentFunction)
  (bind _asbp_commission_3game_mode (Utilities|Casting|CastToBP_Commission3GameMode (Game|GetGameMode)))
  (Math|Integer|IncrementInt (Variables|/Game/OctoInkContent/Blueprints/GameMode/CommissionGameModes/BP_Commission3GameMode.BP_Commission3GameMode_C|GetRequiredPoints _asbp_commission_3game_mode)))

(event Collision|EventActorBeginOverlap
  (params (OtherActor :type Actor%20Object%20Reference))
  (|CallParentFunction OtherActor) ; This node is disabled and will not be called.\nDrag off pins to build functionality.
)

(event EventTick
  (params (DeltaSeconds :type Float%20%28single-precision%29))
  (|CallParentFunction DeltaSeconds) ; This node is disabled and will not be called.\nDrag off pins to build functionality.
)

(fn ConstructionScript
  (|CallParentFunction))

(fn IsEqualtoPlayerColor
  (params (PlayerColor :type Colors%20Enum :default "NewEnumerator7"))
  (bind _notequaltoplayercolor (|CallParentFunction PlayerColor))
  (return _notequaltoplayercolor))