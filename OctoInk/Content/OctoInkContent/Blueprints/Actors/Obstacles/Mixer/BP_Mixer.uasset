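; Puzzle mixer obstacle that stores colors inked by the player, combines them into new colors and lets the player absorb them.
; Ink pushes the player's color onto MixerContents and leaves them transparent, while Absorb pops the last entry back.
; IsMixable matches a full mixer against ColorCombinations in either order, and Mix swaps in the result after a delay.
; SetMixerTable shows contents as one centered or two side meshes with color pointer widgets.
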(event Custom|Mix
  (params (MixedColor :type PDA%20Color%20Object%20Reference))
  (bind _mixercontents (Variables|Default|GetMixerContents))
  (bind _returnvalue (Utilities|Array|Length _mixercontents))
  (Audio|PlaySound2D "/Game/OctoInkContent/Assets/SFX/sounds/MixSfx.MixSfx" 1.0 1.0 0.0 0 0)
  (while (!= _returnvalue 0)
    (Utilities|Array|RemoveItem _mixercontents (Utilities|Array|Get(acopy) _mixercontents (- _returnvalue 1))))
  (CallFunction|SetMixerTable)
  (Utilities|FlowControl|Delay 1.0)
  (Utilities|Array|Add _mixercontents MixedColor)
  (CallFunction|SetMixerTable)
  (Default|CallMixCompleted))

(event EventBeginPlay
  (|CallParentFunction)
  (CallFunction|SetMixerTable)
  (for _array_element (Utilities|Array|MakeArray (Variables|Default|GetLeftWidget) (Variables|Default|GetRightWidget) (Variables|Default|GetCenterWidget))
    (bind _asbp_base_player (Utilities|Casting|CastToBP_BasePlayer (Game|Player|GetPlayerPawn 0)))
    (Transformation|SetWorldRotation _array_element (Math|Rotator|FindLookatRotation (Transformation|GetWorldLocation (Variables|/Script/Paper2D.PaperCharacter|GetSprite _asbp_base_player)) (Transformation|GetWorldLocation (Variables|/Game/OctoInkContent/Blueprints/Actors/Player/BP_BasePlayer.BP_BasePlayer_C|GetCamera _asbp_base_player))) false false)
    (bind _asbp_obstacle_pointer (Utilities|Casting|CastToBP_ObstaclePointer (UserInterface|GetWidget _array_element)))
    (Default|HideAllMouse _asbp_obstacle_pointer)
    (Default|SetLockColor _asbp_obstacle_pointer)
    (Variables|Default|SetTransparentColor "/Game/OctoInkContent/DataAssets/DataAssets/Color/DA_Transparent.DA_Transparent")))

(event Collision|EventActorBeginOverlap
  (params (OtherActor :type Actor%20Object%20Reference))
  (|CallParentFunction OtherActor) ; This node is disabled and will not be called.\nDrag off pins to build functionality.
)

(event EventTick
  (params (DeltaSeconds :type Float%20%28single-precision%29))
  (|CallParentFunction DeltaSeconds))

(event EventAbsorb
  (bind _mixercontents (Variables|Default|GetMixerContents))
  (bind _returnvalue (Utilities|Array|Length _mixercontents))
  (bind _returnvalue_2 (- _returnvalue 1))
  (bind _asbp_puzzle_player (Utilities|Casting|CastToBP_PuzzlePlayer (Game|Player|GetPlayerPawn 0)))
  (Default|SetPlayerColor _asbp_puzzle_player (Utilities|Array|Get(acopy) _mixercontents _returnvalue_2))
  (Utilities|Array|RemoveIndex _mixercontents _returnvalue_2)
  (CallFunction|SetMixerTable))

(event EventInk
  (bind _asbp_puzzle_player (Utilities|Casting|CastToBP_PuzzlePlayer (Game|Player|GetPlayerPawn 0)))
  (Utilities|Array|Add (Variables|Default|GetMixerContents) (Variables|/Game/OctoInkContent/Blueprints/Actors/Player/BP_PuzzlePlayer.BP_PuzzlePlayer_C|GetCurrentColor _asbp_puzzle_player))
  (CallFunction|SetMixerTable)
  (Default|SetPlayerColor _asbp_puzzle_player (Variables|Default|GetTransparentColor)))

(fn ConstructionScript
  (|CallParentFunction))

(fn IsInkable
  (return (< (Utilities|Array|Length (Variables|Default|GetMixerContents)) (Variables|Default|GetMixerMaxSize))))

(fn IsAbsorbable
  (return (> (Utilities|Array|Length (Variables|Default|GetMixerContents)) 0)))

(fn IsMixable
  (bind _mixercontents (Variables|Default|GetMixerContents))
  (bind _output (Utilities|Array|Get(acopy) _mixercontents 1))
  (bind _output_2 (Utilities|Array|Get(acopy) _mixercontents))
  (bind _color (Variables|/Game/OctoInkContent/DataAssets/DataAssets/Color/PDA_Color.PDA_Color_C|GetColor _output_2))
  (bind _color_2 (Variables|/Game/OctoInkContent/DataAssets/DataAssets/Color/PDA_Color.PDA_Color_C|GetColor _output))
  (if (== (Utilities|Array|Length (Variables|Default|GetMixerContents)) (Variables|Default|GetMixerMaxSize))
    (bind _array_element (Utilities|Array|ForEachLoopwithBreak (Variables|Default|GetColorCombinations))
      (:LoopBody
        (bind _output_get (LocalVariables|SetColorMatches (or (and (Utilities|Enum|Equal(Enum) (.firstcolor _array_element) _color) (Utilities|Enum|Equal(Enum) (.secondcolor _array_element) _color_2)) (and (Utilities|Enum|Equal(Enum) (.secondcolor _array_element) _color) (Utilities|Enum|Equal(Enum) (.firstcolor _array_element) _color_2)))))
        (if _output_get
          (return true (.output _array_element))))
      (:Completed
        (return false 0)))
    (else
      (return false 0))))

(fn SetMixerTable
  (switch int (Utilities|Array|Length (Variables|Default|GetMixerContents))
    (:0
      (Development|SetHiddeninGame (Variables|Default|GetLeftMaterial) true true)
      (Development|SetHiddeninGame (Variables|Default|GetRightMaterial) true true)
      (Development|SetHiddeninGame (Variables|Default|GetCenterMaterial) true true))
    (:1
      (Development|SetHiddeninGame (Variables|Default|GetLeftMaterial) true true)
      (Development|SetHiddeninGame (Variables|Default|GetRightMaterial) true true)
      (Development|SetHiddeninGame (Variables|Default|GetCenterMaterial) false true)
      (CallFunction|SetMixerColor (Utilities|Array|MakeArray (Variables|Default|GetCenterMaterial)) (Utilities|Array|MakeArray (Variables|Default|GetCenterWidget))))
    (:2
      (Development|SetHiddeninGame (Variables|Default|GetLeftMaterial) false true)
      (Development|SetHiddeninGame (Variables|Default|GetRightMaterial) false true)
      (Development|SetHiddeninGame (Variables|Default|GetCenterMaterial) true true)
      (CallFunction|SetMixerColor (Utilities|Array|MakeArray (Variables|Default|GetLeftMaterial) (Variables|Default|GetRightMaterial)) (Utilities|Array|MakeArray (Variables|Default|GetLeftWidget) (Variables|Default|GetRightWidget))))))

(fn SetMixerColor
  (params (StaticMesh :type Array%20of%20Static%20Mesh%20Component%20Object%20References) (WidgetComponenet :type Array%20of%20Widget%20Component%20Object%20References))
  (for (_array_element _array_index) (Variables|Default|GetMixerContents)
    (Utilities|FlowControl|Sequence
      (:then_0
        ;[1 1 1] Setting Material In Table
        (Rendering|Material|SetMaterial (Utilities|Array|Get(acopy) StaticMesh _array_index) 0 (Variables|/Game/OctoInkContent/DataAssets/DataAssets/Color/PDA_Color.PDA_Color_C|GetBridgeMaterial _array_element)))
      (:then_1
        ;[1 1 1] Set Pointer Color
        (bind _asbp_obstacle_pointer (Utilities|Casting|CastToBP_ObstaclePointer (UserInterface|GetUserWidgetObject (Utilities|Array|Get(acopy) WidgetComponenet _array_index))))
        (Default|SetPointerColor _asbp_obstacle_pointer _array_element)))))