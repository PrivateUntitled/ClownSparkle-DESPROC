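; Bus stop obstacle actor that opens the map panel when the player interacts with it.
; On BeginPlay it caches the player controller and rotates its widget once to match the direction from the player's sprite to the camera.
; DoInteraction runs only while movement is enabled: it flags the map as open, clears all widgets, disables movement, shows the mouse cursor and adds BP_MapPanel to the viewport.
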(event EventBeginPlay
  (|CallParentFunction)
  (Utilities|FlowControl|Sequence
    (:then_0
      (bind _asbp_base_player (Utilities|Casting|CastToBP_BasePlayer (Game|Player|GetPlayerPawn 0)))
      (Transformation|SetWorldRotation (Variables|Default|GetWidget) (Math|Rotator|FindLookatRotation (Transformation|GetWorldLocation (Variables|/Script/Paper2D.PaperCharacter|GetSprite _asbp_base_player)) (Transformation|GetWorldLocation (Variables|/Game/OctoInkContent/Blueprints/Actors/Player/BP_BasePlayer.BP_BasePlayer_C|GetCamera _asbp_base_player))) false false))
    (:then_1
      (bind _asbp_player_base_controller (Utilities|Casting|CastToBP_PlayerBaseController (Game|GetPlayerController 0)))
      (Variables|Default|SetNewVar_0 _asbp_player_base_controller))))

(event Collision|EventActorBeginOverlap
  (params (OtherActor :type Actor%20Object%20Reference))
  (|CallParentFunction OtherActor) ; This node is disabled and will not be called.\nDrag off pins to build functionality.
)

(event EventTick
  (params (DeltaSeconds :type Float%20%28single-precision%29))
  (|CallParentFunction DeltaSeconds) ; This node is disabled and will not be called.\nDrag off pins to build functionality.
)

(event EventDoInteraction
  (bind _returnvalue (Game|GetPlayerController 0))
  (|CallParentFunction)
  (if (Variables|/Game/OctoInkContent/Blueprints/Controllers/BP_PlayerBaseController.BP_PlayerBaseController_C|GetEnableMovement (Variables|Default|GetNewVar_0))
    (Variables|/Game/OctoInkContent/Blueprints/Controllers/BP_PlayerBaseController.BP_PlayerBaseController_C|SetIsMapOpen (Variables|Default|GetNewVar_0) true)
    (Viewport|RemoveAllWidgets)
    (Utilities|FlowControl|Sequence
      (:then_0
        ;[1 1 1] Setting Movement
        (bind _asbp_player_base_controller (Utilities|Casting|CastToBP_PlayerBaseController _returnvalue))
        (Variables|/Game/OctoInkContent/Blueprints/Controllers/BP_PlayerBaseController.BP_PlayerBaseController_C|SetEnableMovement _asbp_player_base_controller false))
      (:then_1
        ;[1 1 1] Setting Mouse Cursor Visibility
        (Variables|/Script/Engine.PlayerController|SetbShowMouseCursor _returnvalue true))
      (:then_2
        (Viewport|RemoveAllWidgets))
      (:then_3
        ;[1 1 1] Adding New Widget
        (if true
          (bind _returnvalue_2 (UserInterface|CreateWidget "/Game/OctoInkContent/Blueprints/Widgets/BP_MapPanel.BP_MapPanel_C"))
          (UserInterface|Viewport|AddtoViewport _returnvalue_2 0))))))

(fn ConstructionScript
  (|CallParentFunction))