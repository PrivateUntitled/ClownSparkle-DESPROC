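; BP_Blockade is a colored obstacle Blueprint that specializes a parent obstacle class for blockades.
; SetObstacleColor stores the new color, applies its blockade material to the static mesh, then switches the mesh's collision object type.
; One specific color value uses a custom collision channel, while all others use WorldStatic.
; Lowering, raising, requirement setup and player color comparison all defer to the parent.
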(event EventBeginPlay
  (|CallParentFunction))

(event Collision|EventActorBeginOverlap
  (params (OtherActor :type Actor%20Object%20Reference)))

(event EventTick
  (params (DeltaSeconds :type Float%20%28single-precision%29))
  (|CallParentFunction DeltaSeconds))

(event EventLower
  (|CallParentFunction))

(event EventRaise
  (|CallParentFunction))

(fn ConstructionScript)

(fn SetObstacleRequirement
  (|CallParentFunction))

(fn SetObstacleColor
  (params (SetColor :type PDA%20Color%20Object%20Reference))
  (|CallParentFunction SetColor)
  (Utilities|FlowControl|Sequence
    (:then_0
      (bind _output_get (Variables|Default|SetCurrentColor SetColor))
      (Rendering|Material|SetMaterial (Variables|Default|GetStaticMesh) 0 (Variables|/Game/OctoInkContent/DataAssets/DataAssets/Color/PDA_Color.PDA_Color_C|GetBlockadeMaterial _output_get)))
    (:then_1
      (if (Utilities|Enum|NotEqual(Enum) (Variables|/Game/OctoInkContent/DataAssets/DataAssets/Color/PDA_Color.PDA_Color_C|GetColor (Variables|Default|GetCurrentColor)) "NewEnumerator6")
        (Collision|SetCollisionObjectType (Variables|Default|GetStaticMesh) "ECC_WorldStatic")
        (else
          (Collision|SetCollisionObjectType (Variables|Default|GetStaticMesh) "ECC_GameTraceChannel1"))))))

(fn IsEqualtoPlayerColor
  (params (PlayerColor :type Colors%20Enum :default "NewEnumerator0"))
  (bind _notequaltoplayercolor (|CallParentFunction PlayerColor))
  (return _notequaltoplayercolor))