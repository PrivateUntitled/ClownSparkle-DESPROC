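; BP_TempNpc is a placeholder NPC actor that recolors a bridge obstacle when interacted with.
; On the first DoInteraction event, it sets the referenced Bridge's obstacle color to the orange data asset and plays an ink sound, with a DoOnce blocking repeats.
; BeginPlay caches the puzzle player character, though nothing else in this Blueprint uses that reference.
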(event EventBeginPlay
  (|CallParentFunction)
  (bind _asbp_puzzle_player (Utilities|Casting|CastToBP_PuzzlePlayer (Game|GetPlayerCharacter 0)))
  (Variables|Default|SetAs%20BP%20Puzzle%20Player _asbp_puzzle_player))

(event Collision|EventActorBeginOverlap
  (params (OtherActor :type Actor%20Object%20Reference))
  (|CallParentFunction OtherActor) ; This node is disabled and will not be called.\nDrag off pins to build functionality.
)

(event EventTick
  (params (DeltaSeconds :type Float%20%28single-precision%29))
  (|CallParentFunction DeltaSeconds) ; This node is disabled and will not be called.\nDrag off pins to build functionality.
)

(event EventDoInteraction
  (Utilities|FlowControl|DoOnce false
    (:Completed
      (Default|SetObstacleColor (Variables|Default|GetBridge) "/Game/OctoInkContent/DataAssets/DataAssets/Color/DA_Orange.DA_Orange")
      (Audio|PlaySound2D "/Game/OctoInkContent/Assets/SFX/sounds/Ink.Ink" 1.0 1.0 0.0 0 0))))

(fn ConstructionScript
  (|CallParentFunction))