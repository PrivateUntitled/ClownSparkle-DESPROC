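; BP_ColorSource is an obstacle Blueprint that acts as a color source and responds to being absorbed.
; On BeginPlay it applies its current color, and on Absorb it runs the parent logic, then calls GetColor.
; Its SetObstacleColor override stores the color, swaps in that color's source material and sets the mesh's collision object type to WorldStatic.
; Requirement and player-color checks defer to the parent.
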(event EventBeginPlay
  (|CallParentFunction)
  (CallFunction|SetColSourceColor (Variables|Default|GetCurrentColor)))

(event Collision|EventActorBeginOverlap
  (params (OtherActor :type Actor%20Object%20Reference))
  (|CallParentFunction OtherActor) ; This node is disabled and will not be called.\nDrag off pins to build functionality.
)

(event EventTick
  (params (DeltaSeconds :type Float%20%28single-precision%29))
  (|CallParentFunction DeltaSeconds) ; This node is disabled and will not be called.\nDrag off pins to build functionality.
)

(event EventAbsorb
  (|CallParentFunction)
  (CallFunction|GetColor))

(fn ConstructionScript
  (|CallParentFunction))

(fn SetObstacleRequirement
  (|CallParentFunction))

(fn SetObstacleColor
  (params (SetColor :type PDA%20Color%20Object%20Reference))
  (|CallParentFunction SetColor)
  (bind _output_get (Variables|Default|SetCurrentColor SetColor))
  (Rendering|Material|SetMaterial (Variables|Default|GetStaticMesh) 0 (Variables|/Game/OctoInkContent/DataAssets/DataAssets/Color/PDA_Color.PDA_Color_C|GetColorSourceMaterial _output_get))
  (Collision|SetCollisionObjectType (Variables|Default|GetStaticMesh) "ECC_WorldStatic"))

(fn IsEqualtoPlayerColor
  (params (PlayerColor :type Colors%20Enum :default "NewEnumerator7"))
  (bind _notequaltoplayercolor (|CallParentFunction PlayerColor))
  (return _notequaltoplayercolor))