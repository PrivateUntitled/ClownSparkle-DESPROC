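; Player controller that handles input for BP_BasePlayer: movement, dash, interaction, dialogue, and the pause, mixing guide and debug menus.
; WASD moves along diagonal world axes, and truncated axis values pick one of eight directions, setting six animator facings and the collider's rotation.
; Dash briefly boosts speed and acceleration before a cooldown.
; Menus disable movement, while event dispatchers broadcast actions and Interact notifies the in-range interactable, puzzle or NPC.
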(event Custom|Dash
  (bind _playercharacterref (Variables|Default|GetPlayerCharacterRef))
  (bind _playercharacterref_2 (Variables|Default|GetPlayerCharacterRef))
  (bind _charactermovement (Variables|/Script/Engine.Character|GetCharacterMovement _playercharacterref))
  (bind _charactermovement_2 (Variables|/Script/Engine.Character|GetCharacterMovement _playercharacterref_2))
  ;[1 1 1] Dash Ability
  (if (!= (Variables|Default|GetDashMultiplier) 0.0)
    (Audio|PlaySound2D (.OutItem (Utilities|Array|Random (Variables|Default|GetDashSound))) 1.0 1.0 0.0 0 0)
    (Utilities|FlowControl|Sequence
      (:then_0
        ;;[0.4706 0 1] Activate the Dash
        (Variables|Default|SetCanDash false)
        (Variables|/Script/Engine.CharacterMovementComponent|SetMaxWalkSpeed _charactermovement (* (Variables|/Script/Engine.CharacterMovementComponent|GetMaxWalkSpeed (Variables|/Script/Engine.Character|GetCharacterMovement (Variables|Default|GetPlayerCharacterRef))) (Variables|Default|GetDashMultiplier)))
        (Variables|/Script/Engine.CharacterMovementComponent|SetMaxAcceleration _charactermovement 1e+04)
        (Components|Activation|SetActive (Variables|/Game/OctoInkContent/Blueprints/Actors/Player/BP_BasePlayer.BP_BasePlayer_C|GetDashFX (Variables|Default|GetPlayerCharacterRef)) true false))
      (:then_1
        ;;[0.4706 0 1] Deactivate the Dash
        (Utilities|FlowControl|Delay 0.2)
        (Variables|/Script/Engine.CharacterMovementComponent|SetMaxWalkSpeed _charactermovement_2 (/ (Variables|/Script/Engine.CharacterMovementComponent|GetMaxWalkSpeed _charactermovement_2) (Variables|Default|GetDashMultiplier)))
        (Variables|/Script/Engine.CharacterMovementComponent|SetMaxAcceleration _charactermovement_2 2048.0)
        (Components|Activation|SetActive (Variables|/Game/OctoInkContent/Blueprints/Actors/Player/BP_BasePlayer.BP_BasePlayer_C|GetDashFX (Variables|Default|GetPlayerCharacterRef)) false false))
      (:then_2
        ;;[0.4706 0 1] Dash Cooldown
        (Utilities|FlowControl|Delay 1.0)
        (Variables|Default|SetCanDash true))
      (:then_3
        (Default|CallHasDashed)))))

(event Custom|Movement
  (bind _xaxis (Variables|Default|GetXAxis))
  (bind _returnvalue (Math|Float|Truncate _xaxis))
  ;[1 1 1] Setting Player Directions
  (if (Variables|Default|GetEnableMovement)
    (switch int (Math|Float|Truncate (Variables|Default|GetYAxis))
      (:-1
        (switch int _returnvalue
          (:-1
            (CallFunction|SetAnimation "NewEnumerator4"))
          (:0
            (CallFunction|SetAnimation "NewEnumerator2"))
          (:1
            (CallFunction|SetAnimation "NewEnumerator1"))))
      (:0
        (switch int _returnvalue
          (:-1
            (CallFunction|SetAnimation "NewEnumerator5"))
          (:0
            (CallFunction|SetAnimation "NewEnumerator3"))
          (:1
            (CallFunction|SetAnimation "NewEnumerator0"))))
      (:1
        (switch int _returnvalue
          (:-1
            (CallFunction|SetAnimation "NewEnumerator6"))
          (:0
            (CallFunction|SetAnimation "NewEnumerator7"))
          (:1
            (CallFunction|SetAnimation "NewEnumerator8")))))))

(event Custom|SetAnimation
  (params (Direction :type Directions%20Enum :default "NewEnumerator3"))
  (bind _playercharacterref (Variables|Default|GetPlayerCharacterRef))
  (bind _scene (Variables|/Game/OctoInkContent/Blueprints/Actors/Player/BP_BasePlayer.BP_BasePlayer_C|GetScene _playercharacterref))
  (Utilities|FlowControl|Sequence
    (:then_0
      ;[1 1 1] Setting Animation
      (bind _asbp_player_animator (Utilities|Casting|CastToBP_PlayerAnimator (Variables|/Script/PaperZD.PaperZDAnimationComponent|GetAnimInstance (Variables|/Script/PaperZD.PaperZDCharacter|GetAnimationComponent _playercharacterref))))
      (switch Utilities|FlowControl|Switch|SwitchonDirections Direction
        (:NewEnumerator0
          (Variables|/Game/OctoInkContent/Blueprints/Actors/Player/BP_PlayerAnimator.BP_PlayerAnimator_C|SetDirection _asbp_player_animator 3 :!label _label))
        (:NewEnumerator1
          (goto _label))
        (:NewEnumerator2
          (Variables|/Game/OctoInkContent/Blueprints/Actors/Player/BP_PlayerAnimator.BP_PlayerAnimator_C|SetDirection _asbp_player_animator 1))
        (:NewEnumerator4
          (Variables|/Game/OctoInkContent/Blueprints/Actors/Player/BP_PlayerAnimator.BP_PlayerAnimator_C|SetDirection _asbp_player_animator 2 :!label _label_2))
        (:NewEnumerator5
          (goto _label_2))
        (:NewEnumerator6
          (Variables|/Game/OctoInkContent/Blueprints/Actors/Player/BP_PlayerAnimator.BP_PlayerAnimator_C|SetDirection _asbp_player_animator 4))
        (:NewEnumerator7
          (Variables|/Game/OctoInkContent/Blueprints/Actors/Player/BP_PlayerAnimator.BP_PlayerAnimator_C|SetDirection _asbp_player_animator 0))
        (:NewEnumerator8
          (Variables|/Game/OctoInkContent/Blueprints/Actors/Player/BP_PlayerAnimator.BP_PlayerAnimator_C|SetDirection _asbp_player_animator 5))))
    (:then_1
      ;[1 1 1] Set Collider Rotation
      (switch Utilities|FlowControl|Switch|SwitchonDirections Direction
        (:NewEnumerator0
          (Transformation|SetWorldRotation _scene "0,45.000000, 0" false false))
        (:NewEnumerator1
          (Transformation|SetWorldRotation _scene "0,90.000000, 0" false false))
        (:NewEnumerator2
          (Transformation|SetWorldRotation _scene "0,135.000000, 0" false false))
        (:NewEnumerator4
          (Transformation|SetWorldRotation _scene "0,180.000000, 0" false false))
        (:NewEnumerator5
          (Transformation|SetWorldRotation _scene "0,225.000000, 0" false false))
        (:NewEnumerator6
          (Transformation|SetWorldRotation _scene "0,270.000000, 0" false false))
        (:NewEnumerator7
          (Transformation|SetWorldRotation _scene "0,315.000000, 0" false false))
        (:NewEnumerator8
          (Transformation|SetWorldRotation _scene "0, 0, 0" false false))))))

(event EventBeginPlay
  (bind _asbp_base_player (Utilities|Casting|CastToBP_BasePlayer (Game|GetPlayerCharacter 0)))
  (Variables|Default|SetPlayerCharacterRef _asbp_base_player)
  (bind _asmy_game (Utilities|Casting|CastToMyGame (Game|GetGameInstance)))
  (Variables|Default|SetGameInstanceRef _asmy_game))

(event EventTick
  (params (DeltaSeconds :type Float%20%28single-precision%29)))

(event Input|ActionEvents|InputActionPause
  (params (Key :type Key%20Structure))
  ;[1 1 1] Activate Pause Menu
  (:Pressed
    (if (not (Variables|Default|GetisPauseMenuOpen))
      (bind _returnvalue (UserInterface|CreateWidget "/Game/OctoInkContent/Blueprints/Widgets/GeneralWidgets/OverlayWidgets/BP_PauseMenuWidget.BP_PauseMenuWidget_C"))
      (Default|SetPreviousStatus _returnvalue (Variables|Default|GetEnableMovement) (Variables|Default|GetbShowMouseCursor))
      (UserInterface|Viewport|AddtoViewport _returnvalue 0)
      (Variables|/Script/Engine.PlayerController|SetbShowMouseCursor self true)
      (Variables|Default|SetEnableMovement false)
      (Audio|PlaySound2D "/Game/OctoInkContent/Assets/SFX/sounds/MenuSounds/Root_Tone.Root_Tone" 1.0 1.0 0.0 0 0)
      (Default|CallUpdatePauseStatus true))))

(event Input|ActionEvents|InputActionDash
  (params (Key :type Key%20Structure))
  ;[1 1 1] Dash Mechanic (Hook to implement)
  (:Pressed
    (if (Variables|Default|GetEnableMovement)
      (if (Variables|Default|GetCanDash)
        (CallFunction|Dash)))))

(event Input|ActionEvents|InputActionMixingGuide
  (params (Key :type Key%20Structure))
  ;[1 1 1] Activate Mixing Guide
  (:Pressed
    (if (Variables|Default|GetIsMixingGuideOpen)
      (Default|ExitMixingGuide (Variables|Default|GetMixingGuideRef))
      (elif (Math|Boolean|ANDBoolean (not (Variables|Default|GetInDialogue)) (not (Variables|Default|GetIsMapOpen)) (not (Variables|Default|GetisOnMinigame)) (Utilities|Struct|BreakMenuData (Variables|/Game/OctoInkContent/Blueprints/SaveData/MyGame.MyGame_C|GetGameStateData (Variables|Default|GetGameInstanceRef))))
        (Audio|PlaySound2D "/Game/OctoInkContent/Assets/SFX/sounds/MenuSounds/Root_Tone.Root_Tone" 1.0 1.0 0.0 0 0)
        (Default|CallHasOpenedMixingGuide)
        (bind _returnvalue (UserInterface|CreateWidget "/Game/OctoInkContent/Blueprints/Widgets/BP_MixingGuide.BP_MixingGuide_C"))
        (Variables|Default|SetIsMixingGuideOpen true)
        (Variables|/Script/Engine.PlayerController|SetbShowMouseCursor self true)
        (Variables|Default|SetEnableMovement false)
        (bind _output_get (Variables|Default|SetMixingGuideRef _returnvalue))
        (UserInterface|Viewport|AddtoViewport _output_get 0)))))

(event Input|ActionEvents|InputActionOpenDebugMenu
  (params (Key :type Key%20Structure))
  (:Pressed
    (if (not (Variables|Default|GetisPauseMenuOpen))
      (Variables|Default|SetbShowMouseCursor true)
      (Variables|Default|SetEnableMovement false)
      (Variables|Default|SetisPauseMenuOpen true)
      (bind _returnvalue (UserInterface|CreateWidget "/Game/OctoInkContent/Blueprints/Widgets/BP_CheatMenu.BP_CheatMenu_C"))
      (Variables|Default|SetDebugMenu _returnvalue)
      (UserInterface|Viewport|AddtoViewport _returnvalue 0)
      (Default|CallHasOpenedDebugMenu))))

(event Input|ActionEvents|InputActionDialogue
  (params (Key :type Key%20Structure))
  (:Pressed
    (if (not (Variables|Default|GetisPauseMenuOpen))
      (Default|CallProceedNextDialogue))))

(event Input|ActionEvents|InputActionInteract
  (params (Key :type Key%20Structure))
  (:Pressed
    (if (not (Variables|Default|GetisPauseMenuOpen))
      (bind _asbp_base_player (Utilities|Casting|CastToBP_BasePlayer (Game|Player|GetPlayerPawn 0)))
      (Utilities|FlowControl|Sequence
        (:then_0
          (bind _asbp_interactables (Utilities|Casting|CastToBP_Interactables (Variables|/Game/OctoInkContent/Blueprints/Actors/Player/BP_BasePlayer.BP_BasePlayer_C|GetObjectInRange _asbp_base_player)))
          (Default|CallInteractedwithObject _asbp_interactables))
        (:then_1
          (bind _asbp_puzzle_interactable (Utilities|Casting|CastToBP_PuzzleInteractable (Variables|/Game/OctoInkContent/Blueprints/Actors/Player/BP_BasePlayer.BP_BasePlayer_C|GetObjectInRange _asbp_base_player)))
          (Default|CallInteractedwithPuzzle _asbp_puzzle_interactable))
        (:then_2
          (bind _asbp_base_interactable_npc (Utilities|Casting|CastToBP_BaseInteractableNPC (Variables|/Game/OctoInkContent/Blueprints/Actors/Player/BP_BasePlayer.BP_BasePlayer_C|GetObjectInRange _asbp_base_player)))
          (Default|CallInteractedwithNPC _asbp_base_interactable_npc))))))

(event Input|ActionEvents|InputActionJump
  (params (Key :type Key%20Structure))
  ;[1 0 0] Jump Mechanic (Hook to Implement) [ARCHIVED]
)

(event Input|AxisEvents|InputAxisMoveForward
  (params (AxisValue :type Float%20%28single-precision%29))
  ;[1 1 1] WASD Movement
  (if (Variables|Default|GetEnableMovement)
    (bind _output_get (Variables|Default|SetYAxis AxisValue))
    (Pawn|Input|AddMovementInput (Variables|Default|GetPlayerCharacterRef) "1.000000,-1.000000, 0" _output_get false)
    (CallFunction|Movement)))

(event Input|AxisEvents|InputAxisMoveRight
  (params (AxisValue :type Float%20%28single-precision%29))
  ;[1 1 1] WASD Movement
  (if (Variables|Default|GetEnableMovement)
    (bind _output_get (Variables|Default|SetXAxis AxisValue))
    (Pawn|Input|AddMovementInput (Variables|Default|GetPlayerCharacterRef) "1.000000,1.000000, 0" _output_get false)
    (CallFunction|Movement)))

(fn ConstructionScript)