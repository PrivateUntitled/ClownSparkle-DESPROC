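; Archived player controller that drives the BasePlayer character with diagonal world-axis movement, suited to an angled camera, plus a Space bar dash.
; Dash briefly spikes walk speed and acceleration, restores them, then waits out a cooldown.
; WASD press and release events set a Direction on BP_PlayerAnimator, falling back to keys still held; A and S share one value.
; Jump and diagonal-facing logic are left unconnected.
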(event Custom|Dash
  (bind _playercharacterref (Variables|Default|GetPlayerCharacterRef))
  (bind _charactermovement (Variables|/Script/Engine.Character|GetCharacterMovement _playercharacterref))
  (Variables|Default|SetCanDash false)
  (Variables|/Script/Engine.CharacterMovementComponent|SetMaxWalkSpeed _charactermovement 1e+04)
  (Variables|/Script/Engine.CharacterMovementComponent|SetMaxAcceleration _charactermovement 1e+04)
  (Utilities|FlowControl|Delay 0.2)
  (Variables|/Script/Engine.CharacterMovementComponent|SetMaxWalkSpeed _charactermovement 6e+02)
  (Variables|/Script/Engine.CharacterMovementComponent|SetMaxAcceleration _charactermovement 2048.0)
  (Utilities|FlowControl|Delay 1.0)
  (Variables|Default|SetCanDash true))

(event EventBeginPlay
  (bind _asbase_player (Utilities|Casting|CastToBasePlayer (Game|GetPlayerCharacter 0)))
  (Variables|Default|SetPlayerCharacterRef _asbase_player))

(event EventTick
  (params (DeltaSeconds :type Float%20%28single-precision%29)))

(event Input|ActionEvents|InputActionJump
  (params (Key :type Key%20Structure))
  ;[1 1 1] Jump Mechanic (Hook to Implement)
)

(event Input|AxisEvents|InputAxisMoveForward
  (params (AxisValue :type Float%20%28single-precision%29))
  ;[1 1 1] WASD Movement
  (Pawn|Input|AddMovementInput (Variables|Default|GetPlayerCharacterRef) "1.000000,-1.000000, 0" AxisValue false))

(event Input|AxisEvents|InputAxisMoveRight
  (params (AxisValue :type Float%20%28single-precision%29))
  ;[1 1 1] WASD Movement
  (Pawn|Input|AddMovementInput (Variables|Default|GetPlayerCharacterRef) "1.000000,1.000000, 0" AxisValue false))

(event Input|KeyboardEvents|A
  (params (Key :type Key%20Structure))
  (bind _playercharacterref (Variables|Default|GetPlayerCharacterRef))
  (bind _animationcomponent (Variables|/Script/PaperZD.PaperZDCharacter|GetAnimationComponent _playercharacterref))
  (bind _animinstance (Variables|/Script/PaperZD.PaperZDAnimationComponent|GetAnimInstance _animationcomponent))
  ;[1 1 1] Primary Directions
  (:Pressed
    (bind _asbp_player_animator (Utilities|Casting|CastToBP_PlayerAnimator _animinstance))
    (Variables|/Game/OctoInkContent/Blueprints/Actors/Player/BP_PlayerAnimator.BP_PlayerAnimator_C|SetDirection _asbp_player_animator 0))
  (:Released
    (if (Game|Player|IsInputKeyDown "W")
      (bind _asbp_player_animator_2 (Utilities|Casting|CastToBP_PlayerAnimator _animinstance))
      (Variables|/Game/OctoInkContent/Blueprints/Actors/Player/BP_PlayerAnimator.BP_PlayerAnimator_C|SetDirection _asbp_player_animator_2 3)
      (elif (Game|Player|IsInputKeyDown "S")
        (bind _asbp_player_animator_3 (Utilities|Casting|CastToBP_PlayerAnimator _animinstance))
        (Variables|/Game/OctoInkContent/Blueprints/Actors/Player/BP_PlayerAnimator.BP_PlayerAnimator_C|SetDirection _asbp_player_animator_3 0)
        (elif (Game|Player|IsInputKeyDown "D")
          (bind _asbp_player_animator_4 (Utilities|Casting|CastToBP_PlayerAnimator _animinstance))
          (Variables|/Game/OctoInkContent/Blueprints/Actors/Player/BP_PlayerAnimator.BP_PlayerAnimator_C|SetDirection _asbp_player_animator_4 1))))))

(event Input|KeyboardEvents|SpaceBar
  (params (Key :type Key%20Structure))
  ;[1 1 1] Dash Mechanic (Hook to implement)
  (:Pressed
    (if (Variables|Default|GetCanDash)
      (CallFunction|Dash))))

(event Input|KeyboardEvents|W
  (params (Key :type Key%20Structure))
  (bind _playercharacterref (Variables|Default|GetPlayerCharacterRef))
  (bind _animationcomponent (Variables|/Script/PaperZD.PaperZDCharacter|GetAnimationComponent _playercharacterref))
  (bind _animinstance (Variables|/Script/PaperZD.PaperZDAnimationComponent|GetAnimInstance _animationcomponent))
  ;[1 1 1] Primary Directions
  (:Pressed
    (bind _asbp_player_animator (Utilities|Casting|CastToBP_PlayerAnimator _animinstance))
    (Variables|/Game/OctoInkContent/Blueprints/Actors/Player/BP_PlayerAnimator.BP_PlayerAnimator_C|SetDirection _asbp_player_animator 3))
  (:Released
    (if (Game|Player|IsInputKeyDown "D")
      (bind _asbp_player_animator_2 (Utilities|Casting|CastToBP_PlayerAnimator _animinstance :!label _label))
      (Variables|/Game/OctoInkContent/Blueprints/Actors/Player/BP_PlayerAnimator.BP_PlayerAnimator_C|SetDirection _asbp_player_animator_2 0)
      (elif (Game|Player|IsInputKeyDown "A")
        (goto _label)
        (elif (Game|Player|IsInputKeyDown "S")
          (bind _asbp_player_animator_3 (Utilities|Casting|CastToBP_PlayerAnimator _animinstance))
          (Variables|/Game/OctoInkContent/Blueprints/Actors/Player/BP_PlayerAnimator.BP_PlayerAnimator_C|SetDirection _asbp_player_animator_3 0))))))

(event Input|KeyboardEvents|S
  (params (Key :type Key%20Structure))
  (bind _playercharacterref (Variables|Default|GetPlayerCharacterRef))
  (bind _animationcomponent (Variables|/Script/PaperZD.PaperZDCharacter|GetAnimationComponent _playercharacterref))
  (bind _animinstance (Variables|/Script/PaperZD.PaperZDAnimationComponent|GetAnimInstance _animationcomponent))
  ;[1 1 1] Primary Directions
  (:Pressed
    (bind _asbp_player_animator (Utilities|Casting|CastToBP_PlayerAnimator _animinstance))
    (Variables|/Game/OctoInkContent/Blueprints/Actors/Player/BP_PlayerAnimator.BP_PlayerAnimator_C|SetDirection _asbp_player_animator 0))
  (:Released
    (if (Game|Player|IsInputKeyDown "D")
      (bind _asbp_player_animator_2 (Utilities|Casting|CastToBP_PlayerAnimator _animinstance))
      (Variables|/Game/OctoInkContent/Blueprints/Actors/Player/BP_PlayerAnimator.BP_PlayerAnimator_C|SetDirection _asbp_player_animator_2 0)
      (elif (not (Game|Player|IsInputKeyDown "A"))
        (if (Game|Player|IsInputKeyDown "W")
          (bind _asbp_player_animator_3 (Utilities|Casting|CastToBP_PlayerAnimator _animinstance))
          (Variables|/Game/OctoInkContent/Blueprints/Actors/Player/BP_PlayerAnimator.BP_PlayerAnimator_C|SetDirection _asbp_player_animator_3 3))))))

(event Input|KeyboardEvents|D
  (params (Key :type Key%20Structure))
  (bind _playercharacterref (Variables|Default|GetPlayerCharacterRef))
  (bind _animationcomponent (Variables|/Script/PaperZD.PaperZDCharacter|GetAnimationComponent _playercharacterref))
  (bind _animinstance (Variables|/Script/PaperZD.PaperZDAnimationComponent|GetAnimInstance _animationcomponent))
  ;[1 1 1] Primary Directions
  (:Pressed
    (bind _asbp_player_animator (Utilities|Casting|CastToBP_PlayerAnimator _animinstance))
    (Variables|/Game/OctoInkContent/Blueprints/Actors/Player/BP_PlayerAnimator.BP_PlayerAnimator_C|SetDirection _asbp_player_animator 1))
  (:Released
    (if (Game|Player|IsInputKeyDown "W")
      (bind _asbp_player_animator_2 (Utilities|Casting|CastToBP_PlayerAnimator _animinstance))
      (Variables|/Game/OctoInkContent/Blueprints/Actors/Player/BP_PlayerAnimator.BP_PlayerAnimator_C|SetDirection _asbp_player_animator_2 3)
      (elif (Game|Player|IsInputKeyDown "S")
        (bind _asbp_player_animator_3 (Utilities|Casting|CastToBP_PlayerAnimator _animinstance))
        (Variables|/Game/OctoInkContent/Blueprints/Actors/Player/BP_PlayerAnimator.BP_PlayerAnimator_C|SetDirection _asbp_player_animator_3 0)
        (elif (Game|Player|IsInputKeyDown "A")
          (bind _asbp_player_animator_4 (Utilities|Casting|CastToBP_PlayerAnimator _animinstance))
          (Variables|/Game/OctoInkContent/Blueprints/Actors/Player/BP_PlayerAnimator.BP_PlayerAnimator_C|SetDirection _asbp_player_animator_4 0))))))

(fn ConstructionScript)