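; Player controller for the main game mode, which on BeginPlay caches the BP_MainGamePlayer pawn and the MyGame game instance.
; No other logic runs, as the remaining graph code is disconnected.
; That dead code holds an old NPC dialogue and quest-start flow with random NPC voice sounds.
; It also holds a debug routine that sets player status from energy consumed and prints it.
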(event EventBeginPlay
  (|CallParentFunction)
  (bind _asbp_main_game_player (Utilities|Casting|CastToBP_MainGamePlayer (Game|Player|GetPlayerPawn 0)))
  (Variables|Default|SetMainGamePlayer _asbp_main_game_player)
  (bind _asmy_game (Utilities|Casting|CastToMyGame (Game|GetGameInstance)))
  (Variables|Default|SetGameInstanceRef_0 _asmy_game))

(event Input|ActionEvents|InputActionSleep(Temporary)
  (params (Key :type Key%20Structure :default "None")))

(fn ConstructionScript
  (|CallParentFunction))