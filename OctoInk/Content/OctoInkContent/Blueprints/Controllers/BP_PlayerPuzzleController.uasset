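; Player controller for puzzle levels, routing input to the puzzle player pawn and the interactable or mixer in range.
; Ink/Absorb inks when the pawn holds color, otherwise absorbs, each followed by a mental-block roll; blocked players clear it by repeated presses.
; Mix and Interact act on the in-range object, with error sounds for invalid ink, absorb or mix.
; Clamped zoom steps slide the camera along its initial slope, saved in game-instance player stats.
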(event EventBeginPlay
  (|CallParentFunction)
  (bind _asbp_puzzle_player (Utilities|Casting|CastToBP_PuzzlePlayer (Game|Player|GetPlayerPawn 0)))
  (Variables|Default|SetPuzzlePlayerRef _asbp_puzzle_player)
  (bind _asbp_base_player (Utilities|Casting|CastToBP_BasePlayer (Game|Player|GetPlayerPawn 0)))
  (Variables|Default|SetCameraSlope (/ (.z (Variables|/Script/Engine.SceneComponent|GetRelativeLocation (Variables|/Game/OctoInkContent/Blueprints/Actors/Player/BP_BasePlayer.BP_BasePlayer_C|GetCamera _asbp_base_player))) (.x (Variables|/Script/Engine.SceneComponent|GetRelativeLocation (Variables|/Game/OctoInkContent/Blueprints/Actors/Player/BP_BasePlayer.BP_BasePlayer_C|GetCamera _asbp_base_player)))))
  (bind _asmy_game (Utilities|Casting|CastToMyGame (Game|GetGameInstance)))
  (Transformation|SetRelativeLocation (Variables|/Game/OctoInkContent/Blueprints/Actors/Player/BP_BasePlayer.BP_BasePlayer_C|GetCamera _asbp_base_player) (Math|Vector|MakeVector (/ (.Zoom (Utilities|Struct|BreakPlayerStats (Variables|/Game/OctoInkContent/Blueprints/SaveData/MyGame.MyGame_C|GetPlayerStats _asmy_game))) (Variables|Default|GetCameraSlope)) (* -1 (/ (.Zoom (Utilities|Struct|BreakPlayerStats (Variables|/Game/OctoInkContent/Blueprints/SaveData/MyGame.MyGame_C|GetPlayerStats _asmy_game))) (Variables|Default|GetCameraSlope))) (.Zoom (Utilities|Struct|BreakPlayerStats (Variables|/Game/OctoInkContent/Blueprints/SaveData/MyGame.MyGame_C|GetPlayerStats _asmy_game)))) false false)
  (Variables|Default|SetZoomScale (.ZoomScale (Utilities|Struct|BreakPlayerStats (Variables|/Game/OctoInkContent/Blueprints/SaveData/MyGame.MyGame_C|GetPlayerStats _asmy_game)))))

(event Input|ActionEvents|InputActionZoomIn
  (params (Key :type Key%20Structure :default "None"))
  (:Pressed
    (if (> (Variables|Default|GetZoomScale) (Variables|Default|GetZoomMin))
      (bind _result (Math|Integer|DecrementInt (Variables|Default|GetZoomScale))
        (:%20%20
          (bind _asmy_game (Utilities|Casting|CastToMyGame (Game|GetGameInstance)))
          (Utilities|Struct|SetmembersinPlayerStats (Variables|/Game/OctoInkContent/Blueprints/SaveData/MyGame.MyGame_C|GetPlayerStats _asmy_game) (Math|Integer|Max(Integer) _result (Variables|Default|GetZoomMin)))
          (CallFunction|SetZoom -1.0)
          (Default|CallZoominandOut))))))

(event Input|ActionEvents|InputActionZoomOut
  (params (Key :type Key%20Structure :default "None"))
  (:Pressed
    (if (< (Variables|Default|GetZoomScale) (Variables|Default|GetZoomMax))
      (bind _result (Math|Integer|IncrementInt (Variables|Default|GetZoomScale))
        (:%20%20
          (bind _asmy_game (Utilities|Casting|CastToMyGame (Game|GetGameInstance)))
          (Utilities|Struct|SetmembersinPlayerStats (Variables|/Game/OctoInkContent/Blueprints/SaveData/MyGame.MyGame_C|GetPlayerStats _asmy_game) (Math|Integer|Min(Integer) _result (Variables|Default|GetZoomMax)))
          (CallFunction|SetZoom 1.0)
          (Default|CallZoominandOut))))))

(event Input|ActionEvents|InputActionMix
  (params (Key :type Key%20Structure :default "None"))
  (:Pressed
    (bind _asbp_mixer (Utilities|Casting|CastToBP_Mixer (Variables|/Game/OctoInkContent/Blueprints/Actors/Player/BP_PuzzlePlayer.BP_PuzzlePlayer_C|GetObjectInRange (Variables|Default|GetPuzzlePlayerRef))))
    (bind (_mixable _mixedcolor) (Default|IsMixable _asbp_mixer))
    (if _mixable
      (Default|Mix _asbp_mixer _mixedcolor)
      (elif (Variables|Default|GetEnableMovement)
        (Audio|PlaySound2D "/Game/OctoInkContent/Assets/SFX/sounds/MenuSounds/Error.Error" 1.0 1.0 0.0 0 0)))))

(event Input|ActionEvents|InputActionInk/Absorb
  (params (Key :type Key%20Structure :default "None"))
  (bind _puzzleplayerref (Variables|Default|GetPuzzlePlayerRef))
  (bind _puzzleplayerref_2 (Variables|Default|GetPuzzlePlayerRef))
  (bind _puzzleplayerref_3 (Variables|Default|GetPuzzlePlayerRef))
  (bind _puzzleplayerref_4 (Variables|Default|GetPuzzlePlayerRef))
  (bind _puzzleplayerref_5 (Variables|Default|GetPuzzlePlayerRef))
  (bind _objectinrange (Variables|/Game/OctoInkContent/Blueprints/Actors/Player/BP_PuzzlePlayer.BP_PuzzlePlayer_C|GetObjectInRange _puzzleplayerref_5))
  (:Pressed
    (if (not (Variables|/Game/OctoInkContent/Blueprints/Actors/Player/BP_PuzzlePlayer.BP_PuzzlePlayer_C|GetIsMentalBlocked _puzzleplayerref_4))
      (if (Variables|/Game/OctoInkContent/Blueprints/Actors/Player/BP_PuzzlePlayer.BP_PuzzlePlayer_C|GetHasColor _puzzleplayerref_4)
        ;[1 1 1] Ink
        (bind _asbp_puzzle_interactable (Utilities|Casting|CastToBP_PuzzleInteractable (Variables|/Game/OctoInkContent/Blueprints/Actors/Player/BP_PuzzlePlayer.BP_PuzzlePlayer_C|GetObjectInRange _puzzleplayerref_3)))
        (bind _inkable (Default|IsInkable _asbp_puzzle_interactable))
        (if (Math|Boolean|ANDBoolean _inkable (not (Variables|/Game/OctoInkContent/Blueprints/Actors/Player/BP_PuzzlePlayer.BP_PuzzlePlayer_C|GetIsPlayerInObstacle _puzzleplayerref_3)) (Variables|Default|GetEnableMovement))
          (Default|Ink _puzzleplayerref_2)
          (Default|MentalBlockRoll _puzzleplayerref_2)
          (elif (Variables|Default|GetEnableMovement)
            (if (not (Variables|Default|GetIsMixingGuideOpen))
              (Audio|PlaySound2D "/Game/OctoInkContent/Assets/SFX/sounds/MenuSounds/Error.Error" 1.0 1.0 0.0 0 0))))
        (else
          ;[1 1 1] Absorb
          (bind _asbp_puzzle_interactable_2 (Utilities|Casting|CastToBP_PuzzleInteractable _objectinrange))
          (bind _absrobable (Default|IsAbsorbable _asbp_puzzle_interactable_2))
          (if (Math|Boolean|ANDBoolean _absrobable (!= _objectinrange 0) (not (Variables|/Game/OctoInkContent/Blueprints/Actors/Player/BP_PuzzlePlayer.BP_PuzzlePlayer_C|GetIsPlayerInObstacle _puzzleplayerref_5)) (Utilities|Enum|Equal(Enum) "NewEnumerator6" (Variables|/Game/OctoInkContent/DataAssets/DataAssets/Color/PDA_Color.PDA_Color_C|GetColor (Variables|/Game/OctoInkContent/Blueprints/Actors/Player/BP_PuzzlePlayer.BP_PuzzlePlayer_C|GetCurrentColor _puzzleplayerref_5))) (Variables|Default|GetEnableMovement))
            (Default|Absorb _puzzleplayerref)
            (Default|MentalBlockRoll _puzzleplayerref)
            (elif (Variables|Default|GetEnableMovement)
              (if (not (Variables|Default|GetIsMixingGuideOpen))
                (Audio|PlaySound2D "/Game/OctoInkContent/Assets/SFX/sounds/MenuSounds/Error.Error" 1.0 1.0 0.0 0 0)
                (Default|CallInvalidAbsorb)))))))))

(event Input|ActionEvents|InputActionMentalBlock
  (params (Key :type Key%20Structure :default "None"))
  (bind _puzzleplayerref (Variables|Default|GetPuzzlePlayerRef))
  (bind _puzzleplayerref_2 (Variables|Default|GetPuzzlePlayerRef))
  (:Pressed
    (if (Variables|/Game/OctoInkContent/Blueprints/Actors/Player/BP_PuzzlePlayer.BP_PuzzlePlayer_C|GetIsMentalBlocked _puzzleplayerref)
      (bind _output_get (Variables|/Game/OctoInkContent/Blueprints/Actors/Player/BP_PuzzlePlayer.BP_PuzzlePlayer_C|SetPressCount _puzzleplayerref (- (Variables|/Game/OctoInkContent/Blueprints/Actors/Player/BP_PuzzlePlayer.BP_PuzzlePlayer_C|GetPressCount _puzzleplayerref) 1)))
      (if (<= _output_get 0)
        (Variables|/Game/OctoInkContent/Blueprints/Actors/Player/BP_PuzzlePlayer.BP_PuzzlePlayer_C|SetIsMentalBlocked _puzzleplayerref_2 false)
        (Components|Activation|Activate (Variables|/Script/Engine.Character|GetCharacterMovement _puzzleplayerref_2) false)))))

(event Input|ActionEvents|InputActionInteract
  (params (Key :type Key%20Structure :default "None"))
  (:Pressed
    (bind _asbp_puzzle_interactable (Utilities|Casting|CastToBP_PuzzleInteractable (Variables|/Game/OctoInkContent/Blueprints/Actors/Player/BP_PuzzlePlayer.BP_PuzzlePlayer_C|GetObjectInRange (Variables|Default|GetPuzzlePlayerRef))))
    (Default|CallInteractObject _asbp_puzzle_interactable)))

(fn ConstructionScript)

(fn SetZoom
  (params (ZoomAxis :type Float%20%28single-precision%29))
  (bind _asmy_game (Utilities|Casting|CastToMyGame (Game|GetGameInstance)))
  (bind _structout (Utilities|Struct|SetmembersinPlayerStats (Variables|/Game/OctoInkContent/Blueprints/SaveData/MyGame.MyGame_C|GetPlayerStats _asmy_game) (+ (.Zoom (Utilities|Struct|BreakPlayerStats (Variables|/Game/OctoInkContent/Blueprints/SaveData/MyGame.MyGame_C|GetPlayerStats _asmy_game))) (* (Variables|Default|GetZoomDIfference) ZoomAxis))))
  (bind _asbp_base_player (Utilities|Casting|CastToBP_BasePlayer (Game|Player|GetPlayerPawn 0)))
  (Transformation|SetRelativeLocation (Variables|/Game/OctoInkContent/Blueprints/Actors/Player/BP_BasePlayer.BP_BasePlayer_C|GetCamera _asbp_base_player) (Math|Vector|MakeVector (/ (.Zoom (Utilities|Struct|BreakPlayerStats _structout)) (Variables|Default|GetCameraSlope)) (* -1 (/ (.Zoom (Utilities|Struct|BreakPlayerStats _structout)) (Variables|Default|GetCameraSlope))) (.Zoom (Utilities|Struct|BreakPlayerStats _structout))) false false))