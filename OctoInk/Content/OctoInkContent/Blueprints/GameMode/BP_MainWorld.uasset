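; Main world game mode that runs the hub between commissions: tutorial gating, day clock, HUD swapping and the reputation-based ending.
; State lives in the MyGame instance, so StartCommission saves player location and quest before opening its level, and BeginPlay applies earned reputation and energy loss on return.
; A self-recalling delay timer skips while paused, advances time and days, and fires hourly events that fade the fog's sun multiplier between day and night.
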(event Custom|CheckIfSwitch
  (params (Hour :type Integer))
  (if (== Hour 6)
    (CallFunction|NighttoDayCycle)
    (elif (== Hour 18)
      (CallFunction|DaytoNightCycle))))

(event Custom|ShowQuest
  (params (CurrentQuest :type PDA%20Commission%20Object%20Reference))
  ;[1 0 0] Archive Code
)

(event Custom|DoCommission
  (Variables|Default|SetCanOpenQuests true)
  (Variables|Default|SetCanPlayMinigames false)
  (Variables|Default|SetTutorialState "NewEnumerator0")
  (CallFunction|SettingWidget false false "/Game/OctoInkContent/Blueprints/Widgets/BP_TutorialTasks.BP_TutorialTasks_C")
  (Default|CallShowPCIcon))

(event Custom|Stop
  ;[1 0 0] Archive Code
)

(event Custom|NightToDayCycle
  (bind _athmosphericfog (Variables|Default|GetAthmosphericFog))
  (bind _atmosphericfogcomponent (Variables|/Script/Engine.AtmosphericFog|GetAtmosphericFogComponent _athmosphericfog))
  (if (< (Variables|/Script/Engine.AtmosphericFogComponent|GetSunMultiplier _atmosphericfogcomponent) (Variables|Default|GetMaxSunMultiplier)) :!label _label
    (Class|AtmosphericFogComponent|SetSunMultiplier _atmosphericfogcomponent (+ (Variables|/Script/Engine.AtmosphericFogComponent|GetSunMultiplier _atmosphericfogcomponent) 0.1))
    (Utilities|FlowControl|Delay 0.2)
    (goto _label)))

(event Custom|DayToNightCycle
  (bind _athmosphericfog (Variables|Default|GetAthmosphericFog))
  (bind _atmosphericfogcomponent (Variables|/Script/Engine.AtmosphericFog|GetAtmosphericFogComponent _athmosphericfog))
  (if (> (Variables|/Script/Engine.AtmosphericFogComponent|GetSunMultiplier _atmosphericfogcomponent) (Variables|Default|GetMinSunMultiplier)) :!label _label
    (Class|AtmosphericFogComponent|SetSunMultiplier _atmosphericfogcomponent (- (Variables|/Script/Engine.AtmosphericFogComponent|GetSunMultiplier _atmosphericfogcomponent) 0.1))
    (Utilities|FlowControl|Delay 0.2)
    (goto _label)))

(event Custom|SetDaySystem
  (bind _athmosphericfog (Variables|Default|GetAthmosphericFog))
  (bind _atmosphericfogcomponent (Variables|/Script/Engine.AtmosphericFog|GetAtmosphericFogComponent _athmosphericfog))
  (bind _hours (CallFunction|SetHours))
  (if (and (>= _hours 7) (<= _hours 17))
    (Class|AtmosphericFogComponent|SetSunMultiplier _atmosphericfogcomponent (Variables|Default|GetMaxSunMultiplier))
    (else
      (Class|AtmosphericFogComponent|SetSunMultiplier _atmosphericfogcomponent (Variables|Default|GetMinSunMultiplier)))))

(event Custom|EnableMovement
  (bind _gameinstanceref (Variables|ObjectReferences|GetGameInstanceRef))
  (bind _asbp_player_base_controller (Utilities|Casting|CastToBP_PlayerBaseController (Game|GetPlayerController 0)))
  (Variables|/Game/OctoInkContent/Blueprints/Controllers/BP_PlayerBaseController.BP_PlayerBaseController_C|SetEnableMovement _asbp_player_base_controller true)
  (if (Utilities|Struct|BreakGameModeData (Variables|/Game/OctoInkContent/Blueprints/SaveData/MyGame.MyGame_C|GetGameModeData (Variables|ObjectReferences|GetGameInstanceRef)))
    (if (>= (Utilities|Struct|BreakPlayerStats (Variables|/Game/OctoInkContent/Blueprints/SaveData/MyGame.MyGame_C|GetPlayerStats _gameinstanceref)) (Utilities|Struct|BreakGameModeData (Variables|/Game/OctoInkContent/Blueprints/SaveData/MyGame.MyGame_C|GetGameModeData _gameinstanceref)))
      (CallFunction|SettingWidget false true "/Game/OctoInkContent/Blueprints/Widgets/BP_TimeIsUpDialogue.BP_TimeIsUpDialogue_C")
      (Variables|Default|SetIsGameDone true))
    (elif (not (== (Utilities|GetClass (Variables|ObjectReferences|GetCurrentUserWidgetRef)) "/Game/OctoInkContent/Blueprints/Widgets/MainWorld/BP_DialogueHUD.BP_DialogueHUD_C"))
      (CallFunction|SettingWidget false true "/Game/OctoInkContent/Blueprints/Widgets/MainWorld/BP_DialogueHUD.BP_DialogueHUD_C")
      (bind _asbp_dialogue_hud (Utilities|Casting|CastToBP_DialogueHUD (Variables|ObjectReferences|GetCurrentUserWidgetRef)))
      (Default|SetDialogue _asbp_dialogue_hud "NewEnumerator14"))))

(event Custom|ShowDialogue
  (params (Dialogue :type PDA%20Dialogue%20Object%20Reference))
  ;[1 0 0] Archive Code
)

(event Custom|StartCommission
  (params (Current%20Commission :type PDA%20Commission%20Object%20Reference))
  (Utilities|FlowControl|Sequence
    (:then_0
      ;[1 1 1] Set Data for Quest
      (Utilities|Struct|SetmembersinCommissionData (Variables|/Game/OctoInkContent/Blueprints/SaveData/MyGame.MyGame_C|GetCommissionData (Variables|ObjectReferences|GetGameInstanceRef)) (Transformation|GetWorldTransform (Variables|/Script/Engine.Actor|GetRootComponent (Game|Player|GetPlayerPawn 0))) Current%20Commission))
    (:then_1
      ;[1 1 1] Open Commision
      (Game|OpenLevel(byName) (Variables|/Game/OctoInkContent/DataAssets/DataAssets/Commissions/PDA_Commission.PDA_Commission_C|GetLevelName Current%20Commission)))))

(event Custom|StartDayTimer
  (bind _gameinstanceref (Variables|ObjectReferences|GetGameInstanceRef))
  (bind _gameinstanceref_2 (Variables|ObjectReferences|GetGameInstanceRef))
  (bind _gameinstanceref_3 (Variables|ObjectReferences|GetGameInstanceRef))
  (bind _gameinstanceref_4 (Variables|ObjectReferences|GetGameInstanceRef))
  (bind _gamemodedata (Variables|/Game/OctoInkContent/Blueprints/SaveData/MyGame.MyGame_C|GetGameModeData _gameinstanceref_3))
  (bind _gamemodedata_2 (Variables|/Game/OctoInkContent/Blueprints/SaveData/MyGame.MyGame_C|GetGameModeData _gameinstanceref_2))
  (bind _gamemodedata_3 (Variables|/Game/OctoInkContent/Blueprints/SaveData/MyGame.MyGame_C|GetGameModeData _gameinstanceref))
  (bind _gamemodedata_4 (Variables|/Game/OctoInkContent/Blueprints/SaveData/MyGame.MyGame_C|GetGameModeData _gameinstanceref_4))
  (bind (_day _maxday) (Utilities|Struct|BreakGameModeData _gamemodedata))
  (bind (_time _maxtime) (Utilities|Struct|BreakGameModeData _gamemodedata_2))
  (bind _asbp_player_base_controller (Utilities|Casting|CastToBP_PlayerBaseController (Game|GetPlayerController 0)))
  (if (Variables|/Game/OctoInkContent/Blueprints/Controllers/BP_PlayerBaseController.BP_PlayerBaseController_C|GetisPauseMenuOpen _asbp_player_base_controller)
    ;[1 1 1] Skips adding Time/Day if game is paused
    (Utilities|FlowControl|Delay 0.1)
    (CallFunction|StartDayTimer)
    (elif (>= _time _maxtime)
      ;[1 1 1] Adds a Day, and resets current time to 0 if Max Amt of Time is Reached
      (bind _result (Math|Integer|IncrementInt (Utilities|Struct|BreakGameModeData _gamemodedata_3))
        (:%20%20
          (Utilities|Struct|SetmembersinGameModeData _gamemodedata_3 _result)
          (Utilities|Struct|SetmembersinGameModeData (Variables|/Game/OctoInkContent/Blueprints/SaveData/MyGame.MyGame_C|GetGameModeData (Variables|ObjectReferences|GetGameInstanceRef)))
          (if (>= _day _maxday)
            ;[1 1 1] Play Ending if MaxDays (6 Days) is reached
            (CallFunction|SettingWidget false true "/Game/OctoInkContent/Blueprints/Widgets/BP_TimeIsUpDialogue.BP_TimeIsUpDialogue_C")
            (Variables|Default|SetIsGameDone true)
            (else
              ;[1 1 1] Calls Event again after (0.1 miliseconds) 1 seconds =  10 deciseconds
              (Utilities|FlowControl|Delay 0.1 :!label _label)
              (CallFunction|StartDayTimer)))))
      (else
        ;[1 1 1] Adds time
        (bind _result_2 (Math|Integer|IncrementInt (Utilities|Struct|BreakGameModeData _gamemodedata_4))
          (:%20%20
            (Utilities|Struct|SetmembersinGameModeData _gamemodedata_4 _result_2)
            (bind _timeinstring (CallFunction|TrackTime _result_2))
            (Utilities|Struct|SetmembersinGameModeData _gamemodedata_4 _timeinstring)
            (goto _label)))))))

(event Custom|Ending
  (bind _gameinstanceref (Variables|ObjectReferences|GetGameInstanceRef))
  (if (>= (Utilities|Struct|BreakPlayerStats (Variables|/Game/OctoInkContent/Blueprints/SaveData/MyGame.MyGame_C|GetPlayerStats _gameinstanceref)) (.RequiredReputation (Utilities|Struct|BreakGameModeData (Variables|/Game/OctoInkContent/Blueprints/SaveData/MyGame.MyGame_C|GetGameModeData _gameinstanceref))))
    (CallFunction|SettingWidget false true "/Game/OctoInkContent/Blueprints/Widgets/Cutscenes/BP_GoodEndingCutscene.BP_GoodEndingCutscene_C")
    (else
      (CallFunction|SettingWidget false true "/Game/OctoInkContent/Blueprints/Widgets/Cutscenes/BP_BadEndingCutscene.BP_BadEndingCutscene_C"))))

(event Custom|TimerCanIncrement
  ;[1 1 1] Adds time
  (Utilities|FlowControl|Delay 1.0)
  (Variables|TimeSystem|SetboolCanIncrement true))

(event Custom|LoseEnergy
  (bind _gameinstanceref (Variables|ObjectReferences|GetGameInstanceRef))
  (bind _gameinstanceref_2 (Variables|ObjectReferences|GetGameInstanceRef))
  (bind _gameinstanceref_3 (Variables|ObjectReferences|GetGameInstanceRef))
  (bind _gameinstanceref_4 (Variables|ObjectReferences|GetGameInstanceRef))
  (bind _commissiondata (Variables|/Game/OctoInkContent/Blueprints/SaveData/MyGame.MyGame_C|GetCommissionData _gameinstanceref))
  (bind _playerstats (Variables|/Game/OctoInkContent/Blueprints/SaveData/MyGame.MyGame_C|GetPlayerStats _gameinstanceref_2))
  (bind _playerstats_2 (Variables|/Game/OctoInkContent/Blueprints/SaveData/MyGame.MyGame_C|GetPlayerStats _gameinstanceref_4))
  (bind _commissiondata_2 (Variables|/Game/OctoInkContent/Blueprints/SaveData/MyGame.MyGame_C|GetCommissionData _gameinstanceref_3))
  (bind _totalenergyloss (Utilities|Struct|BreakCommissionData _commissiondata_2))
  (bind _totalreputationearned (Utilities|Struct|BreakCommissionData _commissiondata))
  (Utilities|FlowControl|Sequence
    (:then_0
      ;[1 1 1] Disable Movement
      (bind _asbp_player_base_controller (Utilities|Casting|CastToBP_PlayerBaseController (Game|GetPlayerController 0)))
      (Variables|/Game/OctoInkContent/Blueprints/Controllers/BP_PlayerBaseController.BP_PlayerBaseController_C|SetEnableMovement _asbp_player_base_controller false))
    (:then_1
      ;[1 1 1] Show Reputation
      (Utilities|FlowControl|Delay (Variables|Pop-up|GetDuration))
      (bind _returnvalue (Game|SpawnActorfromClass "/Game/OctoInkContent/Blueprints/Actors/MainWorld/BP_Notif.BP_Notif_C" (Math|Conversions|ToTransform(Vector) (Transformation|GetWorldLocation (Variables|/Game/OctoInkContent/Blueprints/Actors/Player/BP_MainGamePlayer.BP_MainGamePlayer_C|GetNotifSpawn (Variables|ObjectReferences|GetMainGamePlayerRef)))) "Undefined" 0 0))
      (Default|SetText _returnvalue (Utilities|Text|FormatText "{+}{Value}{%}" (Utilities|Text|ToText(String) "+") _totalreputationearned (Utilities|Text|ToText(String) " Reputation")))
      (Utilities|Struct|SetmembersinPlayerStats _playerstats (+ (Utilities|Struct|BreakPlayerStats _playerstats) _totalreputationearned))
      (Utilities|Struct|SetmembersinCommissionData (Variables|/Game/OctoInkContent/Blueprints/SaveData/MyGame.MyGame_C|GetCommissionData (Variables|ObjectReferences|GetGameInstanceRef)))
      ;[1 1 1] Show Player Energy
      (Utilities|FlowControl|Delay (Variables|Pop-up|GetDuration))
      (bind _returnvalue_2 (Game|SpawnActorfromClass "/Game/OctoInkContent/Blueprints/Actors/MainWorld/BP_Notif.BP_Notif_C" (Math|Conversions|ToTransform(Vector) (Transformation|GetWorldLocation (Variables|/Game/OctoInkContent/Blueprints/Actors/Player/BP_MainGamePlayer.BP_MainGamePlayer_C|GetNotifSpawn (Variables|ObjectReferences|GetMainGamePlayerRef)))) "Undefined" 0 0))
      (Default|SetText _returnvalue_2 (Utilities|Text|FormatText "-{Value}{%}" (Utilities|Text|ToText(Integer) _totalenergyloss) (Utilities|Text|ToText(String) " Energy")))
      (Utilities|Struct|SetmembersinPlayerStats _playerstats_2 (Math|Integer|Clamp(Integer) (- (Utilities|Struct|BreakPlayerStats _playerstats_2) _totalenergyloss) 0 100))
      (Default|SetPlayerSpeed (Variables|ObjectReferences|GetMainGamePlayerRef))
      (Utilities|Struct|SetmembersinCommissionData (Variables|/Game/OctoInkContent/Blueprints/SaveData/MyGame.MyGame_C|GetCommissionData (Variables|ObjectReferences|GetGameInstanceRef)))
      (if (>= (Utilities|Struct|BreakPlayerStats (Variables|/Game/OctoInkContent/Blueprints/SaveData/MyGame.MyGame_C|GetPlayerStats (Variables|ObjectReferences|GetGameInstanceRef))) 50)
        (CallFunction|EnableMovement)
        (else
          (bind _asbp_main_game_player (Utilities|Casting|CastToBP_MainGamePlayer (Game|Player|GetPlayerPawn 0)))
          (bind _asbp_player_animator (Utilities|Casting|CastToBP_PlayerAnimator (Variables|/Script/PaperZD.PaperZDCharacter|GetAnimInstance _asbp_main_game_player)))
          (EventDispatchers|BindEventtoTransitionDone _asbp_player_animator (delegate Custom|EnableMovement)))))))

(event Custom|DoPuzzle
  (Variables|Default|SetCanOpenQuests false)
  (Variables|Default|SetCanPlayMinigames true)
  (Variables|Default|SetTutorialState "NewEnumerator2")
  (CallFunction|SettingWidget false false "/Game/OctoInkContent/Blueprints/Widgets/BP_TutorialTasks.BP_TutorialTasks_C")
  (Default|CallShowMinigamesIcon))

(event Custom|BackToMainWorld
  (if (Utilities|Struct|BreakGameModeData (Variables|/Game/OctoInkContent/Blueprints/SaveData/MyGame.MyGame_C|GetGameModeData (Variables|ObjectReferences|GetGameInstanceRef)))
    (CallFunction|SettingWidget false false "/Game/OctoInkContent/Blueprints/Widgets/MainWorld/BP_TempMainWorldHUD.BP_TempMainWorldHUD_C")
    (else
      (CallFunction|SettingWidget false false "/Game/OctoInkContent/Blueprints/Widgets/BP_TutorialTasks.BP_TutorialTasks_C"))))

(event EventBeginPlay
  (Utilities|FlowControl|Sequence
    (:then_0
      ;[1 1 1] Setting Up References
      (bind _asmy_game (Utilities|Casting|CastToMyGame (Game|GetGameInstance)))
      (Variables|ObjectReferences|SetGameInstanceRef _asmy_game)
      (bind _asbp_main_game_player (Utilities|Casting|CastToBP_MainGamePlayer (Game|Player|GetPlayerPawn 0)))
      (Variables|ObjectReferences|SetMainGamePlayerRef _asbp_main_game_player))
    (:then_1
      (if (Utilities|Struct|BreakGameModeData (Variables|/Game/OctoInkContent/Blueprints/SaveData/MyGame.MyGame_C|GetGameModeData (Variables|ObjectReferences|GetGameInstanceRef)))
        ;[1 0.5885 0] Non-Tutorial Gameplay
        (Utilities|FlowControl|Sequence
          (:then_0
            ;;[0 0.02745 1] Showing Main World Widget + Allowing Quests & Minigames
            (CallFunction|SettingWidget false false "/Game/OctoInkContent/Blueprints/Widgets/MainWorld/BP_TempMainWorldHUD.BP_TempMainWorldHUD_C")
            (Variables|Default|SetCanOpenQuests true)
            (Variables|Default|SetCanPlayMinigames true))
          (:then_1
            ;;[0 0.02745 1] Set Player Location (Based on where they last were)
            (bind _asbp_main_game_player_2 (Utilities|Casting|CastToBP_MainGamePlayer (Game|Player|GetPlayerPawn 0)))
            (Transformation|SetWorldTransform (Variables|/Script/Engine.Character|GetCapsuleComponent _asbp_main_game_player_2) (Utilities|Struct|BreakCommissionData (Variables|/Game/OctoInkContent/Blueprints/SaveData/MyGame.MyGame_C|GetCommissionData (Variables|ObjectReferences|GetGameInstanceRef))) false false))
          (:then_2
            ;;[0 0.02745 1] Losing Energy, and Gaining Reputation
            (if (!= (Utilities|Struct|BreakCommissionData (Variables|/Game/OctoInkContent/Blueprints/SaveData/MyGame.MyGame_C|GetCommissionData (Variables|ObjectReferences|GetGameInstanceRef))) 0)
              (CallFunction|LoseEnergy)
              (Utilities|Struct|SetmembersinCommissionData (Variables|/Game/OctoInkContent/Blueprints/SaveData/MyGame.MyGame_C|GetCommissionData (Variables|ObjectReferences|GetGameInstanceRef)))))
          (:then_3
            ;;[0 0.02745 1] Losing Energy, and Gaining Reputation
            (if (>= (.Day (Utilities|Struct|BreakGameModeData (Variables|/Game/OctoInkContent/Blueprints/SaveData/MyGame.MyGame_C|GetGameModeData (Variables|ObjectReferences|GetGameInstanceRef)))) (.MaxDay (Utilities|Struct|BreakGameModeData (Variables|/Game/OctoInkContent/Blueprints/SaveData/MyGame.MyGame_C|GetGameModeData (Variables|ObjectReferences|GetGameInstanceRef)))))
              (CallFunction|SettingWidget false true "/Game/OctoInkContent/Blueprints/Widgets/BP_TimeIsUpDialogue.BP_TimeIsUpDialogue_C")
              (Variables|Default|SetIsGameDone true)
              (else
                (CallFunction|StartDayTimer))))
          (:then_4
            (EventDispatchers|BindEventtoNextHour (delegate Custom|CheckIfSwitch))
            (Default|CallShowPCIcon)
            (Default|CallShowMinigamesIcon)))
        (else
          ;[0.7088 0 1] Tutorial Gameplay
          (if (!= (Utilities|Struct|BreakCommissionData (Variables|/Game/OctoInkContent/Blueprints/SaveData/MyGame.MyGame_C|GetCommissionData (Variables|ObjectReferences|GetGameInstanceRef))) 0)
            ;;[1 0.949 0] After Player Plays the Commission
            (CallFunction|LoseEnergy)
            (Utilities|Struct|SetmembersinCommissionData (Variables|/Game/OctoInkContent/Blueprints/SaveData/MyGame.MyGame_C|GetCommissionData (Variables|ObjectReferences|GetGameInstanceRef)))
            (else
              ;;[1 0.949 0] When Player has not played the commission (Start the Game)
              (CallFunction|SettingWidget false true "/Game/OctoInkContent/Blueprints/Widgets/MainWorld/BP_DialogueHUD.BP_DialogueHUD_C")
              (Variables|Default|SetCanOpenQuests false)
              (Variables|Default|SetCanPlayMinigames false)
              (bind _asbp_dialogue_hud (Utilities|Casting|CastToBP_DialogueHUD (Variables|ObjectReferences|GetCurrentUserWidgetRef)))
              (Default|SetDialogue _asbp_dialogue_hud "NewEnumerator6"))))))))

(fn ConstructionScript)

(fn SettingWidget
  (params (ShowMouseCursor :type Boolean) (DisableMovement :type Boolean) (WidgetClass :type User%20Widget%20Class%20Reference))
  (bind _returnvalue (Game|GetPlayerController 0))
  (Utilities|FlowControl|Sequence
    (:then_0
      ;[1 1 1] Setting Movement
      (bind _asbp_player_base_controller (Utilities|Casting|CastToBP_PlayerBaseController _returnvalue))
      (Variables|/Game/OctoInkContent/Blueprints/Controllers/BP_PlayerBaseController.BP_PlayerBaseController_C|SetEnableMovement _asbp_player_base_controller (not DisableMovement)))
    (:then_1
      ;[1 1 1] Setting Mouse Cursor Visibility
      (Variables|/Script/Engine.PlayerController|SetbShowMouseCursor _returnvalue ShowMouseCursor))
    (:then_2
      (Viewport|RemoveAllWidgets))
    (:then_3
      ;[1 1 1] Adding New Widget
      (if (Utilities|IsValidClass WidgetClass)
        (bind _returnvalue_2 (UserInterface|CreateWidget WidgetClass))
        (Variables|ObjectReferences|SetCurrentUserWidgetRef _returnvalue_2)
        (UserInterface|Viewport|AddtoViewport _returnvalue_2 0)))))

(fn CheckGameConditions
  (params (PlayerStats :type Player%20Stats%20Structure)))

(fn TrackTime
  (params (Deciseconds :type Integer))
  (CallFunction|SetHours)
  (if (and (Variables|TimeSystem|GetboolCanIncrement) (== (Math|Float|%(Float) (Math|Conversions|ToFloat(Integer) Deciseconds) (/ (Math|Conversions|ToFloat(Integer) (Utilities|Struct|BreakGameModeData (Variables|/Game/OctoInkContent/Blueprints/SaveData/MyGame.MyGame_C|GetGameModeData (Variables|ObjectReferences|GetGameInstanceRef)))) 24.0)) 0.0))
    (Variables|TimeSystem|SetboolCanIncrement false)
    (CallFunction|TimerCanIncrement)
    (Default|CallNextHour (Variables|TimeSystem|GetHours)))
  ;[1 1 1] Identifies if AM/PM
  (if (> (Variables|TimeSystem|GetHours) 11)
    (Variables|TimeSystem|SetAM/PM%20String "PM")
    (else
      (Variables|TimeSystem|SetAM/PM%20String "AM")))
  (if (== (Variables|TimeSystem|GetHours) 0)
    (Variables|TimeSystem|SetDisplayedHours 12 :!label _label)
    (return (Utilities|String|ToString(Text) (Utilities|Text|FormatText "{Hours} {AM/PM} " (Variables|TimeSystem|GetDisplayedHours) (Variables|TimeSystem|GetAM/PM%20String))))
    (elif (< (Variables|TimeSystem|GetHours) 12)
      (Variables|TimeSystem|SetDisplayedHours (Variables|TimeSystem|GetHours))
      (return (Utilities|String|ToString(Text) (Utilities|Text|FormatText "{Hours} {AM/PM} " (Variables|TimeSystem|GetDisplayedHours) (Variables|TimeSystem|GetAM/PM%20String))))
      (elif (> (Variables|TimeSystem|GetHours) 12)
        (Variables|TimeSystem|SetDisplayedHours (- (Variables|TimeSystem|GetHours) 12))
        (return (Utilities|String|ToString(Text) (Utilities|Text|FormatText "{Hours} {AM/PM} " (Variables|TimeSystem|GetDisplayedHours) (Variables|TimeSystem|GetAM/PM%20String))))
        (elif (== (Variables|TimeSystem|GetHours) 12)
          (goto _label))))))

(fn SetHours
  (bind _asmy_game (Utilities|Casting|CastToMyGame (Game|GetGameInstance)))
  (bind _output_get (Variables|TimeSystem|SetHours (/ (.Time (Utilities|Struct|BreakGameModeData (Variables|/Game/OctoInkContent/Blueprints/SaveData/MyGame.MyGame_C|GetGameModeData _asmy_game))) (/ (.MaxTime (Utilities|Struct|BreakGameModeData (Variables|/Game/OctoInkContent/Blueprints/SaveData/MyGame.MyGame_C|GetGameModeData _asmy_game))) 24))))
  (return _output_get))