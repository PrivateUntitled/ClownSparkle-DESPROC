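; World 2 game mode that runs a color-mixing tutorial through The Elder's dialogue and on-screen tasks, and overrides day/night lighting colors.
; Dialogue data supplies line-by-line messages, task text and a lesson type, which Checker uses to start the next task.
; Tasks bind to player controller ink and mix events, check mixer and obstacle colors, then trigger further dialogue.
; The final test unlocks inking on the second obstacle.
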(event Custom|MixingGuideOpened
  (EventDispatchers|BindEventtoHasExitedMixingGuide (stale Custom|OpenMixingGuideTask _asbp_player_base_controller) (delegate Custom|MixingGuideClosed)))

(event Custom|CustomEvent_3
  (bind _mixerref (Variables|Default|GetMixerRef))
  (bind _mixercontents (Variables|/Game/OctoInkContent/Blueprints/Actors/Obstacles/Mixer/BP_Mixer.BP_Mixer_C|GetMixerContents _mixerref))
  (bind _output (Utilities|Array|Get(acopy) _mixercontents 1))
  (bind _output_2 (Utilities|Array|Get(acopy) _mixercontents))
  (bind _color (Variables|/Game/OctoInkContent/DataAssets/DataAssets/Color/PDA_Color.PDA_Color_C|GetColor _output_2))
  (bind _color_2 (Variables|/Game/OctoInkContent/DataAssets/DataAssets/Color/PDA_Color.PDA_Color_C|GetColor _output_2))
  (bind _returnvalue (Utilities|Enum|Equal(Enum) _color "NewEnumerator0"))
  (bind _returnvalue_2 (Utilities|Enum|Equal(Enum) _color_2 "NewEnumerator4"))
  (if (== (Utilities|Array|Length _mixercontents) 2)
    (if (or (and _returnvalue (Utilities|Enum|Equal(Enum) (Variables|/Game/OctoInkContent/DataAssets/DataAssets/Color/PDA_Color.PDA_Color_C|GetColor _output) "NewEnumerator4")) (and (Utilities|Enum|Equal(Enum) (Variables|/Game/OctoInkContent/DataAssets/DataAssets/Color/PDA_Color.PDA_Color_C|GetColor _output) "NewEnumerator0") _returnvalue_2))
      (Default|PrintStringText (stale Custom|GetPurple _asbp_tutorial_tasks) (.Description (Utilities|Struct|BreakLesson2Struct (Variables|Default|GetMixColor))))
      (Variables|Default|SetHasCorrectColors true)
      (else
        (Variables|Default|SetHasCorrectColors false)))
    (else
      (Variables|Default|SetHasCorrectColors false)
      (if _returnvalue
        (Default|PrintStringText (stale Custom|GetPurple _asbp_tutorial_tasks) (.Description (Utilities|Struct|BreakLesson2Struct (Variables|Default|GetGetBlueColor))))
        (elif _returnvalue_2
          (Default|PrintStringText (stale Custom|GetPurple _asbp_tutorial_tasks) (.Description (Utilities|Struct|BreakLesson2Struct (Variables|Default|GetGetRedColor)))))))))

(event Custom|Checker
  (params (Lesson2 :type Lesson2Stage%20Enum :default "NewEnumerator0"))
  (switch Utilities|FlowControl|Switch|SwitchonLesson2Stage Lesson2
    (:NewEnumerator1
      (CallFunction|GetPurple))
    (:NewEnumerator5
      (CallFunction|PlaceMannequin1Task))
    (:NewEnumerator4
      (CallFunction|FinalTestTask))))

(event Custom|PlaceMannequin1Task
  (bind _asbp_player_puzzle_controller (Utilities|Casting|CastToBP_PlayerPuzzleController (Game|GetPlayerController 0)))
  (EventDispatchers|BindEventtoInk _asbp_player_puzzle_controller (delegate Custom|CustomEvent_5)))

(event Custom|CustomEvent_5
  (bind _obstacles (Variables|Default|GetObstacles))
  (bind _output (Utilities|Array|Get(acopy) _obstacles))
  (if (== (Variables|/Game/OctoInkContent/Blueprints/Actors/Obstacles/BP_Obstacle.BP_Obstacle_C|GetCurrentColor _output) (Variables|/Game/OctoInkContent/Blueprints/Actors/Obstacles/BP_Obstacle.BP_Obstacle_C|GetColorRequired _output))
    (CallFunction|PlayDialogueText (Variables|Default|GetFinalTest))
    (EventDispatchers|UnbindallEventsfromInk (stale Custom|PlaceMannequin1Task _asbp_player_puzzle_controller))))

(event Custom|FinalTestTask
  (bind _obstacles (Variables|Default|GetObstacles))
  (bind _output (Utilities|Array|Get(acopy) _obstacles 1))
  (Variables|/Game/OctoInkContent/Blueprints/Actors/Obstacles/BP_Obstacle.BP_Obstacle_C|SetCanInk _output true)
  (bind _asbp_obstacle_pointer (Utilities|Casting|CastToBP_ObstaclePointer (UserInterface|GetWidget (Variables|/Game/OctoInkContent/Blueprints/Actors/Obstacles/BP_Obstacle.BP_Obstacle_C|GetWidget _output))))
  (Default|HideLock _asbp_obstacle_pointer false))

(event Custom|CustomEvent_4
  (if (Variables|Default|GetHasCorrectColors)
    (bind _asbp_player_puzzle_controller (Utilities|Casting|CastToBP_PlayerPuzzleController (Game|GetPlayerController 0)))
    (EventDispatchers|UnbindallEventsfromInk _asbp_player_puzzle_controller)
    (EventDispatchers|UnbindallEventsfromMixColor _asbp_player_puzzle_controller)
    (CallFunction|PlayDialogueText (Variables|Default|GetPlaceColor))
    (Variables|Default|SetHasCorrectColors false)))

(event Custom|MixingGuideClosed
  (EventDispatchers|UnbindallEventsfromHasOpenedDebugMenu (stale Custom|OpenMixingGuideTask _asbp_player_base_controller))
  (EventDispatchers|UnbindallEventsfromHasExitedMixingGuide (stale Custom|OpenMixingGuideTask _asbp_player_base_controller))
  (if (Utilities|Enum|Equal(Enum) (Variables|Default|GetCurrent) "NewEnumerator0")
    (CallFunction|PlayDialogueText (Variables|Default|GetGetRedColor))))

(event Custom|GetPurple
  (CallFunction|SettingWidget false false "/Game/OctoInkContent/Blueprints/Widgets/BP_TutorialTasks.BP_TutorialTasks_C")
  (bind _asbp_tutorial_tasks (Utilities|Casting|CastToBP_TutorialTasks (Variables|Default|GetCurrentUserWidgetRef)))
  (Default|PrintStringText _asbp_tutorial_tasks (.Description (Utilities|Struct|BreakLesson2Struct (Variables|Default|GetGetRedColor))))
  (bind _asbp_player_puzzle_controller (Utilities|Casting|CastToBP_PlayerPuzzleController (Game|GetPlayerController 0)))
  (EventDispatchers|BindEventtoInk _asbp_player_puzzle_controller (delegate Custom|CustomEvent_3)))

(event Custom|OpenMixingGuideTask
  (Utilities|Struct|SetmembersinMenuData (Variables|/Game/OctoInkContent/Blueprints/SaveData/MyGame.MyGame_C|GetGameStateData (Variables|Default|GetGameInstanceRef)) true)
  (CallFunction|SettingWidget false true "/Game/OctoInkContent/Blueprints/Widgets/BP_TutorialTasks.BP_TutorialTasks_C")
  (bind _asbp_tutorial_tasks (Utilities|Casting|CastToBP_TutorialTasks (Variables|Default|GetCurrentUserWidgetRef)))
  (Default|PrintStringText _asbp_tutorial_tasks (.Description (Utilities|Struct|BreakLesson2Struct (Variables|Default|GetOpenMixingGuide))))
  (bind _asbp_player_base_controller (Utilities|Casting|CastToBP_PlayerBaseController (Game|GetPlayerController 0)))
  (EventDispatchers|BindEventtoHasOpenedMixingGuide _asbp_player_base_controller (delegate Custom|MixingGuideOpened)))

(event Custom|ProceedNextDialogue
  (bind _result (Math|Integer|IncrementInt (Variables|Default|GetCurrentDialogueIndex))
    (:%20%20
      (EventDispatchers|UnbindallEventsfromProceedNextDialogue (stale Custom|TextIsFinished _asbp_player_puzzle_controller))
      (if (< _result (Utilities|Array|Length (.Messages (Utilities|Struct|BreakLesson2Struct (stale Custom|PlayDialogueText Dialogue)))))
        (Audio|PlaySound2D (.OutItem (Utilities|Array|Random (Variables|Default|GetElderSounds))) 1.0 1.0 0.0 0 0)
        (Default|SetSpeakerInfo (stale Custom|PlayDialogueText _asbp_dialogue_hud) "The Elder" "NewEnumerator1")
        (Default|PrintDialogueText (stale Custom|PlayDialogueText _asbp_dialogue_hud) (Utilities|Array|Get(acopy) (.Messages (Utilities|Struct|BreakLesson2Struct (stale Custom|PlayDialogueText Dialogue))) (stale Custom|PlayDialogueText _output_get)))
        (EventDispatchers|BindEventtoTextIsFinished (stale Custom|PlayDialogueText _asbp_dialogue_hud) (delegate Custom|TextIsFinished))
        (else
          (EventDispatchers|UnbindallEventsfromTextIsFinished (stale Custom|PlayDialogueText _asbp_dialogue_hud))
          (CallFunction|SettingWidget false false "/Game/OctoInkContent/Blueprints/Widgets/BP_TutorialTasks.BP_TutorialTasks_C")
          (bind _asbp_tutorial_tasks (Utilities|Casting|CastToBP_TutorialTasks (Variables|Default|GetCurrentUserWidgetRef)))
          (Default|PrintStringText _asbp_tutorial_tasks (.Description (Utilities|Struct|BreakLesson2Struct (stale Custom|PlayDialogueText Dialogue))))
          (CallFunction|Checker (.Lesson2Type (Utilities|Struct|BreakLesson2Struct (stale Custom|PlayDialogueText Dialogue))))
          (bind _asbp_player_puzzle_controller (Utilities|Casting|CastToBP_PlayerPuzzleController (Game|GetPlayerController 0)))
          (Variables|/Game/OctoInkContent/Blueprints/Controllers/BP_PlayerBaseController.BP_PlayerBaseController_C|SetInDialogue _asbp_player_puzzle_controller false)
          (Variables|Default|SetCurrent (.Lesson2Type (Utilities|Struct|BreakLesson2Struct (stale Custom|PlayDialogueText Dialogue)))))))))

(event Custom|PlayDialogueText
  (params (Dialogue :type Lesson%202%20Struct%20Structure))
  (bind _asbp_player_puzzle_controller (Utilities|Casting|CastToBP_PlayerPuzzleController (Game|GetPlayerController 0)))
  (Variables|/Game/OctoInkContent/Blueprints/Controllers/BP_PlayerBaseController.BP_PlayerBaseController_C|SetInDialogue _asbp_player_puzzle_controller true)
  (bind _output_get (Variables|Default|SetCurrentDialogueIndex 0))
  (CallFunction|SettingWidget false true "/Game/OctoInkContent/Blueprints/Widgets/MainWorld/BP_DialogueHUD.BP_DialogueHUD_C")
  (bind _asbp_dialogue_hud (Utilities|Casting|CastToBP_DialogueHUD (Variables|Default|GetCurrentUserWidgetRef)))
  (Audio|PlaySound2D (.OutItem (Utilities|Array|Random (Variables|Default|GetElderSounds))) 1.0 1.0 0.0 0 0)
  (Default|SetSpeakerInfo _asbp_dialogue_hud "The Elder" "NewEnumerator1")
  (Default|PrintDialogueText _asbp_dialogue_hud (Utilities|Array|Get(acopy) (.Messages (Utilities|Struct|BreakLesson2Struct Dialogue)) _output_get))
  (EventDispatchers|BindEventtoTextIsFinished _asbp_dialogue_hud (delegate Custom|TextIsFinished)))

(event Custom|TextIsFinished
  (bind _asbp_player_puzzle_controller (Utilities|Casting|CastToBP_PlayerPuzzleController (Game|GetPlayerController 0)))
  (EventDispatchers|BindEventtoProceedNextDialogue _asbp_player_puzzle_controller (delegate Custom|ProceedNextDialogue)))

(event EventBeginPlay
  (|CallParentFunction)
  (bind _asbp_player_puzzle_controller (Utilities|Casting|CastToBP_PlayerPuzzleController (Game|GetPlayerController 0)))
  (EventDispatchers|BindEventtoMixColor _asbp_player_puzzle_controller (delegate Custom|CustomEvent_4)))

(event EventTick
  (params (DeltaSeconds :type Float%20%28single-precision%29))
  (|CallParentFunction DeltaSeconds) ; This node is disabled and will not be called.\nDrag off pins to build functionality.
)

(event EventIBWin
  (|CallParentFunction))

(fn ConstructionScript
  (|CallParentFunction))

(fn SetDayLighting
  (bind _skylightref (Variables|Default|GetSkyLightRef))
  (bind _lightcomponent (Variables|/Script/Engine.SkyLight|GetLightComponent _skylightref))
  (|CallParentFunction)
  (Rendering|Components|Light|SetLightColor (Variables|/Script/Engine.Light|GetLightComponent (Variables|Default|GetDirectionalLight)) (Variables|Default|GetDayDirectionalLightColor) false)
  (Rendering|Components|Light|SetLightColor _lightcomponent (Variables|Default|GetDaySkyLightColor))
  (Class|SkyLightComponent|RecaptureSky _lightcomponent))

(fn SetNightLighting
  (bind _skylightref (Variables|Default|GetSkyLightRef))
  (bind _lightcomponent (Variables|/Script/Engine.SkyLight|GetLightComponent _skylightref))
  (|CallParentFunction)
  (Rendering|Components|Light|SetLightColor (Variables|/Script/Engine.Light|GetLightComponent (Variables|Default|GetDirectionalLight)) (Variables|Default|GetNightDirectionalLightColor) false)
  (Rendering|Components|Light|SetLightColor _lightcomponent (Variables|Default|GetNightSkyLightColor))
  (Class|SkyLightComponent|RecaptureSky _lightcomponent))