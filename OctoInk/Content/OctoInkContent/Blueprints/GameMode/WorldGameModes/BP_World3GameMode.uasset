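; World 3 game mode that handles the level's directional light for the day/night cycle.
; It extends a parent game mode, calling the parent's cycle and lighting functions before its own changes.
; Each transition plays a timeline that lerps light color and intensity between day and night values, then applies the final preset through SetDayLighting or SetNightLighting.
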(event EventBeginPlay
  (|CallParentFunction))

(event EventTick
  (params (DeltaSeconds :type Float%20%28single-precision%29))
  (|CallParentFunction DeltaSeconds) ; This node is disabled and will not be called.\nDrag off pins to build functionality.
)

(event EventNighttoDayCycle
  (bind _directionallight (Variables|Default|GetDirectionalLight))
  (bind _lightcomponent (Variables|/Script/Engine.Light|GetLightComponent _directionallight))
  (|CallParentFunction)
  (bind _out_alpha (Timeline|Timeline_0 PlayFromStart)
    (:Update
      (Rendering|Components|Light|SetLightColor _lightcomponent (Math|Color|Lerp(LinearColor) (Variables|Default|GetNightDirectionalLightColor) (Variables|Default|GetDayDirectionalLightColor) _out_alpha) false)
      (Rendering|Components|Light|SetIntensity _lightcomponent (Math|Float|Lerp (Variables|Default|GetNightLightIntensity) (Variables|Default|GetDayLightIntensity) _out_alpha)))
    (:Finished
      (CallFunction|SetDayLighting))))

(event EventDaytoNightCycle
  (bind _directionallight (Variables|Default|GetDirectionalLight))
  (bind _lightcomponent (Variables|/Script/Engine.Light|GetLightComponent _directionallight))
  (|CallParentFunction)
  (bind _out_alpha (Timeline|Timeline_1 PlayFromStart)
    (:Update
      (Rendering|Components|Light|SetLightColor _lightcomponent (Math|Color|Lerp(LinearColor) (Variables|Default|GetDayDirectionalLightColor) (Variables|Default|GetNightDirectionalLightColor) _out_alpha) false)
      (Rendering|Components|Light|SetIntensity _lightcomponent (Math|Float|Lerp (Variables|Default|GetDayLightIntensity) (Variables|Default|GetNightLightIntensity) _out_alpha)))
    (:Finished
      (CallFunction|SetNightLighting))))

(fn ConstructionScript
  (|CallParentFunction))

(fn SetDayLighting
  (bind _directionallight (Variables|Default|GetDirectionalLight))
  (bind _lightcomponent (Variables|/Script/Engine.Light|GetLightComponent _directionallight))
  (|CallParentFunction)
  (Rendering|Components|Light|SetLightColor _lightcomponent (Variables|Default|GetDayDirectionalLightColor) false)
  (Rendering|Components|Light|SetIntensity _lightcomponent (Variables|Default|GetDayLightIntensity)))

(fn SetNightLighting
  (bind _directionallight (Variables|Default|GetDirectionalLight))
  (bind _lightcomponent (Variables|/Script/Engine.Light|GetLightComponent _directionallight))
  (|CallParentFunction)
  (Rendering|Components|Light|SetLightColor _lightcomponent (Variables|Default|GetNightDirectionalLightColor) false)
  (Rendering|Components|Light|SetIntensity _lightcomponent (Variables|Default|GetNightLightIntensity)))