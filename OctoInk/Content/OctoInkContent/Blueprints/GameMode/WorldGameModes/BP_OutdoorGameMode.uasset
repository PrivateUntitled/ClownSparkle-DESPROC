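; Outdoor world game mode that extends a parent day/night game mode by recoloring a set of spot lights.
; Cycle events call the parent, then a timeline lerps each light between day and night colors.
; When a timeline finishes, SetDayLighting or SetNightLighting calls its parent version and applies the final color.
; The final day color is set with sRGB on, unlike every other color write.
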(event EventBeginPlay
  (|CallParentFunction) ; This node is disabled and will not be called.\nDrag off pins to build functionality.
)

(event EventTick
  (params (DeltaSeconds :type Float%20%28single-precision%29)))

(event EventDaytoNightCycle
  (|CallParentFunction)
  (bind _out_alpha (Timeline|Timeline_1 PlayFromStart)
    (:Update
      (for _array_element (Variables|Default|GetSpotLightRef)
        (Rendering|Components|Light|SetLightColor (Variables|/Script/Engine.Light|GetLightComponent _array_element) (Math|Color|Lerp(LinearColor) (Variables|Default|GetDayLightColor) (Variables|Default|GetNightLightColor) _out_alpha) false)))
    (:Finished
      (CallFunction|SetNightLighting))))

(event EventNighttoDayCycle
  (|CallParentFunction)
  (bind _out_alpha (Timeline|Timeline_0 PlayFromStart)
    (:Update
      (for _array_element (Variables|Default|GetSpotLightRef)
        (Rendering|Components|Light|SetLightColor (Variables|/Script/Engine.Light|GetLightComponent _array_element) (Math|Color|Lerp(LinearColor) (Variables|Default|GetNightLightColor) (Variables|Default|GetDayLightColor) _out_alpha) false)))
    (:Finished
      (CallFunction|SetDayLighting))))

(fn ConstructionScript
  (|CallParentFunction))

(fn SetDayLighting
  (|CallParentFunction)
  (for _array_element (Variables|Default|GetSpotLightRef)
    (Rendering|Components|Light|SetLightColor (Variables|/Script/Engine.Light|GetLightComponent _array_element) (Variables|Default|GetDayLightColor) true)))

(fn SetNightLighting
  (|CallParentFunction)
  (for _array_element (Variables|Default|GetSpotLightRef)
    (Rendering|Components|Light|SetLightColor (Variables|/Script/Engine.Light|GetLightComponent _array_element) (Variables|Default|GetNightLightColor) false)))