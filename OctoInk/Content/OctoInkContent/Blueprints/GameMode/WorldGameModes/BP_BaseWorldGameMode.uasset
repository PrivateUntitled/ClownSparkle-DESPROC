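; Base game mode for world levels, running the obstacle-inking puzzle that grants the player inspiration.
; BeginPlay binds to the puzzle player's ink event, shows the HUD post-tutorial, calls LoseEnergy during quests and holds a black, muted camera fade before ContinueLoad.
; Correctly colored obstacles stop absorbing and score points; matching the obstacle count refills inspiration duration, spawns an "Inspired" notification and signals completion.
; A helper toggles the Commissioner's visibility, collision and tick.
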(event Custom|Inked
  (params (ObstacleToInk :type BP%20Puzzle%20Interactable%20Object%20Reference))
  (bind _points (Variables|Default|GetPoints))
  (bind _asbp_obstacle (Utilities|Casting|CastToBP_Obstacle ObstacleToInk))
  (if (!= (Variables|/Game/OctoInkContent/Blueprints/Actors/Obstacles/BP_Obstacle.BP_Obstacle_C|GetColorRequired _asbp_obstacle) 0)
    (if (Utilities|Enum|Equal(Enum) (Variables|/Game/OctoInkContent/DataAssets/DataAssets/Color/PDA_Color.PDA_Color_C|GetColor (Variables|/Game/OctoInkContent/Blueprints/Actors/Obstacles/BP_Obstacle.BP_Obstacle_C|GetCurrentColor _asbp_obstacle)) (Variables|/Game/OctoInkContent/DataAssets/DataAssets/Color/PDA_Color.PDA_Color_C|GetColor (Variables|/Game/OctoInkContent/Blueprints/Actors/Obstacles/BP_Obstacle.BP_Obstacle_C|GetColorRequired _asbp_obstacle)))
      (Variables|/Game/OctoInkContent/Blueprints/Actors/Obstacles/BP_Obstacle.BP_Obstacle_C|SetCanAbsorb _asbp_obstacle false)
      (Math|Integer|IncrementInt _points
        (:%20%20
          (if (== _points (Utilities|Array|Length (Variables|Default|GetObstacles)))
            (CallFunction|IBWin)))))))

(event Custom|IBWin
  (bind _gameinstanceref (Variables|Default|GetGameInstanceRef))
  (bind _inspirationdata (Variables|/Game/OctoInkContent/Blueprints/SaveData/MyGame.MyGame_C|GetInspirationData _gameinstanceref))
  (Utilities|Struct|SetmembersinInspirationData _inspirationdata (Utilities|Struct|BreakInspirationData _inspirationdata))
  (bind _returnvalue (Game|SpawnActorfromClass "/Game/OctoInkContent/Blueprints/Actors/MainWorld/BP_Notif.BP_Notif_C" (Math|Conversions|ToTransform(Vector) (Transformation|GetWorldLocation (Variables|/Game/OctoInkContent/Blueprints/Actors/Player/BP_BasePlayer.BP_BasePlayer_C|GetNotifSpawn (Variables|Default|GetBasePlayerRef)))) "Undefined" 0 0))
  (Default|SetText _returnvalue "Inspired")
  (Variables|Default|SetIBFin? true)
  (Default|CallIBCompleted))

(event EventBeginPlay
  (|CallParentFunction)
  (Utilities|FlowControl|Sequence
    (:then_0
      (bind _asbp_puzzle_player (Utilities|Casting|CastToBP_PuzzlePlayer (Game|Player|GetPlayerPawn 0)))
      (EventDispatchers|BindEventtoOnInk _asbp_puzzle_player (delegate Custom|Inked)))
    (:then_1
      (CallFunction|ShowPanel))
    (:then_2
      ;[0 0.02745 1] Losing Energy, and Gaining Reputation
      (if (!= (Utilities|Struct|BreakCommissionData (Variables|/Game/OctoInkContent/Blueprints/SaveData/MyGame.MyGame_C|GetCommissionData (Variables|Default|GetGameInstanceRef))) 0)
        (CallFunction|LoseEnergy)))
    (:then_3
      ;[1 1 1] Mute Audio on Start
      (CameraFades|StartCameraFade :self (Game|GetPlayerCameraManager 0) :FromAlpha 1.0 :ToAlpha 1.0 :Duration 0.0001 :bShouldFadeAudio true :bHoldWhenFinished true)
      (Utilities|FlowControl|Delay 0.0001)
      (CallFunction|ContinueLoad))))

(event EventTick
  (params (DeltaSeconds :type Float%20%28single-precision%29)))

(fn ConstructionScript)

(fn ShowPanel
  (if (.FinishedTutorial (Utilities|Struct|BreakTutorialData (Variables|/Game/OctoInkContent/Blueprints/SaveData/MyGame.MyGame_C|GetTutorialData (Variables|Default|GetGameInstanceRef))))
    (CallFunction|SettingWidget false false "/Game/OctoInkContent/Blueprints/Widgets/MainWorld/BP_TempMainWorldHUD.BP_TempMainWorldHUD_C")))

(fn SetCommissionerVisibility
  (params (HidePerson :type Boolean))
  (bind _returnvalue (not HidePerson))
  (bind _commissioner (Variables|Default|GetCommissioner))
  (bind _capsulecomponent (Variables|/Script/Engine.Character|GetCapsuleComponent _commissioner))
  (Development|SetHiddeninGame _capsulecomponent HidePerson true)
  (Collision|SetActorEnableCollision _commissioner _returnvalue)
  (Actor|Tick|SetActorTickEnabled _commissioner _returnvalue)
  (Development|SetHiddeninGame _capsulecomponent true false))