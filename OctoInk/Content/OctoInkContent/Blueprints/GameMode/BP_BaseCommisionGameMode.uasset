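; Base game mode for commission puzzle levels, handling the HUD, optional quest timer and win/lose outcome.
; BeginPlay creates the puzzle HUD, updates its color on player absorb and ink events, and starts a pause-aware, self-repeating Delay timer ending in an empty TimerCompleted.
; WinLoseCondition shows the commission result widget and updates GameInstance: reputation on wins (inspiration-multiplied), energy cost scaled by consecutive attempts, and day/time from elapsed ticks.
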(event Custom|Timer
  (bind _currenttime (Variables|Default|GetCurrentTime))
  (bind _asbp_player_base_controller (Utilities|Casting|CastToBP_PlayerBaseController (Game|GetPlayerController 0)))
  (if (Variables|/Game/OctoInkContent/Blueprints/Controllers/BP_PlayerBaseController.BP_PlayerBaseController_C|GetisPauseMenuOpen _asbp_player_base_controller)
    (Utilities|FlowControl|Delay 0.1)
    (CallFunction|Timer)
    (else
      (Math|Integer|IncrementInt _currenttime
        (:%20%20
          (if (>= _currenttime (Variables|Default|GetTime))
            (CallFunction|TimerCompleted)
            (else
              (Utilities|FlowControl|Delay 0.1)
              (CallFunction|Timer))))))))

(event Custom|SetColor
  (bind _asbp_puzzle_player (Utilities|Casting|CastToBP_PuzzlePlayer (Game|Player|GetPlayerPawn 0)))
  (CallFunction|SetCurrentColor _asbp_puzzle_player))

(event Custom|WinLoseCondition
  (params (DidPlayerWin :type Boolean))
  (bind _returnvalue (Game|GetPlayerController 0))
  (bind _currenttime (Variables|Default|GetCurrentTime))
  (bind _gameinstanceref (Variables|Default|GetGameInstanceRef))
  (bind _gamemodedata (Variables|/Game/OctoInkContent/Blueprints/SaveData/MyGame.MyGame_C|GetGameModeData _gameinstanceref))
  (bind (_day _time _maxtime) (Utilities|Struct|BreakGameModeData _gamemodedata))
  (bind _returnvalue_2 (/ _currenttime _maxtime))
  (Utilities|FlowControl|Sequence
    (:then_0
      (bind _asbp_player_puzzle_controller (Utilities|Casting|CastToBP_PlayerPuzzleController _returnvalue))
      (Variables|/Game/OctoInkContent/Blueprints/Controllers/BP_PlayerBaseController.BP_PlayerBaseController_C|SetEnableMovement _asbp_player_puzzle_controller false)
      (Variables|/Script/Engine.PlayerController|SetbShowMouseCursor _returnvalue true))
    (:then_1
      (if DidPlayerWin
        (CallFunction|PlayerWins)))
    (:then_2
      (Viewport|RemoveAllWidgets)
      (bind _returnvalue_3 (UserInterface|CreateWidget "/Game/OctoInkContent/Blueprints/Widgets/GeneralWidgets/OverlayWidgets/BP_CommissionWidget.BP_CommissionWidget_C"))
      (Variables|/Game/OctoInkContent/Blueprints/Widgets/GeneralWidgets/OverlayWidgets/BP_CommissionWidget.BP_CommissionWidget_C|SetDidPlayerWin _returnvalue_3 DidPlayerWin)
      (UserInterface|Viewport|AddtoViewport _returnvalue_3 0))
    (:then_3
      (CallFunction|SpendEnergy))
    (:then_4
      (bind _asbp_player_base_controller (Utilities|Casting|CastToBP_PlayerBaseController (Game|GetPlayerController 0)))
      (Variables|/Game/OctoInkContent/Blueprints/Controllers/BP_PlayerBaseController.BP_PlayerBaseController_C|SetisPauseMenuOpen _asbp_player_base_controller true)
      (Utilities|Struct|SetmembersinGameModeData _gamemodedata (+ _returnvalue_2 _day) (+ _time (- _currenttime (* _returnvalue_2 _maxtime)))))))

(event Custom|TimerCompleted)

(event EventBeginPlay
  (Utilities|FlowControl|Sequence
    (:then_0
      (bind _asmy_game (Utilities|Casting|CastToMyGame (Game|GetGameInstance)))
      (Variables|Default|SetGameInstanceRef _asmy_game))
    (:then_1
      ;[1 1 1] Add Puzzle HUD
      (bind _returnvalue (UserInterface|CreateWidget (Variables|Default|GetWidgetClass)))
      (UserInterface|Viewport|AddtoViewport _returnvalue 0)
      (bind _asbp_player_hud (Utilities|Casting|CastToBP_PlayerHUD _returnvalue))
      (Variables|Default|SetPuzzleHUD _asbp_player_hud))
    (:then_2
      ;[1 1 1] Setting up Time in Commision
      (if (and (Variables|Default|GetEnableTime) (!= (Utilities|Struct|BreakCommissionData (Variables|/Game/OctoInkContent/Blueprints/SaveData/MyGame.MyGame_C|GetCommissionData (Variables|Default|GetGameInstanceRef))) 0))
        (Variables|Default|SetTime (Variables|/Game/OctoInkContent/DataAssets/DataAssets/Commissions/PDA_Commission.PDA_Commission_C|GetTimeToComplete (Utilities|Struct|BreakCommissionData (Variables|/Game/OctoInkContent/Blueprints/SaveData/MyGame.MyGame_C|GetCommissionData (Variables|Default|GetGameInstanceRef)))))
        (CallFunction|Timer)))
    (:then_3
      (bind _asbp_puzzle_player (Utilities|Casting|CastToBP_PuzzlePlayer (Game|Player|GetPlayerPawn 0)))
      (CallFunction|SetColor)
      (EventDispatchers|BindEventtoOnAbsorb _asbp_puzzle_player (delegate Custom|SetColor))
      (EventDispatchers|BindEventtoOnInk _asbp_puzzle_player (delegate Custom|SetColor)))))

(fn ConstructionScript)

(fn SpendEnergy
  (bind _gameinstanceref (Variables|Default|GetGameInstanceRef))
  (bind _commissiondata (Variables|/Game/OctoInkContent/Blueprints/SaveData/MyGame.MyGame_C|GetCommissionData _gameinstanceref))
  (bind _playerstats (Variables|/Game/OctoInkContent/Blueprints/SaveData/MyGame.MyGame_C|GetPlayerStats _gameinstanceref))
  (bind _currentquest (Utilities|Struct|BreakCommissionData _commissiondata))
  (bind (_playerenergy _consecutiveattempts) (Utilities|Struct|BreakPlayerStats _playerstats))
  (bind _result (Math|Integer|IncrementInt _consecutiveattempts)
    (:%20%20
      (Utilities|Struct|SetmembersinPlayerStats _playerstats _result)
      (if (!= _currentquest 0)
        (Utilities|Struct|SetmembersinPlayerStats _playerstats (- _playerenergy (* _consecutiveattempts (Variables|/Game/OctoInkContent/DataAssets/DataAssets/Commissions/PDA_Commission.PDA_Commission_C|GetEnergyCost _currentquest))))))))

(fn SetCurrentColor
  (params (Puzzle%20Player%20Ref :type BP%20Puzzle%20Player%20Object%20Reference))
  (bind _puzzlehud (Variables|Default|GetPuzzleHUD))
  (bind _currentcolor (Variables|/Game/OctoInkContent/Blueprints/Actors/Player/BP_PuzzlePlayer.BP_PuzzlePlayer_C|GetCurrentColor Puzzle%20Player%20Ref))
  (Default|SetCurrentColor _puzzlehud (Variables|/Game/OctoInkContent/DataAssets/DataAssets/Color/PDA_Color.PDA_Color_C|GetPointerColor _currentcolor))
  (Default|SetCurrentIconColor _puzzlehud (Variables|/Game/OctoInkContent/DataAssets/DataAssets/Color/PDA_Color.PDA_Color_C|GetPointerColorIcon _currentcolor)))

(fn PlayerWins
  (bind _gameinstanceref (Variables|Default|GetGameInstanceRef))
  (bind _gameinstanceref_2 (Variables|Default|GetGameInstanceRef))
  (bind _playerstats (Variables|/Game/OctoInkContent/Blueprints/SaveData/MyGame.MyGame_C|GetPlayerStats _gameinstanceref_2))
  (bind _inspirationdata (Variables|/Game/OctoInkContent/Blueprints/SaveData/MyGame.MyGame_C|GetInspirationData _gameinstanceref))
  (bind (_duration _inspirationmultiplier) (Utilities|Struct|BreakInspirationData _inspirationdata))
  (if (> _duration 0)
    (LocalVariables|SetReputationMultiplier _inspirationmultiplier)
    (Math|Integer|DecrementInt _duration
      (:%20%20
        _))
    (else
      (LocalVariables|SetReputationMultiplier 1.0)))
  (Utilities|Struct|SetmembersinPlayerStats _playerstats (Math|Float|Truncate (* (+ (Utilities|Struct|BreakPlayerStats _playerstats) (Variables|/Game/OctoInkContent/DataAssets/DataAssets/Commissions/PDA_Commission.PDA_Commission_C|GetReputationEarned (Utilities|Struct|BreakCommissionData (Variables|/Game/OctoInkContent/Blueprints/SaveData/MyGame.MyGame_C|GetCommissionData _gameinstanceref_2)))) (LocalVariables|GetReputationMultiplier)))))