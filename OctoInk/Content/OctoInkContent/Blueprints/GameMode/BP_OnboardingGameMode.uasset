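; Game mode for the onboarding puzzle level, adding tutorial dialogue and an ink-based win check on top of its parent game mode.
; On begin play it requests the first tutorial step and binds CheckWin to the puzzle player's ink event.
; Tutorial requests above the current index advance dialogue one line on the HUD.
; Each ink event compares every blockade's color to its required color to decide whether to trigger the parent's win logic.
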(event Custom|PrintTutorialStep
  (params (StepToPrintIndex :type Integer))
  (if (> StepToPrintIndex (Variables|Default|GetDialogueIndex))
    (Math|Integer|IncrementInt (Variables|Default|GetDialogueIndex)
      (:%20%20
        (Default|PrintDialogueText (Variables|Default|GetPuzzleHUD) (Utilities|Array|Get(acopy) (Variables|Default|GetDialgoueFlow) (Variables|Default|GetDialogueIndex)))))))

(event Custom|CheckWin
  (params (ObstacleToInk :type BP%20Puzzle%20Interactable%20Object%20Reference))
  (CallFunction|CheckWinConidition))

(event EventBeginPlay
  (|CallParentFunction)
  (CallFunction|PrintTutorialStep)
  (bind _asbp_puzzle_player (Utilities|Casting|CastToBP_PuzzlePlayer (Game|Player|GetPlayerPawn 0)))
  (EventDispatchers|BindEventtoOnInk _asbp_puzzle_player (delegate Custom|CheckWin)))

(event EventTick
  (params (DeltaSeconds :type Float%20%28single-precision%29)))

(event EventWinLoseCondition
  (params (DidPlayerWin :type Boolean))
  (|CallParentFunction DidPlayerWin))

(fn ConstructionScript
  (|CallParentFunction))

(fn CheckWinConidition
  (bind _array_element (Utilities|Array|ForEachLoopwithBreak (Variables|Default|GetBlockadeArray) :!label _label)
    (:LoopBody
      (if (not (Utilities|Enum|Equal(Enum) (Variables|/Game/OctoInkContent/DataAssets/DataAssets/Color/PDA_Color.PDA_Color_C|GetColor (Variables|/Game/OctoInkContent/Blueprints/Actors/Obstacles/BP_Obstacle.BP_Obstacle_C|GetCurrentColor _array_element)) (Variables|/Game/OctoInkContent/DataAssets/DataAssets/Color/PDA_Color.PDA_Color_C|GetColor (Variables|/Game/OctoInkContent/Blueprints/Actors/Obstacles/BP_Obstacle.BP_Obstacle_C|GetColorRequired _array_element))))
        (LocalVariables|SetPlayerWins false)
        (goto _label Break)))
    (:Completed
      (if (LocalVariables|GetPlayerWins)
        (CallFunction|WinLoseCondition true)))))

(fn PlayerWins
  (|CallParentFunction))