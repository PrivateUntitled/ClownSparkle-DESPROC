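; Game mode for the third commission, a child of a parent mode that supplies the begin play, timer and win logic.
; On begin play it binds to the puzzle player's ink event, but that handler and SetNewColor are empty.
; An unreachable color-match check would award points and set a new color for a center obstacle.
; A win increments the commission's completion count in the game instance, then runs the parent win logic.
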(event Custom|OnPlayerInk
  (params (ObstacleToInk :type BP%20Puzzle%20Interactable%20Object%20Reference)))

(event EventBeginPlay
  (|CallParentFunction)
  (bind _asbp_puzzle_player (Utilities|Casting|CastToBP_PuzzlePlayer (Game|Player|GetPlayerPawn 0)))
  (EventDispatchers|BindEventtoOnInk _asbp_puzzle_player (delegate Custom|OnPlayerInk)))

(event EventTick
  (params (DeltaSeconds :type Float%20%28single-precision%29)))

(event EventTimer
  (|CallParentFunction))

(fn ConstructionScript
  (|CallParentFunction))

(fn SetNewColor)

(fn PlayerWins
  (Math|Integer|IncrementInt (Utilities|Struct|BreakCommissionData (Variables|/Game/OctoInkContent/Blueprints/SaveData/MyGame.MyGame_C|GetCommissionData (Variables|Default|GetGameInstanceRef)))
    (:%20%20
      (|CallParentFunction))))