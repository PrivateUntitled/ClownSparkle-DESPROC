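; Onboarding game mode that runs The Elder's staged tutorial dialogue over the color-matching obstacle puzzle.
; PlayDialogue locks player movement and steps through lines by chaining the dialogue widget's text-finished event to the controller's proceed event.
; When dialogue ends, it restores movement, swaps to the puzzle HUD with the stage objective and broadcasts DialogueFinished.
; CheckWinConidition compares blockade colors to required ones, triggering a win or playing success or error sounds.
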(event Custom|CustomEvent_1
  (bind _newvar_1 (Variables|Default|GetNewVar_1))
  (bind _result (Math|Integer|IncrementInt (Variables|Default|GetNewVar_0))
    (:%20%20
      (EventDispatchers|UnbindallEventsfromProceedNextDialogue (stale Custom|CustomEvent_0 _asbp_player_puzzle_controller))
      (if (and (< _result (Utilities|Array|Length (.Dialogue (Utilities|Struct|BreakOnboardingStruct (stale Custom|PlayDialogue Stage))))) (Utilities|Enum|Equal(Enum) (.OnboardingStage (Utilities|Struct|BreakOnboardingStruct (stale Custom|PlayDialogue Stage))) (Variables|Default|GetCurrentStage)))
        (Audio|PlaySound2D (.OutItem (Utilities|Array|Random (Variables|Default|GetElderSounds))) 1.0 1.0 0.0 0 0)
        (Default|SetSpeakerInfo _newvar_1 "The Elder" "NewEnumerator1")
        (Default|PrintDialogueText _newvar_1 (Utilities|Array|Get(acopy) (.Dialogue (Utilities|Struct|BreakOnboardingStruct (stale Custom|PlayDialogue Stage))) (stale Custom|PlayDialogue _output_get)))
        (EventDispatchers|BindEventtoTextIsFinished _newvar_1 (delegate Custom|CustomEvent_0))
        (else
          (EventDispatchers|UnbindallEventsfromTextIsFinished _newvar_1)
          (bind _asbp_player_puzzle_controller (Utilities|Casting|CastToBP_PlayerPuzzleController (Game|GetPlayerController 0)))
          (Variables|/Game/OctoInkContent/Blueprints/Controllers/BP_PlayerBaseController.BP_PlayerBaseController_C|SetEnableMovement _asbp_player_puzzle_controller true)
          (CallFunction|ShowPuzzlePanel)
          (Default|CallDialogueFinished (stale Custom|PlayDialogue Stage)))))))

(event Custom|PlayDialogue
  (params (Stage :type Onboarding%20Struct%20Structure))
  (bind (_onboardingstage _dialogue) (Utilities|Struct|BreakOnboardingStruct Stage))
  (bind _newvar_1 (Variables|Default|GetNewVar_1))
  (Variables|Default|SetCurrentDialogue Stage)
  (CallFunction|ShowDialoguePanel)
  (bind _asbp_player_puzzle_controller (Utilities|Casting|CastToBP_PlayerPuzzleController (Game|GetPlayerController 0)))
  (Variables|/Game/OctoInkContent/Blueprints/Controllers/BP_PlayerBaseController.BP_PlayerBaseController_C|SetEnableMovement _asbp_player_puzzle_controller false)
  (Math|Integer|IncrementInt (Variables|Default|GetNextStage)
    (:%20%20
      (Variables|Default|SetCurrentStage _onboardingstage)
      (bind _output_get (Variables|Default|SetNewVar_0 0))
      (Audio|PlaySound2D (.OutItem (Utilities|Array|Random (Variables|Default|GetElderSounds))) 1.0 1.0 0.0 0 0)
      (Default|SetSpeakerInfo _newvar_1 "The Elder" "NewEnumerator1")
      (Default|PrintDialogueText _newvar_1 (Utilities|Array|Get(acopy) _dialogue _output_get))
      (EventDispatchers|BindEventtoTextIsFinished _newvar_1 (delegate Custom|CustomEvent_0)))))

(event Custom|CustomEvent_0
  (bind _asbp_player_puzzle_controller (Utilities|Casting|CastToBP_PlayerPuzzleController (Game|GetPlayerController 0)))
  (EventDispatchers|BindEventtoProceedNextDialogue _asbp_player_puzzle_controller (delegate Custom|CustomEvent_1)))

(event EventBeginPlay
  (|CallParentFunction)
  (Audio|PlaySound2D (Variables|Default|GetSandyBegginingsMusic) 1.0 1.0 0.0 0 0)
  (if (== (Utilities|Struct|BreakOnboardingStruct (Variables|Default|GetIntroDialogue)) (Variables|Default|GetNextStage))
    (CallFunction|PlayDialogue (Variables|Default|GetIntroDialogue))))

(fn ConstructionScript
  (|CallParentFunction))

(fn CheckWinConidition
  (params (PuzzleInteractable :type BP%20Puzzle%20Interactable%20Object%20Reference))
  (bind _array_element (Utilities|Array|ForEachLoopwithBreak (Variables|Default|GetBlockadeArray) :!label _label)
    (:LoopBody
      (if (== _array_element PuzzleInteractable)
        (Utilities|FlowControl|Sequence
          (:then_0
            (bind _array_element_2 (Utilities|Array|ForEachLoopwithBreak (Variables|Default|GetBlockadeArray) :!label _label_2)
              (:LoopBody
                (if (not (Utilities|Enum|Equal(Enum) (Variables|/Game/OctoInkContent/DataAssets/DataAssets/Color/PDA_Color.PDA_Color_C|GetColor (Variables|/Game/OctoInkContent/Blueprints/Actors/Obstacles/BP_Obstacle.BP_Obstacle_C|GetCurrentColor _array_element_2)) (Variables|/Game/OctoInkContent/DataAssets/DataAssets/Color/PDA_Color.PDA_Color_C|GetColor (Variables|/Game/OctoInkContent/Blueprints/Actors/Obstacles/BP_Obstacle.BP_Obstacle_C|GetColorRequired _array_element_2))))
                  (LocalVariables|SetPlayerWins false)
                  (goto _label_2 Break)))
              (:Completed
                (if (LocalVariables|GetPlayerWins)
                  (CallFunction|WinLoseCondition true)
                  (else
                    (bind _asbp_obstacle (Utilities|Casting|CastToBP_Obstacle PuzzleInteractable))
                    (if (Utilities|Enum|Equal(Enum) (Variables|/Game/OctoInkContent/DataAssets/DataAssets/Color/PDA_Color.PDA_Color_C|GetColor (Variables|/Game/OctoInkContent/Blueprints/Actors/Obstacles/BP_Obstacle.BP_Obstacle_C|GetCurrentColor _asbp_obstacle)) (Variables|/Game/OctoInkContent/DataAssets/DataAssets/Color/PDA_Color.PDA_Color_C|GetColor (Variables|/Game/OctoInkContent/Blueprints/Actors/Obstacles/BP_Obstacle.BP_Obstacle_C|GetColorRequired _asbp_obstacle)))
                      (Audio|PlaySound2D "/Game/OctoInkContent/Assets/SFX/sounds/CommissionGeneral/Major_Task_Complete.Major_Task_Complete" 1.0 1.0 0.0 0 0)
                      (else
                        (Audio|PlaySound2D "/Game/OctoInkContent/Assets/SFX/sounds/MenuSounds/Error.Error" 1.0 1.0 0.0 0 0))))))))
          (:then_1
            (goto _label Break)))))))

(fn PlayerWins
  (|CallParentFunction))

(fn ShowDialoguePanel
  (Viewport|RemoveAllWidgets)
  (bind _returnvalue (UserInterface|CreateWidget "/Game/OctoInkContent/Blueprints/Widgets/MainWorld/BP_DialogueHUD.BP_DialogueHUD_C"))
  (UserInterface|Viewport|AddtoViewport _returnvalue 0)
  (Variables|Default|SetNewVar_1 _returnvalue))

(fn ShowPuzzlePanel
  (Viewport|RemoveAllWidgets)
  (bind _returnvalue (UserInterface|CreateWidget "/Game/OctoInkContent/Blueprints/Widgets/Commission/BP_Commission1.BP_PuzzleHUD_C"))
  (UserInterface|Viewport|AddtoViewport _returnvalue 0)
  (Default|SetOnboardingText _returnvalue (Utilities|Struct|BreakOnboardingStruct (Variables|Default|GetCurrentDialogue)))
  (Variables|Default|SetPuzzleHUD _returnvalue))