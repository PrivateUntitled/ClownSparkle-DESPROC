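; Game mode for the second commission puzzle, where the player inks mannequins to match required colors and earn a target score before time runs out.
; Ink events from the puzzle player are checked against each obstacle's required color; matches score by primary, secondary or tertiary tier, spawn point notifications and request new colors.
; Parent overrides handle win/lose, completion counting and timed HUD and sound warnings, while a helper picks random color requirements.
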(event Custom|CustomEvent_0
  (Utilities|FlowControl|Delay 2.0)
  (Variables|Default|SetCanPlayTimerTickSound true))

(event Custom|AddPoint
  (params (Obstacle :type BP%20Obstacle%20Object%20Reference))
  (bind _currentcolor (Variables|/Game/OctoInkContent/Blueprints/Actors/Obstacles/BP_Obstacle.BP_Obstacle_C|GetCurrentColor Obstacle))
  (bind _colortype (Variables|/Game/OctoInkContent/DataAssets/DataAssets/Color/PDA_Color.PDA_Color_C|GetColorType _currentcolor))
  (Default|HideMatchingColor (Variables|/Game/OctoInkContent/Blueprints/Actors/Obstacles/BP_Obstacle.BP_Obstacle_C|GetObstaclePointerRef Obstacle))
  (Utilities|FlowControl|Sequence
    (:then_0
      ;[1 1 1] Add Points
      (switch Utilities|FlowControl|Switch|SwitchonColorType _colortype
        (:NewEnumerator1
          (Math|Integer|IncrementInt (Variables|Default|GetPoints)
            (:%20%20
              (bind _asbp_mannequin (Utilities|Casting|CastToBP_Mannequin Obstacle))
              (CallFunction|AddPointNotif _asbp_mannequin 1))))
        (:NewEnumerator2
          (Variables|Default|SetPoints (Math|Integer|Min(Integer) (+ (Variables|Default|GetPoints) 2) (Variables|Default|GetRequiredPoints)))
          (bind _asbp_mannequin_2 (Utilities|Casting|CastToBP_Mannequin Obstacle))
          (CallFunction|AddPointNotif _asbp_mannequin_2 2))
        (:NewEnumerator3
          (Variables|Default|SetPoints (Math|Integer|Min(Integer) (+ (Variables|Default|GetPoints) 3) (Variables|Default|GetRequiredPoints)))
          (bind _asbp_mannequin_3 (Utilities|Casting|CastToBP_Mannequin Obstacle))
          (CallFunction|AddPointNotif _asbp_mannequin_3 3))))
    (:then_1
      ;[1 1 1] Update UI Text
      (Default|SetColorMannequinText (Variables|Default|GetPuzzleHUD) (Variables|Default|GetPoints) (Variables|Default|GetRequiredPoints)))
    (:then_2
      (if (>= (Variables|Default|GetPoints) (Variables|Default|GetRequiredPoints))
        (CallFunction|WinLoseCondition true)
        (else
          (switch Utilities|FlowControl|Switch|SwitchonColorType _colortype
            (:NewEnumerator0
              _)
            (:NewEnumerator1
              (Audio|PlaySound2D "/Game/OctoInkContent/Assets/SFX/sounds/CommissionGeneral/Major_Task_Complete.Major_Task_Complete" 1.0 1.0 0.0 0 0))
            (:NewEnumerator2
              (Audio|PlaySound2D "/Game/OctoInkContent/Assets/SFX/sounds/CommissionGeneral/Major_Task_Complete2.Major_Task_Complete2" 1.0 1.0 0.0 0 0))
            (:NewEnumerator3
              (Audio|PlaySound2D "/Game/OctoInkContent/Assets/SFX/sounds/CommissionGeneral/Major_Task_Complete3.Major_Task_Complete3" 1.0 1.0 0.0 0 0)))
          (bind _asbp_mannequin_4 (Utilities|Casting|CastToBP_Mannequin Obstacle))
          (Default|FindNewColor _asbp_mannequin_4))))))

(event Custom|OnPlayerInk
  (params (ObstacleToInk :type BP%20Puzzle%20Interactable%20Object%20Reference))
  (bind _asbp_obstacle (Utilities|Casting|CastToBP_Obstacle ObstacleToInk))
  (if (Utilities|Enum|Equal(Enum) (Variables|/Game/OctoInkContent/DataAssets/DataAssets/Color/PDA_Color.PDA_Color_C|GetColor (Variables|/Game/OctoInkContent/Blueprints/Actors/Obstacles/BP_Obstacle.BP_Obstacle_C|GetCurrentColor _asbp_obstacle)) (Variables|/Game/OctoInkContent/DataAssets/DataAssets/Color/PDA_Color.PDA_Color_C|GetColor (Variables|/Game/OctoInkContent/Blueprints/Actors/Obstacles/BP_Obstacle.BP_Obstacle_C|GetColorRequired _asbp_obstacle)))
    (CallFunction|AddPoint _asbp_obstacle)
    (else
      (Audio|PlaySound2D "/Game/OctoInkContent/Assets/SFX/sounds/MenuSounds/Error.Error" 1.0 1.0 0.0 0 0))))

(event EventBeginPlay
  (|CallParentFunction)
  (Default|SetColorMannequinText (Variables|Default|GetPuzzleHUD) (Variables|Default|GetPoints) (Variables|Default|GetRequiredPoints))
  (bind _asbp_puzzle_player (Utilities|Casting|CastToBP_PuzzlePlayer (Game|Player|GetPlayerPawn 0)))
  (EventDispatchers|BindEventtoOnInk _asbp_puzzle_player (delegate Custom|OnPlayerInk))
  (Default|PrintCommission2Task (Variables|Default|GetPuzzleHUD)))

(event EventWinLoseCondition
  (params (DidPlayerWin :type Boolean))
  (|CallParentFunction DidPlayerWin))

(event EventSetColor
  (params (ObstacleToAbsorb :type BP%20Puzzle%20Interactable%20Object%20Reference))
  (|CallParentFunction ObstacleToAbsorb))

(event EventTimerCompleted
  (|CallParentFunction)
  (CallFunction|WinLoseCondition (>= (Variables|Default|GetPoints) (Variables|Default|GetRequiredPoints))))

(event EventTick
  (params (DeltaSeconds :type Float%20%28single-precision%29)))

(fn ConstructionScript
  (|CallParentFunction))

(fn RandomColorRequirement
  (params (Obstacle :type BP%20Obstacle%20Object%20Reference))
  (switch int (Math|Random|RandomIntegerinRange 1 3)
    (:Default
      (Development|PrintString "Default"))
    (:1
      (Default|SetRequiredColor Obstacle (.OutItem (Utilities|Array|Random (Variables|Default|GetPrimaryColors)))))
    (:2
      (Default|SetRequiredColor Obstacle (.OutItem (Utilities|Array|Random (Variables|Default|GetSecondaryColors)))))
    (:3
      (Default|SetRequiredColor Obstacle (.OutItem (Utilities|Array|Random (Variables|Default|GetTertiaryColors)))))))

(fn PlayerWins
  (Math|Integer|IncrementInt (Utilities|Struct|BreakCommissionData (Variables|/Game/OctoInkContent/Blueprints/SaveData/MyGame.MyGame_C|GetCommissionData (Variables|Default|GetGameInstanceRef)))
    (:%20%20
      (|CallParentFunction))))

(fn SetWariningTime
  (bind _puzzlehud (Variables|Default|GetPuzzleHUD))
  (|CallParentFunction)
  (if (Variables|Default|GetCanPlayTimerTickSound)
    (switch string (Utilities|String|ToString(Integer) (/ (- (Variables|Default|GetTime) (Variables|Default|GetCurrentTime)) 10))
      (:120
        (Default|Reminder _puzzlehud :!label _label)
        (Audio|PlaySound2D "/Game/OctoInkContent/Assets/SFX/sounds/CommissionGeneral/Asset_Sound_FX_TimerTick.Asset_Sound_FX_TimerTick" 1.0 1.0 0.0 0 0 :!label _label_2))
      (:60
        (goto _label))
      (:30
        (Default|Warning _puzzlehud)
        (goto _label_2))
      (:5
        (Audio|PlaySound2D "/Game/OctoInkContent/Assets/SFX/sounds/5_seconds_left.5_seconds_left" 1.0 1.0 0.0 0 0)))
    (Variables|Default|SetCanPlayTimerTickSound false)
    (CallFunction|CustomEvent0)))

(fn AddPointNotif
  (params (Mannequin :type BP%20Mannequin%20Object%20Reference) (Points :type Integer))
  (bind _returnvalue (Game|SpawnActorfromClass "/Game/OctoInkContent/Blueprints/Actors/MainWorld/BP_Notif.BP_Notif_C" (Math|Conversions|ToTransform(Vector) (Transformation|GetWorldLocation (Variables|/Game/OctoInkContent/Blueprints/Actors/Obstacles/Blockades/BP_Mannequin.BP_Mannequin_C|GetNotifSpawn Mannequin))) "Undefined" 0 0))
  (Variables|/Game/OctoInkContent/Blueprints/Actors/MainWorld/BP_Notif.BP_Notif_C|SetAlphaLoss _returnvalue 0.05)
  (if (== Points 1)
    (Default|SetText _returnvalue (Utilities|Text|FormatText "+{Value} Point" Points))
    (else
      (Default|SetText _returnvalue (Utilities|Text|FormatText "+{Value} Points" Points)))))