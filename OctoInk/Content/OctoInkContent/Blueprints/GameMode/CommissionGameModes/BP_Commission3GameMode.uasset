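; Game mode for Commission 3, a mural task where the player wins by inking enough paint spots in their required colors before the timer completes.
; It binds to the puzzle player's OnInk event; each color-matched paint spot scores a point, paints the wall and is destroyed.
; Points update the puzzle HUD and trigger the win check, timer completion triggers a loss, and winning increments the completion count in the game instance.
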(event Custom|AddPoint
  (bind _points (Variables|Default|GetPoints))
  (bind _points_2 (Variables|Default|GetPoints))
  (bind _requiredpoints (Variables|Default|GetRequiredPoints))
  (bind _returnvalue (>= _points_2 _requiredpoints))
  (Math|Integer|IncrementInt _points
    (:%20%20
      (Default|SetPaintMuralText (Variables|Default|GetPuzzleHUD) _points (Variables|Default|GetRequiredPoints))
      (if _returnvalue
        (CallFunction|WinLoseCondition _returnvalue)))))

(event Custom|UpdatePointHUD
  (Default|SetPaintMuralText (Variables|Default|GetPuzzleHUD) (Variables|Default|GetPoints) (Variables|Default|GetRequiredPoints)))

(event Custom|OnPlayerInk
  (params (ObstacleToInk :type BP%20Puzzle%20Interactable%20Object%20Reference))
  (bind _asbp_obstacle (Utilities|Casting|CastToBP_Obstacle ObstacleToInk))
  (if (Utilities|Enum|Equal(Enum) (Variables|/Game/OctoInkContent/DataAssets/DataAssets/Color/PDA_Color.PDA_Color_C|GetColor (Variables|/Game/OctoInkContent/Blueprints/Actors/Obstacles/BP_Obstacle.BP_Obstacle_C|GetCurrentColor _asbp_obstacle)) (Variables|/Game/OctoInkContent/DataAssets/DataAssets/Color/PDA_Color.PDA_Color_C|GetColor (Variables|/Game/OctoInkContent/Blueprints/Actors/Obstacles/BP_Obstacle.BP_Obstacle_C|GetColorRequired _asbp_obstacle)))
    (bind _asbp_paint_spot (Utilities|Casting|CastToBP_PaintSpot _asbp_obstacle))
    (CallFunction|AddPoint)
    (Default|PaintWall _asbp_paint_spot)
    (Actor|DestroyActor _asbp_paint_spot)))

(event EventBeginPlay
  (|CallParentFunction)
  (Utilities|FlowControl|Sequence
    (:then_0
      (bind _asbp_puzzle_player (Utilities|Casting|CastToBP_PuzzlePlayer (Game|Player|GetPlayerPawn 0)))
      (EventDispatchers|BindEventtoOnInk _asbp_puzzle_player (delegate Custom|OnPlayerInk))
      (Default|PrintCommission3Task (Variables|Default|GetPuzzleHUD)))
    (:then_1
      (Utilities|FlowControl|Delay 0.0001)
      (Default|SetPaintMuralText (Variables|Default|GetPuzzleHUD) (Variables|Default|GetPoints) (Variables|Default|GetRequiredPoints)))))

(event EventTick
  (params (DeltaSeconds :type Float%20%28single-precision%29)))

(event EventTimerCompleted
  (|CallParentFunction)
  (CallFunction|WinLoseCondition false))

(fn ConstructionScript
  (|CallParentFunction))

(fn PlayerWins
  (Math|Integer|IncrementInt (Utilities|Struct|BreakCommissionData (Variables|/Game/OctoInkContent/Blueprints/SaveData/MyGame.MyGame_C|GetCommissionData (Variables|Default|GetGameInstanceRef)))
    (:%20%20
      (|CallParentFunction))))