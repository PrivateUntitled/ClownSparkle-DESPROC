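; Game mode for the first commission puzzle, where the player wins by inking all required obstacles in their required colors before time runs out.
; It builds the objective HUD and, on each player ink event, checks for a win or plays success/error sounds.
; Each required color toggles matching scenery: trees, flags, jellyfish or bioluminescence.
; It extends parent logic with timed HUD warnings and a completion count saved to the game instance.
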(event Custom|SetObjectives
  (Utilities|FlowControl|Sequence
    (:then_0
      (if (== (Variables|Default|GetPuzzleHUD) 0)
        (bind _returnvalue (UserInterface|CreateWidget (Variables|Default|GetWidgetClass)))
        (UserInterface|Viewport|AddtoViewport _returnvalue 0)
        (bind _asbp_puzzle_hud (Utilities|Casting|CastToBP_PuzzleHUD _returnvalue))
        (Default|Init _asbp_puzzle_hud (Variables|Default|GetCommissionType))
        (Variables|Default|SetPuzzleHUD _asbp_puzzle_hud)))
    (:then_1
      (for (_array_element _array_index) (Variables|Default|GetRequiredObstacles)
        (Default|SetObjectiveText (Variables|Default|GetPuzzleHUD) (+ _array_index 1) _array_element))
      (Default|PrintCommission1Tasks (Variables|Default|GetPuzzleHUD)))))

(event Custom|OnPlayerInk
  (params (ObstacleToInk :type BP%20Puzzle%20Interactable%20Object%20Reference))
  (CallFunction|CheckWinCondition ObstacleToInk))

(event EventBeginPlay
  (|CallParentFunction)
  (bind _asbp_puzzle_player (Utilities|Casting|CastToBP_PuzzlePlayer (Game|Player|GetPlayerPawn 0)))
  (EventDispatchers|BindEventtoOnInk _asbp_puzzle_player (delegate Custom|OnPlayerInk)))

(event EventWinLoseCondition
  (params (DidPlayerWin :type Boolean))
  (|CallParentFunction DidPlayerWin))

(event EventSetColor
  (params (ObstacleToAbsorb :type BP%20Puzzle%20Interactable%20Object%20Reference))
  (|CallParentFunction ObstacleToAbsorb))

(event EventTimerCompleted
  (|CallParentFunction)
  (CallFunction|WinLoseCondition false))

(fn ConstructionScript)

(fn CheckWinCondition
  (params (BP%20Puzzle%20Interactable%20Ref :type BP%20Puzzle%20Interactable%20Object%20Reference))
  (bind _array_element (Utilities|Array|ForEachLoopwithBreak (Variables|Default|GetRequiredObstacles) :!label _label)
    (:LoopBody
      (if (== _array_element BP%20Puzzle%20Interactable%20Ref)
        (Utilities|FlowControl|Sequence
          (:then_0
            (bind _asbp_obstacle (Utilities|Casting|CastToBP_Obstacle BP%20Puzzle%20Interactable%20Ref))
            (Default|SetObstacleRequirement _asbp_obstacle)
            (switch Utilities|FlowControl|Switch|SwitchonColors (Variables|/Game/OctoInkContent/DataAssets/DataAssets/Color/PDA_Color.PDA_Color_C|GetColor (Variables|/Game/OctoInkContent/Blueprints/Actors/Obstacles/BP_Obstacle.BP_Obstacle_C|GetColorRequired _asbp_obstacle))
              (:NewEnumerator16
                (CallFunction|SetTreeVisisbility (Utilities|Enum|NotEqual(Enum) (Variables|/Game/OctoInkContent/DataAssets/DataAssets/Color/PDA_Color.PDA_Color_C|GetColor (Variables|/Game/OctoInkContent/Blueprints/Actors/Obstacles/BP_Obstacle.BP_Obstacle_C|GetCurrentColor _asbp_obstacle)) (Variables|/Game/OctoInkContent/DataAssets/DataAssets/Color/PDA_Color.PDA_Color_C|GetColor (Variables|/Game/OctoInkContent/Blueprints/Actors/Obstacles/BP_Obstacle.BP_Obstacle_C|GetColorRequired _asbp_obstacle)))))
              (:NewEnumerator1
                (CallFunction|SetFlagVisibility (Utilities|Enum|NotEqual(Enum) (Variables|/Game/OctoInkContent/DataAssets/DataAssets/Color/PDA_Color.PDA_Color_C|GetColor (Variables|/Game/OctoInkContent/Blueprints/Actors/Obstacles/BP_Obstacle.BP_Obstacle_C|GetCurrentColor _asbp_obstacle)) (Variables|/Game/OctoInkContent/DataAssets/DataAssets/Color/PDA_Color.PDA_Color_C|GetColor (Variables|/Game/OctoInkContent/Blueprints/Actors/Obstacles/BP_Obstacle.BP_Obstacle_C|GetColorRequired _asbp_obstacle)))))
              (:NewEnumerator2
                (CallFunction|SetJellyfishVisibility (Utilities|Enum|NotEqual(Enum) (Variables|/Game/OctoInkContent/DataAssets/DataAssets/Color/PDA_Color.PDA_Color_C|GetColor (Variables|/Game/OctoInkContent/Blueprints/Actors/Obstacles/BP_Obstacle.BP_Obstacle_C|GetCurrentColor _asbp_obstacle)) (Variables|/Game/OctoInkContent/DataAssets/DataAssets/Color/PDA_Color.PDA_Color_C|GetColor (Variables|/Game/OctoInkContent/Blueprints/Actors/Obstacles/BP_Obstacle.BP_Obstacle_C|GetColorRequired _asbp_obstacle)))))
              (:NewEnumerator4
                (CallFunction|SetBioluminumVisibility (Utilities|Enum|NotEqual(Enum) (Variables|/Game/OctoInkContent/DataAssets/DataAssets/Color/PDA_Color.PDA_Color_C|GetColor (Variables|/Game/OctoInkContent/Blueprints/Actors/Obstacles/BP_Obstacle.BP_Obstacle_C|GetCurrentColor _asbp_obstacle)) (Variables|/Game/OctoInkContent/DataAssets/DataAssets/Color/PDA_Color.PDA_Color_C|GetColor (Variables|/Game/OctoInkContent/Blueprints/Actors/Obstacles/BP_Obstacle.BP_Obstacle_C|GetColorRequired _asbp_obstacle)))))))
          (:then_1
            (bind _array_element_2 (Utilities|Array|ForEachLoopwithBreak (Variables|Default|GetRequiredObstacles) :!label _label_2)
              (:LoopBody
                (if (not (Utilities|Enum|Equal(Enum) (Variables|/Game/OctoInkContent/DataAssets/DataAssets/Color/PDA_Color.PDA_Color_C|GetColor (Variables|/Game/OctoInkContent/Blueprints/Actors/Obstacles/BP_Obstacle.BP_Obstacle_C|GetCurrentColor _array_element_2)) (Variables|/Game/OctoInkContent/DataAssets/DataAssets/Color/PDA_Color.PDA_Color_C|GetColor (Variables|/Game/OctoInkContent/Blueprints/Actors/Obstacles/BP_Obstacle.BP_Obstacle_C|GetColorRequired _array_element_2))))
                  (LocalVariables|SetPlayerWins false)
                  (goto _label_2 Break)))
              (:Completed
                (if (LocalVariables|GetPlayerWins)
                  (CallFunction|WinLoseCondition true)
                  (elif (Utilities|Enum|Equal(Enum) (Variables|/Game/OctoInkContent/DataAssets/DataAssets/Color/PDA_Color.PDA_Color_C|GetColor (Variables|/Game/OctoInkContent/Blueprints/Actors/Obstacles/BP_Obstacle.BP_Obstacle_C|GetCurrentColor _asbp_obstacle)) (Variables|/Game/OctoInkContent/DataAssets/DataAssets/Color/PDA_Color.PDA_Color_C|GetColor (Variables|/Game/OctoInkContent/Blueprints/Actors/Obstacles/BP_Obstacle.BP_Obstacle_C|GetColorRequired _asbp_obstacle)))
                    (Audio|PlaySound2D "/Game/OctoInkContent/Assets/SFX/sounds/CommissionGeneral/Major_Task_Complete.Major_Task_Complete" 1.0 1.0 0.0 0 0)
                    (else
                      (Audio|PlaySound2D "/Game/OctoInkContent/Assets/SFX/sounds/MenuSounds/Error.Error" 1.0 1.0 0.0 0 0)))))))
          (:then_2
            (goto _label Break)))))))

(fn SetCurrentColor
  (params (Puzzle%20Player%20Ref :type BP%20Puzzle%20Player%20Object%20Reference))
  (|CallParentFunction Puzzle%20Player%20Ref))

(fn SpendEnergy
  (|CallParentFunction))

(fn PlayerWins
  (Math|Integer|IncrementInt (.Commision1Completions (Utilities|Struct|BreakCommissionData (Variables|/Game/OctoInkContent/Blueprints/SaveData/MyGame.MyGame_C|GetCommissionData (Variables|Default|GetGameInstanceRef))))
    (:%20%20
      (|CallParentFunction))))

(fn SetTreeVisisbility
  (params (HideTrees :type Boolean))
  (for _array_element (Variables|Default|GetTrees)
    (for _array_element_2 (Actor|GetAttachedActors _array_element true)
      (Rendering|SetActorHiddenInGame _array_element_2 HideTrees))))

(fn SetJellyfishVisibility
  (params (HideJellyfish :type Boolean))
  (for _array_element (Variables|Default|GetJellyFish)
    (Rendering|SetActorHiddenInGame _array_element HideJellyfish))
  (for _array_element_2 (Variables|Default|GetJellyFishFX)
    (Components|Activation|SetActive (Variables|/Script/Niagara.NiagaraActor|GetNiagaraComponent _array_element_2) (not HideJellyfish) false)))

(fn SetFlagVisibility
  (params (HideFlags :type Boolean))
  (for _array_element (Variables|Default|GetFlags)
    (for _array_element_2 (Actor|GetAttachedActors _array_element true)
      (Rendering|SetActorHiddenInGame _array_element_2 HideFlags))))

(fn SetBioluminumVisibility
  (params (HideBioluminum :type Boolean))
  (Rendering|SetActorHiddenInGame (Variables|Default|GetBioluminescence) HideBioluminum))

(fn SetWariningTime
  (bind _puzzlehud (Variables|Default|GetPuzzleHUD))
  (|CallParentFunction)
  (if (Variables|Default|GetCanPlayTimerTickSound)
    (switch string (Utilities|String|ToString(Integer) (/ (- (Variables|Default|GetTime) (Variables|Default|GetCurrentTime)) 10))
      (:240
        (Default|Reminder _puzzlehud :!label _label)
        (Audio|PlaySound2D "/Game/OctoInkContent/Assets/SFX/sounds/CommissionGeneral/Asset_Sound_FX_TimerTick.Asset_Sound_FX_TimerTick" 1.0 1.0 0.0 0 0 :!label _label_2))
      (:180
        (goto _label))
      (:120
        (goto _label))
      (:60
        (Default|Warning _puzzlehud :!label _label_3)
        (goto _label_2))
      (:30
        (goto _label_3))
      (:5
        (Audio|PlaySound2D "/Game/OctoInkContent/Assets/SFX/sounds/5_seconds_left.5_seconds_left" 1.0 1.0 0.0 0 0)))
    (Variables|Default|SetCanPlayTimerTickSound false)
    (CallFunction|SetTimeDelay)))