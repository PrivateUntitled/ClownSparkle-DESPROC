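; Puzzle game mode that runs a timed colour-matching quest, won when every required obstacle has its required colour.
; The player's absorb and ink events update the HUD colour, and inking also refreshes obstacle requirements and checks for a win.
; A self-calling one-second delay counts up to the quest time, triggering a loss.
; Either outcome records stats, shows the commission widget and deducts energy scaled by consecutive attempts.
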(event Custom|OnWin
  (bind _asbp_player_puzzle_controller (Utilities|Casting|CastToBP_PlayerPuzzleController (Game|GetPlayerController 0)))
  (Variables|/Game/OctoInkContent/Blueprints/Controllers/BP_PlayerBaseController.BP_PlayerBaseController_C|SetSetMovement _asbp_player_puzzle_controller false)
  (bind _asmy_game (Utilities|Casting|CastToMyGame (Game|GetGameInstance)))
  (Utilities|Struct|SetmembersinPlayerStats (Variables|/Game/OctoInkContent/Blueprints/SaveData/MyGame.MyGame_C|GetPlayerStats _asmy_game) (+ (.Wins (Utilities|Struct|BreakPlayerStats (Variables|/Game/OctoInkContent/Blueprints/SaveData/MyGame.MyGame_C|GetPlayerStats _asmy_game))) 1))
  (Variables|/Script/Engine.PlayerController|SetbShowMouseCursor (Game|GetPlayerController 0) true)
  (Viewport|RemoveAllWidgets)
  (bind _returnvalue (UserInterface|CreateWidget "/Game/OctoInkContent/Blueprints/Widgets/GeneralWidgets/OverlayWidgets/BP_CommissionWidget.BP_CommissionWidget_C"))
  (Variables|/Game/OctoInkContent/Blueprints/Widgets/GeneralWidgets/OverlayWidgets/BP_CommissionWidget.BP_CommissionWidget_C|SetDidPlayerWin _returnvalue true)
  (UserInterface|Viewport|AddtoViewport _returnvalue 0)
  (CallFunction|SpendEnergy)
  (bind _asbp_player_base_controller (Utilities|Casting|CastToBP_PlayerBaseController (Game|GetPlayerController 0)))
  (Variables|/Game/OctoInkContent/Blueprints/Controllers/BP_PlayerBaseController.BP_PlayerBaseController_C|SetSetMovement _asbp_player_base_controller true))

(event Custom|Timer
  (bind _currenttime (Variables|Default|GetCurrentTime))
  (Math|Integer|IncrementInt _currenttime
    (:%20%20
      (if (>= _currenttime (Variables|Default|GetTime))
        (CallFunction|OnLose)
        (else
          (Utilities|FlowControl|Delay 1.0)
          (CallFunction|Timer))))))

(event Custom|OnLose
  (bind _asbp_player_puzzle_controller (Utilities|Casting|CastToBP_PlayerPuzzleController (Game|GetPlayerController 0)))
  (Variables|/Game/OctoInkContent/Blueprints/Controllers/BP_PlayerBaseController.BP_PlayerBaseController_C|SetSetMovement _asbp_player_puzzle_controller false)
  (bind _asmy_game (Utilities|Casting|CastToMyGame (Game|GetGameInstance)))
  (Utilities|Struct|SetmembersinPlayerStats (Variables|/Game/OctoInkContent/Blueprints/SaveData/MyGame.MyGame_C|GetPlayerStats _asmy_game) (+ (.Loss (Utilities|Struct|BreakPlayerStats (Variables|/Game/OctoInkContent/Blueprints/SaveData/MyGame.MyGame_C|GetPlayerStats _asmy_game))) 1))
  (Variables|/Script/Engine.PlayerController|SetbShowMouseCursor (Game|GetPlayerController 0) true)
  (Viewport|RemoveAllWidgets)
  (bind _returnvalue (UserInterface|CreateWidget "/Game/OctoInkContent/Blueprints/Widgets/GeneralWidgets/OverlayWidgets/BP_CommissionWidget.BP_CommissionWidget_C"))
  (Variables|/Game/OctoInkContent/Blueprints/Widgets/GeneralWidgets/OverlayWidgets/BP_CommissionWidget.BP_CommissionWidget_C|SetDidPlayerWin _returnvalue false)
  (UserInterface|Viewport|AddtoViewport _returnvalue 0)
  (CallFunction|SpendEnergy)
  (bind _asbp_player_base_controller (Utilities|Casting|CastToBP_PlayerBaseController (Game|GetPlayerController 0)))
  (Variables|/Game/OctoInkContent/Blueprints/Controllers/BP_PlayerBaseController.BP_PlayerBaseController_C|SetSetMovement _asbp_player_base_controller true))

(event Custom|OnPlayerInk
  (Utilities|FlowControl|Sequence
    (:then_0
      (for _array_element (Variables|Default|GetRequiredObstacles)
        (Default|SetObstacleRequirment _array_element)
        (if (== _array_element (Variables|/Game/OctoInkContent/Blueprints/Actors/Player/PuzzlePlayer.PuzzlePlayer_C|GetObjectInRange (stale EventBeginPlay _aspuzzle_player)))
          (CallFunction|CheckWinCondition))))
    (:then_1
      (CallFunction|SetCurrentColor (stale EventBeginPlay _aspuzzle_player)))))

(event Custom|OnPlayerAbsorb
  (CallFunction|SetCurrentColor (stale EventBeginPlay _aspuzzle_player)))

(event EventBeginPlay
  (Utilities|FlowControl|Sequence
    (:then_0
      (bind _asmy_game (Utilities|Casting|CastToMyGame (Game|GetGameInstance)))
      (Variables|Default|SetTime (.questtime (Variables|/Game/OctoInkContent/Blueprints/SaveData/MyGame.MyGame_C|GetQuestData _asmy_game)))
      (CallFunction|Timer)
      (bind _returnvalue (UserInterface|CreateWidget "/Game/OctoInkContent/Blueprints/Widgets/Puzzle/BP_PuzzleHUD.BP_PuzzleHUD_C"))
      (UserInterface|Viewport|AddtoViewport _returnvalue 0)
      (Variables|Default|SetPuzzleHUD _returnvalue))
    (:then_1
      (bind _aspuzzle_player (Utilities|Casting|CastToPuzzlePlayer (Game|Player|GetPlayerPawn 0)))
      (EventDispatchers|BindEventtoOnAbsorb _aspuzzle_player (delegate Custom|OnPlayerAbsorb)))
    (:then_2
      (EventDispatchers|BindEventtoOnInk _aspuzzle_player (delegate Custom|OnPlayerInk)))))

(fn ConstructionScript)

(fn CheckWinCondition
  (bind _array_element (Utilities|Array|ForEachLoopwithBreak (Variables|Default|GetRequiredObstacles) :!label _label)
    (:LoopBody
      (if (not (Utilities|Enum|Equal(Enum) (Variables|/Game/OctoInkContent/DataAssets/DataAssets/Color/PDA_Color.PDA_Color_C|GetColor (Variables|/Game/OctoInkContent/Blueprints/Actors/Obstacles/Obstacle.Obstacle_C|GetCurrentColor _array_element)) (Variables|/Game/OctoInkContent/DataAssets/DataAssets/Color/PDA_Color.PDA_Color_C|GetColor (Variables|/Game/OctoInkContent/Blueprints/Actors/Obstacles/Obstacle.Obstacle_C|GetColorRequired _array_element))))
        (LocalVariables|SetPlayerWins false)
        (goto _label Break)))
    (:Completed
      (if (LocalVariables|GetPlayerWins)
        (CallFunction|OnWin)))))

(fn SetCurrentColor
  (params (NewParam :type Puzzle%20Player%20Object%20Reference))
  (Default|SetCurrentColor (Variables|Default|GetPuzzleHUD) (Variables|/Game/OctoInkContent/DataAssets/DataAssets/Color/PDA_Color.PDA_Color_C|GetPointerColor (Variables|/Game/OctoInkContent/Blueprints/Actors/Player/PuzzlePlayer.PuzzlePlayer_C|GetCurrentColor NewParam))))

(fn SpendEnergy
  (bind _asmy_game (Utilities|Casting|CastToMyGame (Game|GetGameInstance)))
  (bind _result (Math|Integer|IncrementInt (.ConsecutiveAttempts (Utilities|Struct|BreakPlayerStats (Variables|/Game/OctoInkContent/Blueprints/SaveData/MyGame.MyGame_C|GetPlayerStats _asmy_game))))
    (:%20%20
      (Utilities|Struct|SetmembersinPlayerStats (Variables|/Game/OctoInkContent/Blueprints/SaveData/MyGame.MyGame_C|GetPlayerStats _asmy_game) _result)
      (Utilities|Struct|SetmembersinPlayerStats (Variables|/Game/OctoInkContent/Blueprints/SaveData/MyGame.MyGame_C|GetPlayerStats _asmy_game) (- (.PlayerEnergy (Utilities|Struct|BreakPlayerStats (Variables|/Game/OctoInkContent/Blueprints/SaveData/MyGame.MyGame_C|GetPlayerStats _asmy_game))) (* (.ConsecutiveAttempts (Utilities|Struct|BreakPlayerStats (Variables|/Game/OctoInkContent/Blueprints/SaveData/MyGame.MyGame_C|GetPlayerStats _asmy_game))) (Utilities|Struct|BreakQuestData (Variables|/Game/OctoInkContent/Blueprints/SaveData/MyGame.MyGame_C|GetQuestData _asmy_game))))))))