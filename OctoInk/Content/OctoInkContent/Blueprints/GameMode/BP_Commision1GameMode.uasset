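; Game mode for Commission 1 of an ink-colouring puzzle, extending a parent game mode with this level's win check and scenery reveals.
; Each player ink event updates required obstacles, showing flags, trees or jellyfish with Niagara effects when their colours match; Blue only prints.
; A win is declared when all obstacles match, and timer completion triggers a loss.
; Winning increments the commission's completion count in the game instance.
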(event Custom|OnPlayerInk
  (Development|PrintString "Hello")
  (CallFunction|CheckWinCondition))

(event EventBeginPlay
  (|CallParentFunction)
  (bind _asbp_puzzle_player (Utilities|Casting|CastToBP_PuzzlePlayer (Game|Player|GetPlayerPawn 0)))
  (EventDispatchers|BindEventtoOnInk _asbp_puzzle_player (delegate Custom|OnPlayerInk)))

(event EventWinLoseCondition
  (params (DidPlayerWin :type Boolean))
  (|CallParentFunction DidPlayerWin))

(event EventSetColor
  (|CallParentFunction))

(event EventTimerCompleted
  (|CallParentFunction)
  (CallFunction|WinLoseCondition false))

(fn ConstructionScript)

(fn CheckWinCondition
  (Utilities|FlowControl|Sequence
    (:then_0
      (bind _array_element (Utilities|Array|ForEachLoopwithBreak (Variables|Default|GetRequiredObstacles))
        (:LoopBody
          (Default|SetObstacleRequirement _array_element)
          (switch Utilities|FlowControl|Switch|SwitchonColors (Variables|/Game/OctoInkContent/DataAssets/DataAssets/Color/PDA_Color.PDA_Color_C|GetColor (Variables|/Game/OctoInkContent/Blueprints/Actors/Obstacles/BP_Obstacle.BP_Obstacle_C|GetColorRequired _array_element))
            (:NewEnumerator8
              (Development|PrintString "Show Flag")
              (CallFunction|SetFlagVisibility (Utilities|Enum|NotEqual(Enum) (Variables|/Game/OctoInkContent/DataAssets/DataAssets/Color/PDA_Color.PDA_Color_C|GetColor (Variables|/Game/OctoInkContent/Blueprints/Actors/Obstacles/BP_Obstacle.BP_Obstacle_C|GetCurrentColor _array_element)) (Variables|/Game/OctoInkContent/DataAssets/DataAssets/Color/PDA_Color.PDA_Color_C|GetColor (Variables|/Game/OctoInkContent/Blueprints/Actors/Obstacles/BP_Obstacle.BP_Obstacle_C|GetColorRequired _array_element)))))
            (:NewEnumerator16
              (Development|PrintString "Show Trees")
              (CallFunction|SetTreeVisisbility (Utilities|Enum|NotEqual(Enum) (Variables|/Game/OctoInkContent/DataAssets/DataAssets/Color/PDA_Color.PDA_Color_C|GetColor (Variables|/Game/OctoInkContent/Blueprints/Actors/Obstacles/BP_Obstacle.BP_Obstacle_C|GetCurrentColor _array_element)) (Variables|/Game/OctoInkContent/DataAssets/DataAssets/Color/PDA_Color.PDA_Color_C|GetColor (Variables|/Game/OctoInkContent/Blueprints/Actors/Obstacles/BP_Obstacle.BP_Obstacle_C|GetColorRequired _array_element)))))
            (:NewEnumerator2
              (Development|PrintString "Show Jellyfish")
              (CallFunction|SetJellyfishVisibility (Utilities|Enum|NotEqual(Enum) (Variables|/Game/OctoInkContent/DataAssets/DataAssets/Color/PDA_Color.PDA_Color_C|GetColor (Variables|/Game/OctoInkContent/Blueprints/Actors/Obstacles/BP_Obstacle.BP_Obstacle_C|GetCurrentColor _array_element)) (Variables|/Game/OctoInkContent/DataAssets/DataAssets/Color/PDA_Color.PDA_Color_C|GetColor (Variables|/Game/OctoInkContent/Blueprints/Actors/Obstacles/BP_Obstacle.BP_Obstacle_C|GetColorRequired _array_element)))))
            (:NewEnumerator4
              (Development|PrintString "Show Biolum"))))))
    (:then_1
      (bind _array_element_2 (Utilities|Array|ForEachLoopwithBreak (Variables|Default|GetRequiredObstacles) :!label _label)
        (:LoopBody
          (if (not (Utilities|Enum|Equal(Enum) (Variables|/Game/OctoInkContent/DataAssets/DataAssets/Color/PDA_Color.PDA_Color_C|GetColor (Variables|/Game/OctoInkContent/Blueprints/Actors/Obstacles/BP_Obstacle.BP_Obstacle_C|GetCurrentColor _array_element_2)) (Variables|/Game/OctoInkContent/DataAssets/DataAssets/Color/PDA_Color.PDA_Color_C|GetColor (Variables|/Game/OctoInkContent/Blueprints/Actors/Obstacles/BP_Obstacle.BP_Obstacle_C|GetColorRequired _array_element_2))))
            (LocalVariables|SetPlayerWins false)
            (goto _label Break)))
        (:Completed
          (if (LocalVariables|GetPlayerWins)
            (CallFunction|WinLoseCondition true)))))))

(fn SetCurrentColor
  (params (Puzzle%20Player%20Ref :type BP%20Puzzle%20Player%20Object%20Reference))
  (|CallParentFunction Puzzle%20Player%20Ref))

(fn SpendEnergy
  (|CallParentFunction))

(fn PlayerWins
  (Math|Integer|IncrementInt (.Commision1Completions (Utilities|Struct|BreakCommissionData (Variables|/Game/OctoInkContent/Blueprints/SaveData/MyGame.MyGame_C|GetCommissionData (Variables|Default|GetGameInstanceRef))))
    (:%20%20
      (|CallParentFunction))))

(fn SetTreeVisisbility
  (params (HideTrees :type Boolean))
  (for _array_element (Variables|Default|GetTrees)
    (for _array_element_2 (Actor|GetAttachedActors _array_element true)
      (Rendering|SetActorHiddenInGame _array_element_2 HideTrees))))

(fn SetJellyfishVisibility
  (params (HideJellyfish :type Boolean))
  (for _array_element (Variables|Default|GetJellyFish)
    (Rendering|SetActorHiddenInGame _array_element HideJellyfish))
  (for _array_element_2 (Variables|Default|GetJellyFishFX)
    (Components|Activation|SetActive (Variables|/Script/Niagara.NiagaraActor|GetNiagaraComponent _array_element_2) (not HideJellyfish) false)))

(fn SetFlagVisibility
  (params (HideFlags :type Boolean))
  (for _array_element (Variables|Default|GetFlags)
    (Rendering|SetActorHiddenInGame _array_element HideFlags)))