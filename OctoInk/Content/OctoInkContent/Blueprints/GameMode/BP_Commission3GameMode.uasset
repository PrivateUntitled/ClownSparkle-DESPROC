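; Game mode for a timed ink puzzle commission where the player scores by inking mannequins in their required colors.
; Each player ink event scores the first matching mannequin, worth more for secondary and tertiary colors than primary.
; A scored mannequin turns transparent and, after a short delay, gets a random required color from a random tier.
; When the parent's timer completes, the point total against RequiredPoints decides win or loss.
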(event Custom|AddPoint
  (params (Obstacle :type BP%20Obstacle%20Object%20Reference))
  (Utilities|FlowControl|Sequence
    (:then_0
      (switch Utilities|FlowControl|Switch|SwitchonColorType (Variables|/Game/OctoInkContent/DataAssets/DataAssets/Color/PDA_Color.PDA_Color_C|GetColorType (Variables|/Game/OctoInkContent/Blueprints/Actors/Obstacles/BP_Obstacle.BP_Obstacle_C|GetCurrentColor Obstacle))
        (:NewEnumerator1
          (Math|Integer|IncrementInt (Variables|Default|GetPoints)))
        (:NewEnumerator2
          (Variables|Default|SetPoints (+ (Variables|Default|GetPoints) 2)))
        (:NewEnumerator3
          (Variables|Default|SetPoints (+ (Variables|Default|GetPoints) 3)))))
    (:then_1
      (Development|PrintString (Utilities|String|ToString(Integer) (Variables|Default|GetPoints)))
      (Variables|/Game/OctoInkContent/Blueprints/Actors/Obstacles/BP_Obstacle.BP_Obstacle_C|SetColorRequired Obstacle 0)
      (Default|SetObstacleColor Obstacle "/Game/OctoInkContent/DataAssets/DataAssets/Color/DA_Transparent.DA_Transparent")
      (Utilities|FlowControl|Delay 3.0)
      (CallFunction|RandomColorRequirement Obstacle))))

(event Custom|OnPlayerInk
  (bind _array_element (Utilities|Array|ForEachLoopwithBreak (Variables|Default|GetMannequins) :!label _label)
    (:LoopBody
      (if (Utilities|Enum|Equal(Enum) (Variables|/Game/OctoInkContent/DataAssets/DataAssets/Color/PDA_Color.PDA_Color_C|GetColor (Variables|/Game/OctoInkContent/Blueprints/Actors/Obstacles/BP_Obstacle.BP_Obstacle_C|GetCurrentColor _array_element)) (Variables|/Game/OctoInkContent/DataAssets/DataAssets/Color/PDA_Color.PDA_Color_C|GetColor (Variables|/Game/OctoInkContent/Blueprints/Actors/Obstacles/BP_Obstacle.BP_Obstacle_C|GetColorRequired _array_element)))
        (CallFunction|AddPoint _array_element)
        (goto _label Break)))))

(event EventBeginPlay
  (|CallParentFunction)
  (bind _asbp_puzzle_player (Utilities|Casting|CastToBP_PuzzlePlayer (Game|Player|GetPlayerPawn 0)))
  (EventDispatchers|BindEventtoOnInk _asbp_puzzle_player (delegate Custom|OnPlayerInk)))

(event EventWinLoseCondition
  (params (DidPlayerWin :type Boolean))
  (|CallParentFunction DidPlayerWin))

(event EventSetColor
  (|CallParentFunction))

(event EventTimerCompleted
  (|CallParentFunction)
  (CallFunction|WinLoseCondition (>= (Variables|Default|GetPoints) (Variables|Default|GetRequiredPoints))))

(event EventTick
  (params (DeltaSeconds :type Float%20%28single-precision%29)))

(fn ConstructionScript
  (|CallParentFunction))

(fn RandomColorRequirement
  (params (Obstacle :type BP%20Obstacle%20Object%20Reference))
  (switch int (Math|Random|RandomIntegerinRange 1 3)
    (:Default
      (Development|PrintString "Default"))
    (:1
      (Variables|/Game/OctoInkContent/Blueprints/Actors/Obstacles/BP_Obstacle.BP_Obstacle_C|SetColorRequired Obstacle (.OutItem (Utilities|Array|Random (Variables|Default|GetPrimaryColors))))
      (Default|SetObstacleColor Obstacle "/Game/OctoInkContent/DataAssets/DataAssets/Color/DA_Transparent.DA_Transparent"))
    (:2
      (Variables|/Game/OctoInkContent/Blueprints/Actors/Obstacles/BP_Obstacle.BP_Obstacle_C|SetColorRequired Obstacle (.OutItem (Utilities|Array|Random (Variables|Default|GetSecondaryColors))))
      (Default|SetObstacleColor Obstacle "/Game/OctoInkContent/DataAssets/DataAssets/Color/DA_Transparent.DA_Transparent"))
    (:3
      (Variables|/Game/OctoInkContent/Blueprints/Actors/Obstacles/BP_Obstacle.BP_Obstacle_C|SetColorRequired Obstacle (.OutItem (Utilities|Array|Random (Variables|Default|GetTertiaryColors))))
      (Default|SetObstacleColor Obstacle "/Game/OctoInkContent/DataAssets/DataAssets/Color/DA_Transparent.DA_Transparent"))))