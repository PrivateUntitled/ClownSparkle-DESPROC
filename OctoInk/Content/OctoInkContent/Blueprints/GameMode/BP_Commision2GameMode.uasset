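; BP_Commision2GameMode is the game mode for the second commission, a color-matching challenge played with the ink puzzle player.
; On BeginPlay it binds to the player's OnInk event, and each ink scores a point if the center obstacle's color matches its required color.
; A match then picks a random required color and resets the obstacle to transparent.
; Winning increments the commission's completion count before running parent logic.
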(event Custom|OnPlayerInk
  (bind _centerobstacle (Variables|Default|GetCenterObstacle))
  (if (Utilities|Enum|Equal(Enum) (Variables|/Game/OctoInkContent/DataAssets/DataAssets/Color/PDA_Color.PDA_Color_C|GetColor (Variables|/Game/OctoInkContent/Blueprints/Actors/Obstacles/BP_Obstacle.BP_Obstacle_C|GetCurrentColor _centerobstacle)) (Variables|/Game/OctoInkContent/DataAssets/DataAssets/Color/PDA_Color.PDA_Color_C|GetColor (Variables|/Game/OctoInkContent/Blueprints/Actors/Obstacles/BP_Obstacle.BP_Obstacle_C|GetColorRequired _centerobstacle)))
    (Math|Integer|IncrementInt (Variables|Default|GetPoints)
      (:%20%20
        (CallFunction|SetNewColor)))))

(event EventBeginPlay
  (|CallParentFunction)
  (bind _asbp_puzzle_player (Utilities|Casting|CastToBP_PuzzlePlayer (Game|Player|GetPlayerPawn 0)))
  (EventDispatchers|BindEventtoOnInk _asbp_puzzle_player (delegate Custom|OnPlayerInk)))

(event EventTick
  (params (DeltaSeconds :type Float%20%28single-precision%29)))

(event EventTimer
  (|CallParentFunction))

(fn ConstructionScript
  (|CallParentFunction))

(fn SetNewColor
  (bind _colorlist (Variables|Default|GetColorList))
  (bind _output_get (LocalVariables|SetNewLocalVar_0 (.OutIndex (Utilities|Array|Random _colorlist))))
  (Variables|/Game/OctoInkContent/Blueprints/Actors/Obstacles/BP_Obstacle.BP_Obstacle_C|SetColorRequired (Variables|Default|GetCenterObstacle) (Utilities|Array|Get(acopy) _colorlist _output_get))
  (Variables|/Game/OctoInkContent/Blueprints/Actors/Obstacles/BP_Obstacle.BP_Obstacle_C|SetColorsRestricted (Variables|Default|GetCenterObstacle) (Utilities|Array|MakeArray (Utilities|Array|Get(acopy) _colorlist _output_get)))
  (Default|SetObstacleColor (Variables|Default|GetCenterObstacle) "/Game/OctoInkContent/DataAssets/DataAssets/Color/DA_Transparent.DA_Transparent"))

(fn PlayerWins
  (Math|Integer|IncrementInt (Utilities|Struct|BreakQuestData (Variables|/Game/OctoInkContent/Blueprints/SaveData/MyGame.MyGame_C|GetCommissionData (Variables|Default|GetGameInstanceRef)))
    (:%20%20
      (|CallParentFunction))))