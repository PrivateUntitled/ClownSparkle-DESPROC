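; BP_PuzzlePlayer is a player character for color puzzles that swaps its color with nearby obstacles.
; Box overlaps track the obstacle in range, while mesh overlaps flag whether the player is inside one.
; Absorb and Ink both exchange colors through SetPlayerColor and SetObstacleColor, updating the player's material and HasColor flag.
; Ink also asks the BP_Puzzle game mode to check the win condition when that obstacle is a required one.
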(event OnComponentBeginOverlap(Box)
  (params (OverlappedComponent :type Primitive%20Component%20Object%20Reference) (OtherActor :type Actor%20Object%20Reference) (OtherComp :type Primitive%20Component%20Object%20Reference) (OtherBodyIndex :type Integer) (bFromSweep :type Boolean) (SweepResult :type Hit%20Result%20Structure%20%28by%20ref%29))
  (bind _asobstacle (Utilities|Casting|CastToObstacle OtherActor))
  (Variables|Default|SetObjectInRange _asobstacle))

(event OnComponentEndOverlap(Box)
  (params (OverlappedComponent :type Primitive%20Component%20Object%20Reference) (OtherActor :type Actor%20Object%20Reference) (OtherComp :type Primitive%20Component%20Object%20Reference) (OtherBodyIndex :type Integer))
  (Utilities|Casting|CastToObstacle OtherActor)
  (Variables|Default|SetObjectInRange 0))

(event OnComponentBeginOverlap(Mesh)
  (params (OverlappedComponent :type Primitive%20Component%20Object%20Reference) (OtherActor :type Actor%20Object%20Reference) (OtherComp :type Primitive%20Component%20Object%20Reference) (OtherBodyIndex :type Integer) (bFromSweep :type Boolean) (SweepResult :type Hit%20Result%20Structure%20%28by%20ref%29))
  (Utilities|Casting|CastToObstacle OtherActor)
  (Variables|Default|SetIsPlayerInObstacle true))

(event OnComponentEndOverlap(Mesh)
  (params (OverlappedComponent :type Primitive%20Component%20Object%20Reference) (OtherActor :type Actor%20Object%20Reference) (OtherComp :type Primitive%20Component%20Object%20Reference) (OtherBodyIndex :type Integer))
  (Utilities|Casting|CastToObstacle OtherActor)
  (Variables|Default|SetIsPlayerInObstacle false))

(event EventBeginPlay
  (CallFunction|SetPlayerColor (Variables|Default|GetCurrentColor))
  (|CallParentFunction))

(fn ConstructionScript)

(fn Absorb
  (Utilities|FlowControl|Sequence
    (:then_0
      (bind _asobstacle (Utilities|Casting|CastToObstacle (Variables|Default|GetObjectInRange)))
      ;[1 1 1] Set Player Color
      (LocalVariables|SetObstacleColor (Variables|/Game/OctoInkContent/Actors/Obstacle.Obstacle_C|GetCurrentColor _asobstacle)))
    (:then_1
      ;[1 1 1] Set Enemy Material
      (Default|SetObstacleColor _asobstacle (Variables|Default|GetCurrentColor)))
    (:then_2
      (CallFunction|SetPlayerColor (LocalVariables|GetObstacleColor)))))

(fn Ink
  (Utilities|FlowControl|Sequence
    (:then_0
      (bind _asobstacle (Utilities|Casting|CastToObstacle (Variables|Default|GetObjectInRange)))
      (LocalVariables|SetEnemyMaterial (Variables|/Game/OctoInkContent/Actors/Obstacle.Obstacle_C|GetCurrentColor _asobstacle)))
    (:then_1
      (Default|SetObstacleColor _asobstacle (Variables|Default|GetCurrentColor)))
    (:then_2
      (CallFunction|SetPlayerColor (LocalVariables|GetEnemyMaterial)))
    (:then_3
      (bind _asbp_puzzle (Utilities|Casting|CastToBP_Puzzle (Game|GetGameMode)))
      (for _array_element (Variables|/Game/OctoInkContent/GameMode/BP_Puzzle.BP_Puzzle_C|GetRequiredObstacles _asbp_puzzle)
        (if (== _array_element (Variables|Default|GetObjectInRange))
          (Default|CheckWinCondition _asbp_puzzle))))))

(fn SetPlayerColor
  (params (NewCharacterColor :type PDA%20Color%20Object%20Reference))
  (bind _output_get (Variables|Default|SetCurrentColor NewCharacterColor))
  (Rendering|Material|SetMaterial (Variables|Character|GetMesh) 0 (Variables|/Game/OctoInkContent/Data_Assets/Color/PDA_Color.PDA_Color_C|GetRockMaterial _output_get))
  (Variables|Default|SetHasColor (Utilities|Enum|NotEqual(Enum) (Variables|/Game/OctoInkContent/Data_Assets/Color/PDA_Color.PDA_Color_C|GetColor (Variables|Default|GetCurrentColor)) "NewEnumerator6")))