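; BP_Quest is a quest-giver NPC that offers a quest to the player through dialogue.
; TalkToPlayer binds to the player controller's DialogueDone event before running the parent's talk logic.
; The Response event switches on dialogue type, telling the BP_MainWorld game mode to show the quest, start it or stop.
; ReplyYes and ReplyNo have the game mode show the matching accept or decline dialogue.
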(event Custom|Response
  (params (Dialogue :type PDA%20Dialogue%20Object%20Reference))
  (bind _returnvalue (Game|GetGameMode))
  (switch Utilities|FlowControl|Switch|SwitchonDialogueType (Variables|/Game/OctoInkContent/Data_Assets/PDA_Dialogue.PDA_Dialogue_C|GetType Dialogue)
    (:NewEnumerator6
      (bind _asbp_main_world (Utilities|Casting|CastToBP_MainWorld _returnvalue))
      (Default|ShowQuest _asbp_main_world (Variables|Default|GetQuest)))
    (:NewEnumerator7
      (bind _asbp_main_world_2 (Utilities|Casting|CastToBP_MainWorld _returnvalue))
      (Default|StartQuest _asbp_main_world_2))
    (:NewEnumerator8
      (bind _asbp_main_world_3 (Utilities|Casting|CastToBP_MainWorld _returnvalue))
      (Default|Stop _asbp_main_world_3))))

(event EventBeginPlay
  (|CallParentFunction) ; This node is disabled and will not be called.\nDrag off pins to build functionality.
)

(event Collision|EventActorBeginOverlap
  (params (OtherActor :type Actor%20Object%20Reference))
  (|CallParentFunction OtherActor) ; This node is disabled and will not be called.\nDrag off pins to build functionality.
)

(event EventTick
  (params (DeltaSeconds :type Float%20%28single-precision%29))
  (|CallParentFunction DeltaSeconds) ; This node is disabled and will not be called.\nDrag off pins to build functionality.
)

(fn ConstructionScript
  (|CallParentFunction))

(fn TalktoPlayer
  (bind _asbp_player_main_game_controller (Utilities|Casting|CastToBP_PlayerMainGameController (Pawn|GetController (Game|Player|GetPlayerPawn 0))))
  (EventDispatchers|BindEventtoDialogueDone _asbp_player_main_game_controller (EventDispatchers|CreateEvent :!event Custom|Response))
  (|CallParentFunction))

(fn ReplyYes
  (bind _asbp_main_world (Utilities|Casting|CastToBP_MainWorld (Game|GetGameMode)))
  (Default|ShowDialogue _asbp_main_world (Variables|Default|GetYesDialogue)))

(fn ReplyNo
  (bind _asbp_main_world (Utilities|Casting|CastToBP_MainWorld (Game|GetGameMode)))
  (Default|ShowDialogue _asbp_main_world (Variables|Default|GetNoDialogue)))