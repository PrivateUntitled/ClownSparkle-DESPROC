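; Player Blueprint for OctoInk that trades color with nearby obstacles through material swaps.
; Box overlaps track the Obstacle in range, while mesh overlaps flag when the player is inside one.
; Absorb and Ink both swap slot-0 materials with that obstacle; Absorb clears HasColor and disables obstacle collision, and Ink does the reverse.
; Neither function is called within this Blueprint or checks that an obstacle is in range.
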(event OnComponentBeginOverlap(Box)
  (params (OverlappedComponent :type Primitive%20Component%20Object%20Reference) (OtherActor :type Actor%20Object%20Reference) (OtherComp :type Primitive%20Component%20Object%20Reference) (OtherBodyIndex :type Integer) (bFromSweep :type Boolean) (SweepResult :type Hit%20Result%20Structure%20%28by%20ref%29))
  (bind _asobstacle (Utilities|Casting|CastToObstacle OtherActor))
  (Variables|Default|SetObstacleInRange _asobstacle))

(event OnComponentEndOverlap(Box)
  (params (OverlappedComponent :type Primitive%20Component%20Object%20Reference) (OtherActor :type Actor%20Object%20Reference) (OtherComp :type Primitive%20Component%20Object%20Reference) (OtherBodyIndex :type Integer))
  (Utilities|Casting|CastToObstacle OtherActor)
  (Variables|Default|SetObstacleInRange 0))

(event OnComponentBeginOverlap(Mesh)
  (params (OverlappedComponent :type Primitive%20Component%20Object%20Reference) (OtherActor :type Actor%20Object%20Reference) (OtherComp :type Primitive%20Component%20Object%20Reference) (OtherBodyIndex :type Integer) (bFromSweep :type Boolean) (SweepResult :type Hit%20Result%20Structure%20%28by%20ref%29))
  (Utilities|Casting|CastToObstacle OtherActor)
  (Variables|Default|SetIsPlayerInObstacle true))

(event OnComponentEndOverlap(Mesh)
  (params (OverlappedComponent :type Primitive%20Component%20Object%20Reference) (OtherActor :type Actor%20Object%20Reference) (OtherComp :type Primitive%20Component%20Object%20Reference) (OtherBodyIndex :type Integer))
  (Utilities|Casting|CastToObstacle OtherActor)
  (Variables|Default|SetIsPlayerInObstacle false))

(event EventBeginPlay)

(event Collision|EventActorBeginOverlap
  (params (OtherActor :type Actor%20Object%20Reference)))

(event EventTick
  (params (DeltaSeconds :type Float%20%28single-precision%29)))

(fn ConstructionScript)

(fn Absorb
  (bind _obstacleinrange (Variables|Default|GetObstacleInRange))
  (bind _staticmesh (Variables|/Game/OctoInkContent/Actors/Obstacle.Obstacle_C|GetStaticMesh _obstacleinrange))
  (Utilities|FlowControl|Sequence
    (:then_0
      ;[1 1 1] Set Player Color
      (LocalVariables|SetPlayerColor (Rendering|Material|GetMaterial (Variables|Character|GetMesh) 0)))
    (:then_1
      ;[1 1 1] Set Enemy Material
      (Rendering|Material|SetMaterial (Variables|Character|GetMesh) 0 (Rendering|Material|GetMaterial _staticmesh 0)))
    (:then_2
      ;[1 1 1] Set Player Material
      (Rendering|Material|SetMaterial _staticmesh 0 (LocalVariables|GetPlayerColor)))
    (:then_3
      (Variables|Default|SetHasColor false))
    (:then_4
      (Default|SetCollision (Variables|Default|GetObstacleInRange) false))))

(fn Ink
  (bind _obstacleinrange (Variables|Default|GetObstacleInRange))
  (bind _staticmesh (Variables|/Game/OctoInkContent/Actors/Obstacle.Obstacle_C|GetStaticMesh _obstacleinrange))
  (Utilities|FlowControl|Sequence
    (:then_0
      (LocalVariables|SetEnemyMaterial (Rendering|Material|GetMaterial _staticmesh 0)))
    (:then_1
      (Rendering|Material|SetMaterial _staticmesh 0 (Rendering|Material|GetMaterial (Variables|Character|GetMesh) 0)))
    (:then_2
      (Rendering|Material|SetMaterial (Variables|Character|GetMesh) 0 (LocalVariables|GetEnemyMaterial)))
    (:then_3
      (Variables|Default|SetHasColor true))
    (:then_4
      (Default|SetCollision (Variables|Default|GetObstacleInRange) true))))