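; BP_Puzzle runs a timed colour-matching puzzle level, with its time limit taken from the quest time in MyGame save data.
; BeginPlay shows the puzzle HUD and starts a self-recalling one-second Delay timer that triggers a loss on expiry.
; CheckWinCondition triggers a win when every required obstacle has its required colour.
; Both outcomes disable movement, update SaveData (reward gold or mental energy penalty) and open MainGame.
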(event Custom|OnWin
  (bind _asbp_player_puzzle_controller (Utilities|Casting|CastToBP_PlayerPuzzleController (Game|GetPlayerController 0)))
  (Variables|/Game/OctoInkContent/Controllers/BP_PlayerBaseController.BP_PlayerBaseController_C|SetSetMovement _asbp_player_puzzle_controller false)
  (bind _asmy_game (Utilities|Casting|CastToMyGame (Game|GetGameInstance)))
  (Variables|/Game/OctoInkContent/MyGame.MyGame_C|SetSaveData _asmy_game (Utilities|Struct|MakeSaveGameData 0 0 (+ (.playergold (Variables|/Game/OctoInkContent/MyGame.MyGame_C|GetSaveData _asmy_game)) (.questreward (Variables|/Game/OctoInkContent/MyGame.MyGame_C|GetSaveData _asmy_game))) (.playermentalenergy (Variables|/Game/OctoInkContent/MyGame.MyGame_C|GetSaveData _asmy_game)) (.playerphysicalenergy (Variables|/Game/OctoInkContent/MyGame.MyGame_C|GetSaveData _asmy_game)) (.playerlastknownmainworldlocation (Variables|/Game/OctoInkContent/MyGame.MyGame_C|GetSaveData _asmy_game))))
  (Game|OpenLevel(byName) "MainGame"))

(event Custom|Timer
  (bind _currenttime (Variables|Default|GetCurrentTime))
  (Math|Integer|IncrementInt _currenttime
    (:%20%20
      (if (>= _currenttime (Variables|Default|GetTime))
        (CallFunction|OnLose)
        (else
          (Utilities|FlowControl|Delay 1.0)
          (CallFunction|Timer))))))

(event Custom|OnLose
  (bind _asbp_player_puzzle_controller (Utilities|Casting|CastToBP_PlayerPuzzleController (Game|GetPlayerController 0)))
  (Variables|/Game/OctoInkContent/Controllers/BP_PlayerBaseController.BP_PlayerBaseController_C|SetSetMovement _asbp_player_puzzle_controller false)
  (bind _asmy_game (Utilities|Casting|CastToMyGame (Game|GetGameInstance)))
  (Variables|/Game/OctoInkContent/MyGame.MyGame_C|SetSaveData _asmy_game (Utilities|Struct|MakeSaveGameData (.questreward (Variables|/Game/OctoInkContent/MyGame.MyGame_C|GetSaveData _asmy_game)) (.questtime (Variables|/Game/OctoInkContent/MyGame.MyGame_C|GetSaveData _asmy_game)) (.playergold (Variables|/Game/OctoInkContent/MyGame.MyGame_C|GetSaveData _asmy_game)) (- (.playermentalenergy (Variables|/Game/OctoInkContent/MyGame.MyGame_C|GetSaveData _asmy_game)) 100) (.playerphysicalenergy (Variables|/Game/OctoInkContent/MyGame.MyGame_C|GetSaveData _asmy_game)) (.playerlastknownmainworldlocation (Variables|/Game/OctoInkContent/MyGame.MyGame_C|GetSaveData _asmy_game))))
  (Game|OpenLevel(byName) "MainGame"))

(event EventBeginPlay
  (bind _asmy_game (Utilities|Casting|CastToMyGame (Game|GetGameInstance)))
  (Variables|Default|SetTime (.questtime (Variables|/Game/OctoInkContent/MyGame.MyGame_C|GetSaveData _asmy_game)))
  (CallFunction|Timer)
  (bind _returnvalue (UserInterface|CreateWidget "/Game/OctoInkContent/HUD/BP_PuzzleHUD.BP_PuzzleHUD_C"))
  (UserInterface|Viewport|AddtoViewport _returnvalue 0))

(event EventTick
  (params (DeltaSeconds :type Float%20%28single-precision%29)))

(fn ConstructionScript)

(fn CheckWinCondition
  (bind _array_element (Utilities|Array|ForEachLoopwithBreak (Variables|Default|GetRequiredObstacles) :!label _label)
    (:LoopBody
      (if (not (Utilities|Enum|Equal(Enum) (Variables|/Game/OctoInkContent/Data_Assets/Color/PDA_Color.PDA_Color_C|GetColor (Variables|/Game/OctoInkContent/Actors/Obstacle.Obstacle_C|GetCurrentColor _array_element)) (Variables|/Game/OctoInkContent/Actors/Obstacle.Obstacle_C|GetColorRequired _array_element)))
        (LocalVariables|SetPlayerWins false)
        (goto _label Break)))
    (:Completed
      (if (LocalVariables|GetPlayerWins)
        (CallFunction|OnWin)))))