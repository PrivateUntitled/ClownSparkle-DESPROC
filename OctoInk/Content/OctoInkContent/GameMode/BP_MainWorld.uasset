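; Main world game mode that switches between HUD, quest and dialogue screens and launches quest levels.
; On BeginPlay it restores the player's transform, gold and mental energy from the MyGame instance.
; ShowQuest, ShowDialogue and Stop route through SettingWidget, which replaces all widgets and sets cursor visibility and the controller's SetMovement flag.
; StartQuest saves quest reward, time, player stats (including physical energy) and transform to MyGame, then opens the quest's level.
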(event Custom|Stop
  (CallFunction|SettingWidget false false "/Game/OctoInkContent/HUD/BP_MainWorldHUD.BP_MainWorldHUD_C")
  (Variables|Default|SetCurrentQuest 0)
  (Variables|Default|SetCurrentDialogue 0))

(event Custom|ShowQuest
  (params (CurrentQuest :type PDA%20Quest%20Object%20Reference))
  (Variables|Default|SetCurrentQuest CurrentQuest)
  (CallFunction|SettingWidget true true "/Game/OctoInkContent/HUD/BP_Quest.BP_Quest_C"))

(event Custom|ShowDialogue
  (params (Dialogue :type PDA%20Dialogue%20Object%20Reference))
  (Variables|Default|SetCurrentDialogue Dialogue)
  (CallFunction|SettingWidget false true "/Game/OctoInkContent/HUD/BP_Dialogue.BP_Dialogue_C"))

(event Custom|StartQuest
  (bind _returnvalue (Game|Player|GetPlayerPawn 0))
  (bind _currentquest (Variables|Default|GetCurrentQuest))
  (bind _asmy_game (Utilities|Casting|CastToMyGame (Game|GetGameInstance)))
  (bind _asmain_game_player (Utilities|Casting|CastToMainGamePlayer _returnvalue))
  (Default|SetGameInstance _asmy_game (Utilities|Struct|MakeSaveGameData (Variables|/Game/OctoInkContent/Data_Assets/PDA_Quest.PDA_Quest_C|GetReward _currentquest) (Variables|/Game/OctoInkContent/Data_Assets/PDA_Quest.PDA_Quest_C|GetTime _currentquest) (Variables|/Game/OctoInkContent/Actors/Player/MainGamePlayer.MainGamePlayer_C|GetGold _asmain_game_player) (Variables|/Game/OctoInkContent/Actors/Player/BasePlayer.BasePlayer_C|GetMentalEnergy _asmain_game_player) (Variables|/Game/OctoInkContent/Actors/Player/BasePlayer.BasePlayer_C|GetPhysicalEnergy _asmain_game_player) (Transformation|GetWorldTransform (Variables|/Script/Engine.Actor|GetRootComponent _returnvalue))))
  (Game|OpenLevel(byName) (Variables|/Game/OctoInkContent/Data_Assets/PDA_Quest.PDA_Quest_C|GetLevelName _currentquest)))

(event EventBeginPlay
  (CallFunction|SettingWidget false false "/Game/OctoInkContent/HUD/BP_MainWorldHUD.BP_MainWorldHUD_C")
  (bind _asmy_game (Utilities|Casting|CastToMyGame (Game|GetGameInstance)))
  (bind _savedata (Default|GetGameInstace _asmy_game))
  (bind _asmain_game_player (Utilities|Casting|CastToMainGamePlayer (Game|Player|GetPlayerPawn 0)))
  (Utilities|FlowControl|Sequence
    (:then_0
      (Transformation|SetWorldTransform (Variables|/Script/Engine.Character|GetCapsuleComponent _asmain_game_player) (.playerlastknownmainworldlocation _savedata) false false))
    (:then_1
      (Variables|/Game/OctoInkContent/Actors/Player/MainGamePlayer.MainGamePlayer_C|SetGold _asmain_game_player (.playergold _savedata)))
    (:then_2
      (Variables|/Game/OctoInkContent/Actors/Player/BasePlayer.BasePlayer_C|SetMentalEnergy _asmain_game_player (.playermentalenergy _savedata)))))

(event EventTick
  (params (DeltaSeconds :type Float%20%28single-precision%29)))

(fn ConstructionScript)

(fn SettingWidget
  (params (ShowMouseCursor :type Boolean) (IsTalking :type Boolean) (WidgetClass :type User%20Widget%20Class%20Reference))
  (bind _returnvalue (Game|GetPlayerController 0))
  (Utilities|FlowControl|Sequence
    (:then_0
      (bind _asbp_player_base_controller (Utilities|Casting|CastToBP_PlayerBaseController _returnvalue))
      (Variables|/Game/OctoInkContent/Controllers/BP_PlayerBaseController.BP_PlayerBaseController_C|SetSetMovement _asbp_player_base_controller IsTalking))
    (:then_1
      (Variables|/Script/Engine.PlayerController|SetbShowMouseCursor _returnvalue ShowMouseCursor))
    (:then_2
      (Viewport|RemoveAllWidgets))
    (:then_3
      (if (Utilities|IsValidClass WidgetClass)
        (bind _returnvalue_2 (UserInterface|CreateWidget WidgetClass))
        (UserInterface|Viewport|AddtoViewport _returnvalue_2 0)))))