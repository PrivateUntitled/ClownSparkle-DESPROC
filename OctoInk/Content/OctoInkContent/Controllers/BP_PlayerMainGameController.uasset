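; Main game player controller that handles left-click interaction with quest NPCs in range of the player.
; With a dialogue widget open, a click advances and prints the next line, or calls DialogueDone with the game mode's current dialogue on the last one.
; Otherwise, if no BP_Quest widget is showing, it starts conversation through TalkToPlayer.
; Starting or advancing a conversation plays a random NPC sound at the player's location.
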(event EventBeginPlay
  (|CallParentFunction)
  (bind _asmain_game_player (Utilities|Casting|CastToMainGamePlayer (Game|Player|GetPlayerPawn 0)))
  (Variables|Default|SetMainGamePlayer _asmain_game_player))

(event Input|MouseEvents|LeftMouseButton
  (params (Key :type Key%20Structure :default "None"))
  (bind _maingameplayer (Variables|Default|GetMainGamePlayer))
  (bind _questinrange (Variables|/Game/OctoInkContent/Actors/Player/MainGamePlayer.MainGamePlayer_C|GetQuestInRange _maingameplayer))
  (:Pressed
    (bind _foundwidgets (Widget|GetAllWidgetsOfClass "/Game/OctoInkContent/HUD/BP_Dialogue.BP_Dialogue_C" true))
    (if (and (Utilities|IsValid (Utilities|Array|Get(acopy) _foundwidgets)) (Utilities|IsValid (Variables|/Game/OctoInkContent/Actors/Player/MainGamePlayer.MainGamePlayer_C|GetQuestInRange (Variables|Default|GetMainGamePlayer))))
      (bind _asbp_main_world (Utilities|Casting|CastToBP_MainWorld (Game|GetGameMode)))
      (if (< (Variables|/Game/OctoInkContent/HUD/BP_Dialogue.BP_Dialogue_C|GetDialogueIndex (Utilities|Array|Get(acopy) _foundwidgets)) (- (Utilities|Array|Length (Variables|/Game/OctoInkContent/Data_Assets/PDA_Dialogue.PDA_Dialogue_C|GetDialogue (Variables|/Game/OctoInkContent/GameMode/BP_MainWorld.BP_MainWorld_C|GetCurrentDialogue _asbp_main_world))) 1))
        (Math|Integer|IncrementInt (Variables|/Game/OctoInkContent/HUD/BP_Dialogue.BP_Dialogue_C|GetDialogueIndex (Utilities|Array|Get(acopy) _foundwidgets))
          (:%20%20
            (Default|PrintDialogueText (Utilities|Array|Get(acopy) _foundwidgets))
            (bind _asmain_game_player (Utilities|Casting|CastToMainGamePlayer (Game|Player|GetPlayerPawn 0)))
            (bind _asbp_quest (Utilities|Casting|CastToBP_Quest (Variables|/Game/OctoInkContent/Actors/Player/MainGamePlayer.MainGamePlayer_C|GetQuestInRange _asmain_game_player)))
            (Audio|PlaySoundatLocation (.OutItem (Utilities|Array|Random (Variables|/Game/OctoInkContent/Actors/QuestPeople/BaseNPCs/BP_BasePerson.BP_BasePerson_C|GetNPC_Sounds _asbp_quest))) (Transformation|GetWorldLocation (Variables|/Script/Engine.Character|GetCapsuleComponent _asmain_game_player)) "0, 0, 0" 1.0 1.0 0.0 0 0 0)))
        (else
          (Default|CallDialogueDone self (Variables|/Game/OctoInkContent/GameMode/BP_MainWorld.BP_MainWorld_C|GetCurrentDialogue _asbp_main_world))))
      (else
        (bind _foundwidgets_2 (Widget|GetAllWidgetsOfClass "/Game/OctoInkContent/HUD/BP_Quest.BP_Quest_C" true))
        (if (and (not (Utilities|IsValid (Utilities|Array|Get(acopy) _foundwidgets_2))) (Utilities|IsValid _questinrange))
          (bind _asbp_base_person (Utilities|Casting|CastToBP_BasePerson _questinrange))
          (bind _asmain_game_player_2 (Utilities|Casting|CastToMainGamePlayer (Game|Player|GetPlayerPawn 0)))
          (bind _asbp_quest_2 (Utilities|Casting|CastToBP_Quest (Variables|/Game/OctoInkContent/Actors/Player/MainGamePlayer.MainGamePlayer_C|GetQuestInRange _asmain_game_player_2)))
          (Audio|PlaySoundatLocation (.OutItem (Utilities|Array|Random (Variables|/Game/OctoInkContent/Actors/QuestPeople/BaseNPCs/BP_BasePerson.BP_BasePerson_C|GetNPC_Sounds _asbp_quest_2))) (Transformation|GetWorldLocation (Variables|/Script/Engine.Character|GetCapsuleComponent _asmain_game_player_2)) "0, 0, 0" 1.0 1.0 0.0 0 0 0)
          (Default|TalktoPlayer _asbp_base_person))))))

(fn ConstructionScript
  (|CallParentFunction))