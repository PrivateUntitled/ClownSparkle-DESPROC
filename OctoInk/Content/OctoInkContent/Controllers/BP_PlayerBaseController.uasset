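; Player controller that drives the BasePlayer character with isometric eight-way movement and a short dash on Space.
; Move axes apply diagonal world-space input, then Movement converts their truncated values into a compass direction.
; SetAnimation passes that direction to BP_PlayerAnimator, which receives only four facings, and rotates the character's Scene component in 45-degree steps.
; Dash briefly spikes walk speed and acceleration before a cooldown; jump calls exist but are unwired.
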(event Custom|Dash
  (bind _playercharacterref (Variables|Default|GetPlayerCharacterRef))
  (bind _charactermovement (Variables|/Script/Engine.Character|GetCharacterMovement _playercharacterref))
  (Variables|Default|SetCanDash false)
  (Variables|/Script/Engine.CharacterMovementComponent|SetMaxWalkSpeed _charactermovement 1e+04)
  (Variables|/Script/Engine.CharacterMovementComponent|SetMaxAcceleration _charactermovement 1e+04)
  (Utilities|FlowControl|Delay 0.2)
  (Variables|/Script/Engine.CharacterMovementComponent|SetMaxWalkSpeed _charactermovement 6e+02)
  (Variables|/Script/Engine.CharacterMovementComponent|SetMaxAcceleration _charactermovement 2048.0)
  (Utilities|FlowControl|Delay 1.0)
  (Variables|Default|SetCanDash true))

(event Custom|Movement
  (bind _xaxis (Variables|Default|GetXAxis))
  (bind _returnvalue (Math|Float|Truncate _xaxis))
  (switch int (Math|Float|Truncate (Variables|Default|GetYAxis))
    (:-1
      (switch int _returnvalue
        (:-1
          (CallFunction|SetAnimation "NewEnumerator4"))
        (:0
          (CallFunction|SetAnimation "NewEnumerator2"))
        (:1
          (CallFunction|SetAnimation "NewEnumerator1"))))
    (:0
      (switch int _returnvalue
        (:-1
          (CallFunction|SetAnimation "NewEnumerator5"))
        (:0
          (CallFunction|SetAnimation "NewEnumerator3"))
        (:1
          (CallFunction|SetAnimation "NewEnumerator0"))))
    (:1
      (switch int _returnvalue
        (:-1
          (CallFunction|SetAnimation "NewEnumerator6"))
        (:0
          (CallFunction|SetAnimation "NewEnumerator7"))
        (:1
          (CallFunction|SetAnimation "NewEnumerator8"))))))

(event Custom|SetAnimation
  (params (Direction :type Directions%20Enum :default "NewEnumerator3"))
  (bind _playercharacterref (Variables|Default|GetPlayerCharacterRef))
  (bind _scene (Variables|/Game/OctoInkContent/Actors/Player/BasePlayer.BasePlayer_C|GetScene _playercharacterref))
  (Utilities|FlowControl|Sequence
    (:then_0
      ;[1 1 1] Setting Animation
      (bind _asbp_player_animator (Utilities|Casting|CastToBP_PlayerAnimator (Variables|/Script/PaperZD.PaperZDAnimationComponent|GetAnimInstance (Variables|/Script/PaperZD.PaperZDCharacter|GetAnimationComponent _playercharacterref))))
      (switch Utilities|FlowControl|Switch|SwitchonDirections Direction
        (:NewEnumerator0
          (Variables|/Game/OctoInkContent/Assets/Dan/BP_PlayerAnimator.BP_PlayerAnimator_C|SetDirection _asbp_player_animator 1 :!label _label))
        (:NewEnumerator1
          (goto _label))
        (:NewEnumerator4
          (Variables|/Game/OctoInkContent/Assets/Dan/BP_PlayerAnimator.BP_PlayerAnimator_C|SetDirection _asbp_player_animator 0 :!label _label_2))
        (:NewEnumerator5
          (goto _label_2))
        (:NewEnumerator6
          (Variables|/Game/OctoInkContent/Assets/Dan/BP_PlayerAnimator.BP_PlayerAnimator_C|SetDirection _asbp_player_animator 2))
        (:NewEnumerator8
          (Variables|/Game/OctoInkContent/Assets/Dan/BP_PlayerAnimator.BP_PlayerAnimator_C|SetDirection _asbp_player_animator 3))))
    (:then_1
      (switch Utilities|FlowControl|Switch|SwitchonDirections Direction
        (:NewEnumerator0
          (Transformation|SetWorldRotation _scene "0,45.000000, 0" false false))
        (:NewEnumerator1
          (Transformation|SetWorldRotation _scene "0,90.000000, 0" false false))
        (:NewEnumerator2
          (Transformation|SetWorldRotation _scene "0,135.000000, 0" false false))
        (:NewEnumerator4
          (Transformation|SetWorldRotation _scene "0,180.000000, 0" false false))
        (:NewEnumerator5
          (Transformation|SetWorldRotation _scene "0,225.000000, 0" false false))
        (:NewEnumerator6
          (Transformation|SetWorldRotation _scene "0,270.000000, 0" false false))
        (:NewEnumerator7
          (Transformation|SetWorldRotation _scene "0,315.000000, 0" false false))
        (:NewEnumerator8
          (Transformation|SetWorldRotation _scene "0, 0, 0" false false))))))

(event EventBeginPlay
  (bind _asbase_player (Utilities|Casting|CastToBasePlayer (Game|GetPlayerCharacter 0)))
  (Variables|Default|SetPlayerCharacterRef _asbase_player)
  (CallFunction|SetAnimation "NewEnumerator4"))

(event EventTick
  (params (DeltaSeconds :type Float%20%28single-precision%29)))

(event Input|ActionEvents|InputActionJump
  (params (Key :type Key%20Structure :default "None"))
  ;[1 1 1] Jump Mechanic (Hook to Implement)
)

(event Input|AxisEvents|InputAxisMoveForward
  (params (AxisValue :type Float%20%28single-precision%29))
  ;[1 1 1] WASD Movement
  (bind _output_get (Variables|Default|SetYAxis AxisValue))
  (Pawn|Input|AddMovementInput (Variables|Default|GetPlayerCharacterRef) "1.000000,-1.000000, 0" _output_get false)
  (CallFunction|Movement))

(event Input|AxisEvents|InputAxisMoveRight
  (params (AxisValue :type Float%20%28single-precision%29))
  ;[1 1 1] WASD Movement
  (bind _output_get (Variables|Default|SetXAxis AxisValue))
  (Pawn|Input|AddMovementInput (Variables|Default|GetPlayerCharacterRef) "1.000000,1.000000, 0" _output_get false)
  (CallFunction|Movement))

(event Input|KeyboardEvents|SpaceBar
  (params (Key :type Key%20Structure :default "None"))
  ;[1 1 1] Dash Mechanic (Hook to implement)
  (:Pressed
    (if (Variables|Default|GetCanDash)
      (CallFunction|Dash))))

(fn ConstructionScript)