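; Player controller that drives BP_Player with diagonally rotated WASD movement, a dash, and ink/absorb actions.
; Movement axes add input along world diagonals, while key press/release handlers snap the mesh to eight-way facings.
; Space briefly boosts walk speed and acceleration; jump calls are unwired.
; Mouse buttons call Ink (left) or Absorb (right) on the player after checking HasColor, player position and whether the nearby obstacle's material is Transparent.
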(event EventBeginPlay
  (bind _asbp_player (Utilities|Casting|CastToBP_Player (Game|GetPlayerCharacter 0)))
  (Variables|Default|SetPlayerCharacterRef _asbp_player))

(event Input|ActionEvents|InputActionJump
  (params (Key :type Key%20Structure :default "None"))
  ;[1 1 1] Jump Mechanic (Hook to Implement)
)

(event Input|AxisEvents|InputAxisMoveForward
  (params (AxisValue :type Float%20%28single-precision%29))
  (bind _playercharacterref (Variables|Default|GetPlayerCharacterRef))
  (bind _mesh (Variables|/Script/Engine.Character|GetMesh _playercharacterref))
  ;[1 1 1] WASD Movement
  (Pawn|Input|AddMovementInput (Variables|Default|GetPlayerCharacterRef) "1.000000,-1.000000, 0" AxisValue false)
  ;[1 1 1] Makes sure the movement leaves you at the right direction on NWSE
  (if (and (Game|Player|IsInputKeyDown "S") (Game|Player|IsInputKeyDown "D"))
    (Transformation|SetWorldRotation _mesh "0, 0, 0" false false)
    (elif (and (Game|Player|IsInputKeyDown "S") (Game|Player|IsInputKeyDown "A"))
      (Transformation|SetWorldRotation _mesh "0,90.000000, 0" false false))))

(event Input|AxisEvents|InputAxisMoveRight
  (params (AxisValue :type Float%20%28single-precision%29))
  (bind _playercharacterref (Variables|Default|GetPlayerCharacterRef))
  (bind _mesh (Variables|/Script/Engine.Character|GetMesh _playercharacterref))
  ;[1 1 1] WASD Movement
  (Pawn|Input|AddMovementInput (Variables|Default|GetPlayerCharacterRef) "1.000000,1.000000, 0" AxisValue false)
  ;[1 1 1] Makes sure the movement leaves you at the right direction on NWSE
  (if (and (Game|Player|IsInputKeyDown "W") (Game|Player|IsInputKeyDown "D"))
    (Transformation|SetWorldRotation _mesh "0,-90.000000, 0" false false)
    (elif (and (Game|Player|IsInputKeyDown "W") (Game|Player|IsInputKeyDown "A"))
      (Transformation|SetWorldRotation _mesh "0,180.000000, 0" false false))))

(event Input|MouseEvents|RightMouseButton
  (params (Key :type Key%20Structure :default "None"))
  (bind _playercharacterref (Variables|Default|GetPlayerCharacterRef))
  (bind _obstacleinrange (Variables|/Game/OctoInkContent/Actors/BP_Player.BP_Player_C|GetObstacleInRange _playercharacterref))
  ;[1 1 1] Absorb
  (:Pressed
    (if (Math|Boolean|ANDBoolean (!= _obstacleinrange 0) (Variables|/Game/OctoInkContent/Actors/BP_Player.BP_Player_C|GetHasColor _playercharacterref) (not (Variables|/Game/OctoInkContent/Actors/BP_Player.BP_Player_C|GetIsPlayerInObstacle _playercharacterref)))
      (if (!= (Rendering|Material|GetMaterial (Variables|/Game/OctoInkContent/Actors/Obstacle.Obstacle_C|GetStaticMesh _obstacleinrange) 0) "/Game/OctoInkContent/Materials/Transparent.Transparent")
        (Default|Absorb (Variables|Default|GetPlayerCharacterRef))))))

(event Input|KeyboardEvents|A
  (params (Key :type Key%20Structure :default "None"))
  (bind _playercharacterref (Variables|Default|GetPlayerCharacterRef))
  (bind _mesh (Variables|/Script/Engine.Character|GetMesh _playercharacterref))
  ;[1 1 1] Makes sure movement leaves you facing the right direction NW, NE, SW, SE
  (:Pressed
    (Transformation|SetWorldRotation _mesh "0,135.000000, 0" false false))
  (:Released
    (if (Game|Player|IsInputKeyDown "W")
      (Transformation|SetWorldRotation _mesh "0,-135.000000, 0" false false)
      (elif (Game|Player|IsInputKeyDown "S")
        (Transformation|SetWorldRotation _mesh "0,45.000000, 0" false false)
        (elif (Game|Player|IsInputKeyDown "D")
          (Transformation|SetWorldRotation _mesh "0,-45.000000, 0" false false))))))

(event Input|KeyboardEvents|SpaceBar
  (params (Key :type Key%20Structure :default "None"))
  (bind _playercharacterref (Variables|Default|GetPlayerCharacterRef))
  (bind _charactermovement (Variables|/Script/Engine.Character|GetCharacterMovement _playercharacterref))
  ;[1 1 1] Dash Mechanic (Hook to implement)
  (:Pressed
    (Variables|/Script/Engine.CharacterMovementComponent|SetMaxWalkSpeed _charactermovement 1e+04)
    (Variables|/Script/Engine.CharacterMovementComponent|SetMaxAcceleration _charactermovement 1e+04)
    (Utilities|FlowControl|Delay 0.2)
    (Variables|/Script/Engine.CharacterMovementComponent|SetMaxWalkSpeed _charactermovement 6e+02)
    (Variables|/Script/Engine.CharacterMovementComponent|SetMaxAcceleration _charactermovement 2048.0)))

(event Input|MouseEvents|LeftMouseButton
  (params (Key :type Key%20Structure :default "None"))
  (bind _playercharacterref (Variables|Default|GetPlayerCharacterRef))
  (bind _obstacleinrange (Variables|/Game/OctoInkContent/Actors/BP_Player.BP_Player_C|GetObstacleInRange _playercharacterref))
  ;[1 1 1] Ink
  (:Pressed
    (if (Math|Boolean|ANDBoolean (!= _obstacleinrange 0) (not (Variables|/Game/OctoInkContent/Actors/BP_Player.BP_Player_C|GetHasColor _playercharacterref)) (not (Variables|/Game/OctoInkContent/Actors/BP_Player.BP_Player_C|GetIsPlayerInObstacle _playercharacterref)))
      (if (== (Rendering|Material|GetMaterial (Variables|/Game/OctoInkContent/Actors/Obstacle.Obstacle_C|GetStaticMesh _obstacleinrange) 0) "/Game/OctoInkContent/Materials/Transparent.Transparent")
        (Default|Ink (Variables|Default|GetPlayerCharacterRef))))))

(event Input|KeyboardEvents|W
  (params (Key :type Key%20Structure :default "None"))
  (bind _playercharacterref (Variables|Default|GetPlayerCharacterRef))
  (bind _mesh (Variables|/Script/Engine.Character|GetMesh _playercharacterref))
  ;[1 1 1] Makes sure movement leaves you facing the right direction NW, NE, SW, SE
  (:Pressed
    (Transformation|SetWorldRotation _mesh "0,-135.000000, 0" false false))
  (:Released
    (if (Game|Player|IsInputKeyDown "D")
      (Transformation|SetWorldRotation _mesh "0,-45.000000, 0" false false)
      (elif (Game|Player|IsInputKeyDown "A")
        (Transformation|SetWorldRotation _mesh "0,135.000000, 0" false false)
        (elif (Game|Player|IsInputKeyDown "S")
          (Transformation|SetWorldRotation _mesh "0,45.000000, 0" false false))))))

(event Input|KeyboardEvents|S
  (params (Key :type Key%20Structure :default "None"))
  (bind _playercharacterref (Variables|Default|GetPlayerCharacterRef))
  (bind _mesh (Variables|/Script/Engine.Character|GetMesh _playercharacterref))
  ;[1 1 1] Makes sure movement leaves you facing the right direction NW, NE, SW, SE
  (:Pressed
    (Transformation|SetWorldRotation _mesh "0,45.000000, 0" false false))
  (:Released
    (if (Game|Player|IsInputKeyDown "D")
      (Transformation|SetWorldRotation _mesh "0,-45.000000, 0" false false)
      (elif (Game|Player|IsInputKeyDown "A")
        (Transformation|SetWorldRotation _mesh "0,135.000000, 0" false false)
        (elif (Game|Player|IsInputKeyDown "W")
          (Transformation|SetWorldRotation _mesh "0,-135.000000, 0" false false))))))

(event Input|KeyboardEvents|D
  (params (Key :type Key%20Structure :default "None"))
  (bind _playercharacterref (Variables|Default|GetPlayerCharacterRef))
  (bind _mesh (Variables|/Script/Engine.Character|GetMesh _playercharacterref))
  ;[1 1 1] Makes sure movement leaves you facing the right direction NW, NE, SW, SE
  (:Pressed
    (Transformation|SetWorldRotation _mesh "0,-45.000000, 0" false false))
  (:Released
    (if (Game|Player|IsInputKeyDown "W")
      (Transformation|SetWorldRotation _mesh "0,-135.000000, 0" false false)
      (elif (Game|Player|IsInputKeyDown "S")
        (Transformation|SetWorldRotation _mesh "0,45.000000, 0" false false)
        (elif (Game|Player|IsInputKeyDown "A")
          (Transformation|SetWorldRotation _mesh "0,135.000000, 0" false false))))))

(fn ConstructionScript)