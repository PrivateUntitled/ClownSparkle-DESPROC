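; Player controller for the puzzle player that maps mouse clicks to the absorb and ink color mechanics.
; It caches the PuzzlePlayer pawn on BeginPlay and gates both actions on that pawn's state, blocking them while inside an obstacle.
; Right click absorbs from an object in range when the player holds no color.
; Left click inks an in-range Obstacle when the held color matches its required color or that requirement is a specific wildcard value.
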(event EventBeginPlay
  (|CallParentFunction)
  (bind _aspuzzle_player (Utilities|Casting|CastToPuzzlePlayer (Game|Player|GetPlayerPawn 0)))
  (Variables|Default|SetPuzzlePlayerRef _aspuzzle_player))

(event Input|MouseEvents|RightMouseButton
  (params (Key :type Key%20Structure :default "None"))
  (bind _puzzleplayerref (Variables|Default|GetPuzzlePlayerRef))
  ;[1 1 1] Absorb
  (:Pressed
    (if (Math|Boolean|ANDBoolean (!= (Variables|/Game/OctoInkContent/Actors/Player/PuzzlePlayer.PuzzlePlayer_C|GetObjectInRange _puzzleplayerref) 0) (not (Variables|/Game/OctoInkContent/Actors/Player/PuzzlePlayer.PuzzlePlayer_C|GetHasColor _puzzleplayerref)) (not (Variables|/Game/OctoInkContent/Actors/Player/PuzzlePlayer.PuzzlePlayer_C|GetIsPlayerInObstacle _puzzleplayerref)) (Utilities|Enum|Equal(Enum) "NewEnumerator6" (Variables|/Game/OctoInkContent/Data_Assets/PDA_Color.PDA_Color_C|GetColor (Variables|/Game/OctoInkContent/Actors/Player/PuzzlePlayer.PuzzlePlayer_C|GetCurrentColor _puzzleplayerref))))
      (Default|Absorb (Variables|Default|GetPuzzlePlayerRef)))))

(event Input|MouseEvents|LeftMouseButton
  (params (Key :type Key%20Structure :default "None"))
  (bind _puzzleplayerref (Variables|Default|GetPuzzlePlayerRef))
  (bind _currentcolor (Variables|/Game/OctoInkContent/Actors/Player/PuzzlePlayer.PuzzlePlayer_C|GetCurrentColor _puzzleplayerref))
  (bind _color (Variables|/Game/OctoInkContent/Data_Assets/PDA_Color.PDA_Color_C|GetColor _currentcolor))
  ;[1 1 1] Ink
  (:Pressed
    (bind _asobstacle (Utilities|Casting|CastToObstacle (Variables|/Game/OctoInkContent/Actors/Player/PuzzlePlayer.PuzzlePlayer_C|GetObjectInRange _puzzleplayerref)))
    (if (Math|Boolean|ANDBoolean (or (Utilities|Enum|Equal(Enum) (Variables|/Game/OctoInkContent/Actors/Obstacle.Obstacle_C|GetColorRequired _asobstacle) _color) (Utilities|Enum|Equal(Enum) (Variables|/Game/OctoInkContent/Actors/Obstacle.Obstacle_C|GetColorRequired _asobstacle) "NewEnumerator7")) (Variables|/Game/OctoInkContent/Actors/Player/PuzzlePlayer.PuzzlePlayer_C|GetHasColor _puzzleplayerref) (not (Variables|/Game/OctoInkContent/Actors/Player/PuzzlePlayer.PuzzlePlayer_C|GetIsPlayerInObstacle _puzzleplayerref)) (Utilities|Enum|NotEqual(Enum) _color "NewEnumerator6"))
      (Default|Ink (Variables|Default|GetPuzzlePlayerRef)))))

(fn ConstructionScript)