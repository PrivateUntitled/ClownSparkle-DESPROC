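; Player controller that drives BP_Player movement and triggers its Absorb and Ink actions on nearby obstacles.
; Caches the player character on BeginPlay and moves the pawn along axes flattened to the control rotation's yaw.
; Right mouse calls Absorb when HasColor is set and the obstacle isn't Transparent; left mouse calls Ink when HasColor is unset and it is.
; Both actions require an obstacle in range and the player outside obstacles.
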(event EventBeginPlay
  (bind _asbp_player (Utilities|Casting|CastToBP_Player (Game|GetPlayerCharacter 0)))
  (Variables|Default|SetPlayerCharacter _asbp_player))

(event EventTick
  (params (DeltaSeconds :type Float%20%28single-precision%29)))

(event Input|AxisEvents|InputAxisMoveForward
  (params (AxisValue :type Float%20%28single-precision%29))
  (Pawn|Input|AddMovementInput (Game|Player|GetPlayerPawn 0) (Math|Vector|GetForwardVector (Math|Rotator|MakeRotator 0.0 0.0 (.Yaw (Math|Rotator|BreakRotator (Pawn|GetControlRotation :!class /Script/Engine.Controller))))) AxisValue false))

(event Input|AxisEvents|InputAxisMoveRight
  (params (AxisValue :type Float%20%28single-precision%29))
  (Pawn|Input|AddMovementInput (Game|Player|GetPlayerPawn 0) (Math|Vector|GetRightVector (Math|Rotator|MakeRotator 0.0 0.0 (.Yaw (Math|Rotator|BreakRotator (Pawn|GetControlRotation :!class /Script/Engine.Controller))))) AxisValue false))

(event Input|MouseEvents|RightMouseButton
  (params (Key :type Key%20Structure))
  (bind _playercharacter (Variables|Default|GetPlayerCharacter))
  (bind _obstacleinrange (Variables|/Game/OctoInkContent/Actors/BP_Player.BP_Player_C|GetObstacleInRange _playercharacter))
  (:Pressed
    (if (Math|Boolean|ANDBoolean (!= _obstacleinrange 0) (Variables|/Game/OctoInkContent/Actors/BP_Player.BP_Player_C|GetHasColor _playercharacter) (not (Variables|/Game/OctoInkContent/Actors/BP_Player.BP_Player_C|GetIsPlayerInObstacle _playercharacter)))
      (if (!= (Rendering|Material|GetMaterial (Variables|/Game/OctoInkContent/Actors/Obstacle.Obstacle_C|GetStaticMesh _obstacleinrange) 0) "/Game/OctoInkContent/Materials/Transparent.Transparent")
        (Default|Absorb (Variables|Default|GetPlayerCharacter))))))

(event Input|MouseEvents|LeftMouseButton
  (params (Key :type Key%20Structure))
  (bind _playercharacter (Variables|Default|GetPlayerCharacter))
  (bind _obstacleinrange (Variables|/Game/OctoInkContent/Actors/BP_Player.BP_Player_C|GetObstacleInRange _playercharacter))
  (:Pressed
    (if (Math|Boolean|ANDBoolean (!= _obstacleinrange 0) (not (Variables|/Game/OctoInkContent/Actors/BP_Player.BP_Player_C|GetHasColor _playercharacter)) (not (Variables|/Game/OctoInkContent/Actors/BP_Player.BP_Player_C|GetIsPlayerInObstacle _playercharacter)))
      (if (== (Rendering|Material|GetMaterial (Variables|/Game/OctoInkContent/Actors/Obstacle.Obstacle_C|GetStaticMesh _obstacleinrange) 0) "/Game/OctoInkContent/Materials/Transparent.Transparent")
        (Default|Ink (Variables|Default|GetPlayerCharacter))))))

(fn ConstructionScript)